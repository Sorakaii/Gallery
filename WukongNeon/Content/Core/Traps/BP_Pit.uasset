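; BP_Pit is a pit trap that moves the mesh of BP_Wukong vertically when that character overlaps its Box.
; Box overlap plays a timeline whose Z output is added to the mesh's relative location on each update, so the offset accumulates.
; End overlap clears FallingVoid before testing it, so re-enabling input never runs; BeginPlay also leaves the Wukong reference set to None.
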(event OnComponentBeginOverlap(Box)
  (params (OverlappedComponent :type Primitive%20Component%20Object%20Reference) (OtherActor :type Actor%20Object%20Reference) (OtherComp :type Primitive%20Component%20Object%20Reference) (OtherBodyIndex :type Integer) (bFromSweep :type Boolean) (SweepResult :type Hit%20Result%20Structure%20%28by%20ref%29))
  (bind _asbp_wukong (Utilities|Casting|CastToBP_Wukong OtherActor))
  (bind _z (Timeline|Timeline_0 Play)
    (:Update
      (Transformation|AddRelativeLocation (Variables|/Script/Engine.Character|GetMesh _asbp_wukong) (Math|Vector|MakeVector 0.0 0.0 _z) false false))))

(event OnComponentEndOverlap(Box)
  (params (OverlappedComponent :type Primitive%20Component%20Object%20Reference) (OtherActor :type Actor%20Object%20Reference) (OtherComp :type Primitive%20Component%20Object%20Reference) (OtherBodyIndex :type Integer))
  (Utilities|Casting|CastToBP_Wukong OtherActor)
  (bind _output_get (Variables|Default|SetfallingVoid false))
  (if _output_get
    (Input|EnableInput (.Wukong (Variables|Default|GetWukong)) (Game|GetPlayerController 0))))

(event EventBeginPlay
  (bind _returnvalue (Actor|GetActorOfClass "/Game/Core/PlayerCharacter/BP_Wukong.BP_Wukong_C"))
  (Variables|Default|SetWukong 0 _returnvalue))

(event Collision|EventActorBeginOverlap
  (params (OtherActor :type Actor%20Object%20Reference)))

(event EventTick
  (params (DeltaSeconds :type Float%20%28single-precision%29)))

(fn ConstructionScript)