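; Trap that repeatedly launches balls at the player (BP_Wukong) while they stand inside its trigger box.
; Entering the box stores the player and starts a looping timer at the RateFire interval; leaving clears it.
; Each shot spawns a BP_ball at the Scene component rotated toward the player's current location, passes it DamageTrap, plays a Wwise sound and activates a Niagara effect.
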(event OnComponentBeginOverlap(Box)
  (params (OverlappedComponent :type Primitive%20Component%20Object%20Reference) (OtherActor :type Actor%20Object%20Reference) (OtherComp :type Primitive%20Component%20Object%20Reference) (OtherBodyIndex :type Integer) (bFromSweep :type Boolean) (SweepResult :type Hit%20Result%20Structure%20%28by%20ref%29))
  (bind _asbp_wukong (Utilities|Casting|CastToBP_Wukong OtherActor))
  (Variables|Default|SetAs%20BP%20Wukong _asbp_wukong)
  (bind _returnvalue (Utilities|Time|SetTimerbyEvent (delegate Custom|Fire) (Variables|Default|GetrateFire) true))
  (Variables|Default|SetClearTimer _returnvalue))

(event OnComponentEndOverlap(Box)
  (params (OverlappedComponent :type Primitive%20Component%20Object%20Reference) (OtherActor :type Actor%20Object%20Reference) (OtherComp :type Primitive%20Component%20Object%20Reference) (OtherBodyIndex :type Integer))
  (Utilities|Casting|CastToBP_Wukong OtherActor)
  (Utilities|Time|ClearandInvalidateTimerbyHandle (Variables|Default|GetClearTimer)))

(event Custom|Fire
  (bind _scene (Variables|Default|GetScene))
  (bind _returnvalue (Transformation|GetWorldLocation _scene))
  (if true
    (Class|AkGameplayStatics|PostEvent "/Game/WwiseAudio/Events/Lucas/Play_BlowBalls.Play_BlowBalls" self)
    (bind _returnvalue_2 (Game|SpawnActorfromClass "/Game/Core/Traps/BP_ball.BP_ball_C" (Math|Transform|MakeTransform _returnvalue (Math|Rotator|FindLookatRotation _returnvalue (Transformation|GetActorLocation (Variables|Default|GetAs%20BP%20Wukong))) "1,1,1") "Undefined" 0 0))
    (Variables|/Game/Core/Traps/BP_ball.BP_ball_C|SetDamageTrap _returnvalue_2 (Variables|Default|GetDamage%20Trap))
    (Components|Activation|Activate (Variables|Default|GetNiagara) true)))

(event EventBeginPlay)

(event Collision|EventActorBeginOverlap
  (params (OtherActor :type Actor%20Object%20Reference)))

(event EventTick
  (params (DeltaSeconds :type Float%20%28single-precision%29)))

(fn ConstructionScript)