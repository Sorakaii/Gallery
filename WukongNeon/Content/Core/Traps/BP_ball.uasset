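; BP_ball is a short-lived trap ball that damages the Wukong character on contact.
; A looping timer spins the Sphere mesh while a one-second delay destroys the actor.
; Overlap on Sphere1 casts to BP_Wukong_WithSkin, applies DamageTrap damage and destroys the ball.
; BeginPlay also stores a Minion_Parent_BP reference in Ennemies, which these graphs never use.
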(event OnComponentBeginOverlap(Sphere1)
  (params (OverlappedComponent :type Primitive%20Component%20Object%20Reference) (OtherActor :type Actor%20Object%20Reference) (OtherComp :type Primitive%20Component%20Object%20Reference) (OtherBodyIndex :type Integer) (bFromSweep :type Boolean) (SweepResult :type Hit%20Result%20Structure%20%28by%20ref%29))
  (bind _asbp_wukong_with_skin (Utilities|Casting|CastToBP_Wukong_WithSkin OtherActor))
  (Game|Damage|ApplyDamage _asbp_wukong_with_skin (Variables|Default|GetDamageTrap) 0 0)
  (Actor|DestroyActor))

(event Custom|sETrOTATION
  (Transformation|AddWorldRotation (Variables|Default|GetSphere) "5.000000,4.000000,2.000000" false false))

(event EventBeginPlay
  (bind _returnvalue (Actor|GetActorOfClass "/Game/Core/AI/Minions/Minion_Parent_BP.Minion_Parent_BP_C"))
  (Variables|Default|Setennemies _returnvalue)
  (Utilities|Time|SetTimerbyEvent (delegate Custom|sETrOTATION) 0.01 true)
  (Utilities|FlowControl|Delay 1.0)
  (Actor|DestroyActor))

(event Collision|EventActorBeginOverlap
  (params (OtherActor :type Actor%20Object%20Reference)))

(event EventTick
  (params (DeltaSeconds :type Float%20%28single-precision%29)))

(fn ConstructionScript)