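; Ground spike trap that moves a mesh or component vertically when BP_Wukong enters its trigger box and damages on contact.
; The Box overlap starts a timeline that drives the Z location of Object, replaying from the start while Wukong stays inside.
; A separate Dmg collider applies DamageTrap when Wukong touches it, then destroys the actor, so the trap hits only once.
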(event OnComponentBeginOverlap(Box)
  (params (OverlappedComponent :type Primitive%20Component%20Object%20Reference) (OtherActor :type Actor%20Object%20Reference) (OtherComp :type Primitive%20Component%20Object%20Reference) (OtherBodyIndex :type Integer) (bFromSweep :type Boolean) (SweepResult :type Hit%20Result%20Structure%20%28by%20ref%29))
  (Utilities|Casting|CastToBP_Wukong OtherActor)
  (Variables|Default|Setinside true)
  (bind _z (Timeline|Timeline_0 Play)
    (:Update
      (Transformation|SetRelativeLocation (Variables|Default|Getobject) (Math|Vector|MakeVector 0.0 0.0 _z) false false))
    (:Finished
      (if (Variables|Default|Getinside)
        (Timeline|Timeline_0 PlayFromStart)))))

(event OnComponentEndOverlap(Box)
  (params (OverlappedComponent :type Primitive%20Component%20Object%20Reference) (OtherActor :type Actor%20Object%20Reference) (OtherComp :type Primitive%20Component%20Object%20Reference) (OtherBodyIndex :type Integer))
  (Utilities|Casting|CastToBP_Wukong OtherActor)
  (Variables|Default|Setinside false))

(event OnComponentBeginOverlap(Dmg)
  (params (OverlappedComponent :type Primitive%20Component%20Object%20Reference) (OtherActor :type Actor%20Object%20Reference) (OtherComp :type Primitive%20Component%20Object%20Reference) (OtherBodyIndex :type Integer) (bFromSweep :type Boolean) (SweepResult :type Hit%20Result%20Structure%20%28by%20ref%29))
  (Utilities|Casting|CastToBP_Wukong OtherActor)
  (Game|Damage|ApplyDamage 0 (Variables|Default|GetDamageTrap) 0 0)
  (Actor|DestroyActor))

(event EventBeginPlay)

(event Collision|EventActorBeginOverlap
  (params (OtherActor :type Actor%20Object%20Reference)))

(event EventTick
  (params (DeltaSeconds :type Float%20%28single-precision%29)))

(fn ConstructionScript)