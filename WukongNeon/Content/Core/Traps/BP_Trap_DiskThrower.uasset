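; BP_Trap_DiskThrower is a trap that repeatedly throws disks at the player while they are inside its trigger box.
; It caches the BP_Wukong player on BeginPlay, then box overlap starts a looping fire timer and end overlap clears it.
; Each shot spawns a BP_TrapComponent_Disk at the Scene component, rotated toward the player's current location, and activates a Niagara effect.
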(event OnComponentBeginOverlap(Box)
  (params (OverlappedComponent :type Primitive%20Component%20Object%20Reference) (OtherActor :type Actor%20Object%20Reference) (OtherComp :type Primitive%20Component%20Object%20Reference) (OtherBodyIndex :type Integer) (bFromSweep :type Boolean) (SweepResult :type Hit%20Result%20Structure%20%28by%20ref%29))
  (Utilities|Casting|CastToBP_Wukong OtherActor)
  (bind _returnvalue (Utilities|Time|SetTimerbyEvent (delegate Custom|fire) (Variables|Default|GetrateFire) true))
  (Variables|Default|SetNewVar_0 _returnvalue))

(event OnComponentEndOverlap(Box)
  (params (OverlappedComponent :type Primitive%20Component%20Object%20Reference) (OtherActor :type Actor%20Object%20Reference) (OtherComp :type Primitive%20Component%20Object%20Reference) (OtherBodyIndex :type Integer))
  (Utilities|Casting|CastToBP_Wukong OtherActor)
  (Utilities|Time|ClearandInvalidateTimerbyHandle (Variables|Default|GetNewVar_0)))

(event Custom|fire
  (bind _scene (Variables|Default|GetScene))
  (bind _returnvalue (Transformation|GetWorldLocation _scene))
  (Game|SpawnActorfromClass "/Game/Core/Traps/BP_TrapComponent_Disk.BP_TrapComponent_Disk_C" (Math|Transform|MakeTransform _returnvalue (Math|Rotator|FindLookatRotation _returnvalue (Transformation|GetActorLocation (Variables|Default|GetPlayer))) "1,1,1") "Undefined" 0 0)
  (Components|Activation|Activate (Variables|Default|GetNiagara) true))

(event EventBeginPlay
  (bind _asbp_wukong (Utilities|Casting|CastToBP_Wukong (Game|GetPlayerCharacter 0)))
  (Variables|Default|SetPlayer _asbp_wukong))

(event Collision|EventActorBeginOverlap
  (params (OtherActor :type Actor%20Object%20Reference)))

(event EventTick
  (params (DeltaSeconds :type Float%20%28single-precision%29)))

(fn ConstructionScript)