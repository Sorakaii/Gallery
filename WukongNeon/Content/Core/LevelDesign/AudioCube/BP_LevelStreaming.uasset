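; Trigger-box actor that loads or unloads a named sublevel, depending on its streaming type, when the player overlaps it.
; Loading blocks, then stores the count of minion actors in the Wukong player's enemy count.
; If no upgrade actor exists, it spawns a random upgrade at the last TargetPoint found, then hides itself and disables its collision.
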(event OnComponentBeginOverlap(Box)
  (params (OverlappedComponent :type Primitive%20Component%20Object%20Reference) (OtherActor :type Actor%20Object%20Reference) (OtherComp :type Primitive%20Component%20Object%20Reference) (OtherBodyIndex :type Integer) (bFromSweep :type Boolean) (SweepResult :type Hit%20Result%20Structure%20%28by%20ref%29))
  (bind _level_name (Variables|Default|GetLevel%20Name))
  (bind _structupgrade (Variables|Default|GetstructUpgrade))
  (if (== OtherActor (Game|GetPlayerCharacter 0))
    (if (Utilities|Enum|Equal(Enum) (Variables|Default|GetStreamingType) "NewEnumerator0")
      (Game|LoadStreamLevel(byName) _level_name true true)
      (bind _outactors (Actor|GetAllActorsOfClass "/Game/Core/AI/Minions/Minion_Parent_BP.Minion_Parent_BP_C"))
      (bind _asbp_wukong_with_skin (Utilities|Casting|CastToBP_Wukong_WithSkin (Game|GetPlayerCharacter 0)))
      (Variables|/Game/Core/PlayerCharacter/BP_Wukong_WithSkin.BP_Wukong_WithSkin_C|SetEnemyCount _asbp_wukong_with_skin (Utilities|Array|Length _outactors))
      (bind _returnvalue (Actor|GetActorOfClass "/Game/Core/Upgrades/BP_Upgrade_Parent.BP_Upgrade_Parent_C"))
      (Utilities|IsValid _returnvalue
        (:Is%20Not%20Valid
          (bind _outactors_2 (Actor|GetAllActorsOfClass "/Script/Engine.TargetPoint"))
          (Utilities|IsValid (Utilities|Array|Get(acopy) _outactors_2 (- (Utilities|Array|Length _outactors_2) 1))
            (:Is%20Valid
              (Game|SpawnActorfromClass (.upgrade (Utilities|Array|Get(acopy) _structupgrade (Math|Random|RandomInteger (Utilities|Array|Length _structupgrade)))) (Math|Transform|MakeTransform (Transformation|GetActorLocation (Utilities|Array|Get(acopy) _outactors_2 (- (Utilities|Array|Length _outactors_2) 1))) "0, 0, 0" "1,1,1") "Undefined" 0 0)
              (Rendering|SetActorHiddenInGame true)
              (Collision|SetActorEnableCollision false)))))
      (else
        (Game|UnloadStreamLevel(byName) _level_name false)))))

(event EventBeginPlay)

(event Collision|EventActorBeginOverlap
  (params (OtherActor :type Actor%20Object%20Reference)))

(fn ConstructionScript)