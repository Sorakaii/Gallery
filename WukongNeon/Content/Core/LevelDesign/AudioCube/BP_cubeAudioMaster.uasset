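; BP_cubeAudioMaster is a cube actor that plays a configurable sound after a start delay and can make its material glow in time with the audio.
; Each tick it normalizes the audio component's envelope value against a running peak, which a looping timer slowly decays so the response adapts to loudness changes.
; When glow is enabled, that normalized volume drives the emissive strength of a dynamic material instance.
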(event OnAudioSingleEnvelopeValue(AudioComponent)
  (params (PlayingSoundWave :type Sound%20Wave%20Object%20Reference) (EnvelopeValue :type Float%20%28single-precision%29))
  ;[1 1 1] Store latest envelope value
  (Variables|Default|SetLatestEnvelopeValue EnvelopeValue))

(event OnAudioPlaybackPercent(AudioComponent)
  (params (PlayingSoundWave :type Sound%20Wave%20Object%20Reference) (PlaybackPercent :type Float%20%28single-precision%29))
  ;[1 1 1] Store latest playback percent value
  (Variables|Default|SetAudioPlaybackPercent PlaybackPercent))

(event Custom|LowerMaxRecordedVolume
  (bind _output_get (Variables|Default|SetMaxRecordedVol (* (stale _output_get) 0.95))))

(event EventBeginPlay
  (Utilities|FlowControl|Sequence
    (:then_0
      (bind _returnvalue (Rendering|Material|CreateDynamicMaterialInstance (Variables|Default|GetBaseMaterial) "None" "None" :!class /Script/Engine.KismetMaterialLibrary))
      (Variables|Default|SetMID _returnvalue)
      (Rendering|Material|SetMaterial (Variables|Default|GetCube) 0 (Variables|Default|GetMID)))
    (:then_1
      (Utilities|Time|SetTimerbyEvent (delegate Custom|LowerMaxRecordedVolume) 0.5 true))
    (:then_2
      (Utilities|FlowControl|Delay (Variables|Default|GetDelayedStartInSeconds))
      (Audio|Components|Audio|SetSound (Variables|Default|GetAudioComponent) (Variables|Default|GetSoundToPlay))
      (Variables|/Script/Engine.AudioComponent|SetVolumeMultiplier (Variables|Default|GetAudioComponent) (Variables|Default|GetVolumeMP))
      (Audio|Components|Audio|SetPitchMultiplier (Variables|Default|GetAudioComponent) (Variables|Default|GetPitchMultiplier))
      (Audio|Components|Audio|Play (Variables|Default|GetAudioComponent) 0.0))))

(event Collision|EventActorBeginOverlap
  (params (OtherActor :type Actor%20Object%20Reference)))

(event EventTick
  (params (DeltaSeconds :type Float%20%28single-precision%29))
  (Utilities|FlowControl|Sequence
    (:then_0
      (CallFunction|NormalizeVolume (Variables|Default|GetLatestEnvelopeValue)))
    (:then_1
      (if (Variables|Default|GetGlowMaterialToAudio)
        (CallFunction|UpdateMaterialEmissive)))))

(fn ConstructionScript)

(fn NormalizeVolume
  (params (LatestEnvelopeValue :type Float%20%28single-precision%29))
  (LocalVariables|Set_latestEnvelope LatestEnvelopeValue)
  (Utilities|FlowControl|Sequence
    (:then_0
      ;[1 1 1] store maximum normalized volume
      (if (> (LocalVariables|Get_latestEnvelope) (Variables|Default|GetMaxRecordedVol))
        (Variables|Default|SetMaxRecordedVol (LocalVariables|Get_latestEnvelope))))
    (:then_1
      ;[1 1 1] Clamp 0-1
      (Variables|Default|SetNormalizedVolume (Math|Float|Clamp(Float) (Math|Float|NormalizetoRange (LocalVariables|Get_latestEnvelope) 0.0 (Variables|Default|GetMaxRecordedVol)))))
    (:then_2
      ;[1 1 1] Return
      (return (Variables|Default|GetNormalizedVolume)))))

(fn UpdateMaterialEmissive
  (Rendering|Material|SetScalarParameterValue (Variables|Default|GetMID) "EmissiveMultiplier" (* (Variables|Default|GetNormalizedVolume) (Variables|Default|GetMaterialEmissiveStrength)) :!class /Script/Engine.MaterialInstanceDynamic))