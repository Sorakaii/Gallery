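; BP_cubeAudio is a level cube whose material glow can pulse with audio volume.
; On BeginPlay it applies a dynamic material instance to the cube and finds the BP_cubeAudioMaster actor.
; Each tick it normalizes the envelope value against the recorded maximum and, if enabled, scales the EmissiveMultiplier parameter by it.
; It then copies the latest envelope and maximum from the master, so the glow uses the previous tick's values.
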(event EventBeginPlay
  (Utilities|FlowControl|Sequence
    (:then_0
      (bind _returnvalue (Rendering|Material|CreateDynamicMaterialInstance (Variables|Default|GetBaseMaterial) "None" "None" :!class /Script/Engine.KismetMaterialLibrary))
      (Variables|Default|SetMID _returnvalue)
      (Rendering|Material|SetMaterial (Variables|Default|GetCube) 0 (Variables|Default|GetMID)))
    (:then_1
      (bind _returnvalue_2 (Actor|GetActorOfClass "/Game/Core/LevelDesign/AudioCube/BP_cubeAudioMaster.BP_cubeAudioMaster_C"))
      (Variables|Default|SetAudioMasterRef _returnvalue_2))))

(event Collision|EventActorBeginOverlap
  (params (OtherActor :type Actor%20Object%20Reference)))

(event EventTick
  (params (DeltaSeconds :type Float%20%28single-precision%29))
  (bind _audiomasterref (Variables|Default|GetAudioMasterRef))
  (Utilities|FlowControl|Sequence
    (:then_0
      (CallFunction|NormalizeVolume (Variables|Default|GetLatestEnvelopeValue)))
    (:then_1
      (if (Variables|Default|GetGlowMaterialToAudio)
        (CallFunction|UpdateMaterialEmissive)))
    (:then_2
      (Variables|Default|SetLatestEnvelopeValue (Variables|/Game/Core/LevelDesign/AudioCube/BP_cubeAudioMaster.BP_cubeAudioMaster_C|GetLatestEnvelopeValue _audiomasterref))
      (Variables|Default|SetMaxRecordedVol (Variables|/Game/Core/LevelDesign/AudioCube/BP_cubeAudioMaster.BP_cubeAudioMaster_C|GetMaxRecordedVol _audiomasterref)))))

(fn ConstructionScript)

(fn NormalizeVolume
  (params (LatestEnvelopeValue :type Float%20%28single-precision%29))
  (LocalVariables|Set_latestEnvelope LatestEnvelopeValue)
  (Utilities|FlowControl|Sequence
    (:then_0
      ;[1 1 1] store maximum normalized volume
      (if (> (LocalVariables|Get_latestEnvelope) (Variables|Default|GetMaxRecordedVol))
        (Variables|Default|SetMaxRecordedVol (LocalVariables|Get_latestEnvelope))))
    (:then_1
      ;[1 1 1] Clamp 0-1
      (Variables|Default|SetNormalizedVolume (Math|Float|Clamp(Float) (Math|Float|NormalizetoRange (LocalVariables|Get_latestEnvelope) 0.0 (Variables|Default|GetMaxRecordedVol)))))
    (:then_2
      ;[1 1 1] Return
      (return (Variables|Default|GetNormalizedVolume)))))

(fn UpdateMaterialEmissive
  (Rendering|Material|SetScalarParameterValue (Variables|Default|GetMID) "EmissiveMultiplier" (* (Variables|Default|GetNormalizedVolume) (Variables|Default|GetMaterialEmissiveStrength)) :!class /Script/Engine.MaterialInstanceDynamic))