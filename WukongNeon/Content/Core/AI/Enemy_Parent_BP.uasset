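; Enemy_Parent_BP is a base enemy Blueprint that handles health loss and death.
; AnyDamage subtracts the truncated damage from an integer Hp clamped between zero and MaxHp, then calls the Death event at zero, which destroys the actor.
; Tick only forwards to the parent, while BeginPlay and the GetDamaged function are empty.
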(event Custom|Death
  (Actor|DestroyActor))

(event EventBeginPlay)

(event Collision|EventActorBeginOverlap
  (params (OtherActor :type Actor%20Object%20Reference)))

(event Game|Damage|EventAnyDamage
  (params (Damage :type Float%20%28single-precision%29) (DamageType :type Damage%20Type%20Object%20Reference) (InstigatedBy :type Controller%20Object%20Reference) (DamageCauser :type Actor%20Object%20Reference))
  (Variables|Default|Sethp (Math|Integer|Clamp(Integer) (- (Variables|Default|Gethp) (Math|Float|Truncate Damage)) 0 (Variables|Default|GetmaxHp)))
  (if (<= (Variables|Default|Gethp) 0)
    (CallFunction|Death)))

(event EventTick
  (params (DeltaSeconds :type Float%20%28single-precision%29))
  (|CallParentFunction DeltaSeconds))

(fn ConstructionScript)

(fn GetDamaged
  (params (Damage :type Integer)))