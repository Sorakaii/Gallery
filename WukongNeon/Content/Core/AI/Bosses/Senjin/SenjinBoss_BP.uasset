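; Senjin boss Blueprint for the fight against Wukong, passing the player to its Blackboard and exposing three attack events.
; Mirror rings the player with clones, hides the boss among them and converges on center into a flying kick, while an overlap box impulses escapees back.
; Pose teleports to trace-checked spots around the player and fires timed, fanned clone projectiles.
; Charge performs two timeline dashes with once-per-dash box-trace damage, backflipping and re-aiming after each.
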(event OnComponentBeginOverlap(BoxNoEscape)
  (params (OverlappedComponent :type Primitive%20Component%20Object%20Reference) (OtherActor :type Actor%20Object%20Reference) (OtherComp :type Primitive%20Component%20Object%20Reference) (OtherBodyIndex :type Integer) (bFromSweep :type Boolean) (SweepResult :type Hit%20Result%20Structure%20%28by%20ref%29))
  (bind _asbp_wukong (Utilities|Casting|CastToBP_Wukong OtherActor))
  (CallFunction|PlayerPushBacktoCenter _asbp_wukong))

(event Custom|Mirror
  (Variables|Default|SetisInMirror true)
  (Collision|SetCollisionEnabled (Variables|Default|GetBoxNoEscape) "QueryOnly")
  (Variables|Clones|SetspawnCenter (Transformation|GetActorLocation (Game|GetPlayerCharacter 0)))
  (for _index (range 1 (Variables|Clones|GetcloneQuantity))
    (bind _returnvalue (Game|SpawnActorfromClass "/Game/Core/AI/Bosses/Senjin/SenjinBoss_Clone_BP.SenjinBoss_Clone_BP_C" (Math|Transform|MakeTransform (+ (* (Math|Vector|GetForwardVector (Math|Rotator|MakeRotator 0.0 0.0 (Math|Conversions|ToFloat(Integer) (* _index (/ 360 (Variables|Clones|GetcloneQuantity)))))) (Variables|Clones|GetspawnRadius)) (Variables|Clones|GetspawnCenter)) (Math|Rotator|FindLookatRotation (+ (* (Math|Vector|GetForwardVector (Math|Rotator|MakeRotator 0.0 0.0 (Math|Conversions|ToFloat(Integer) (* _index (/ 360 (Variables|Clones|GetcloneQuantity)))))) (Variables|Clones|GetspawnRadius)) (Variables|Clones|GetspawnCenter)) (Variables|Clones|GetspawnCenter)) "1,1,1") "Undefined" 0 (Variables|Clones|GetspawnCenter) self 0))
    (Utilities|Array|Add (Variables|Clones|GetClones_Array) _returnvalue))
  (Variables|Clones|SetcloneToReplace (Utilities|Array|Get(acopy) (Variables|Clones|GetClones_Array) (Math|Random|RandomInteger (Variables|Clones|GetcloneQuantity))))
  (Transformation|SetActorLocation (Transformation|GetActorLocation (Variables|Clones|GetcloneToReplace)) false false)
  (Transformation|SetActorRotation (Transformation|GetActorRotation (Variables|Clones|GetcloneToReplace)))
  (Utilities|Array|RemoveItem (Variables|Clones|GetClones_Array) (Variables|Clones|GetcloneToReplace))
  (Actor|DestroyActor (Variables|Clones|GetcloneToReplace))
  (Utilities|FlowControl|Delay 3.0)
  (for _array_element (Variables|Clones|GetClones_Array)
    (AI|AIMoveTo _array_element (Variables|Clones|GetspawnCenter) 0 (Variables|Default|GetacceptanceRadiusFromPlayer) false))
  (Variables|/Script/Engine.CharacterMovementComponent|SetMaxWalkSpeed (Variables|Character|GetCharacterMovement) 1e+02)
  (AI|AIMoveTo self (Variables|Clones|GetspawnCenter) 0 (Variables|Default|GetacceptanceRadiusFromPlayer) false
    (:OnSuccess
      (Collision|SetCollisionEnabled (Variables|Default|GetBoxNoEscape) "NoCollision")
      (Animation|Montage|PlayMontage (Variables|Character|GetMesh) "/Game/Characters/Bosses/Senjin/SenjinUpdate/animation/Flying_Kick__1__Montage.Flying_Kick__1__Montage"
        (:OnCompleted
          (Variables|Default|SetisInMirror false))))))

(event Custom|playerPushBackToCenter
  (params (playerRef :type BP%20Wukong%20Object%20Reference))
  (bind _returnvalue (Utilities|Time|SetTimerbyEvent (delegate Custom|Push) 0.01 true))
  (Variables|Default|SetpushTimer _returnvalue))

(event Custom|Push
  (Physics|AddImpulse (Variables|/Script/Engine.Character|GetCharacterMovement (Game|GetPlayerCharacter 0)) (* (- (Transformation|GetActorLocation (Game|GetPlayerCharacter 0)) (Variables|Clones|GetspawnCenter)) -1.0) true)
  (if (Math|Vector|Equal(Vector) (Transformation|GetActorLocation (Game|GetPlayerCharacter 0)) (Variables|Clones|GetspawnCenter) 1e+02)
    (Utilities|Time|ClearandInvalidateTimerbyHandle (Variables|Default|GetpushTimer))))

(event Custom|Charge
  (bind _returnvalue (Transformation|GetActorLocation))
  (Variables|Default|SetsenjinLocation (Transformation|GetActorLocation) :!label _label)
  (bind _alpha (Timeline|Charge_Timeline PlayFromStart)
    (:Update
      (Transformation|SetActorLocation (Math|Vector|MakeVector (.x (Math|Vector|Lerp(Vector) (Variables|Default|GetsenjinLocation) (+ (Variables|Default|GetsenjinLocation) (* (Transformation|GetActorForwardVector) 2.7e+03)) _alpha)) (.y (Math|Vector|Lerp(Vector) (Variables|Default|GetsenjinLocation) (+ (Variables|Default|GetsenjinLocation) (* (Transformation|GetActorForwardVector) 2.7e+03)) _alpha)) (.z (Variables|Default|GetsenjinLocation))) true false)
      (bind (_outhit _returnvalue_2) (Class|KismetSystemLibrary|BoxTraceSingleforObjects _returnvalue _returnvalue "70.000000,70.000000,70.000000" "0, 0, 0" (Utilities|Array|MakeArray "ObjectTypeQuery7") false 0 "None" true))
      (if _returnvalue_2
        (Utilities|FlowControl|DoOnce false
          (:Completed
            (Game|Damage|ApplyDamage (Game|GetPlayerCharacter 0) (Variables|Default|GetdashDamage) 0 self)))))
    (:Finished
      (CallFunction|ResetHitBox)
      (Animation|Montage|PlayMontage (Variables|Character|GetMesh) "/Game/Characters/Bosses/Senjin/SenjinUpdate/animation/Backflip_Montage.Backflip_Montage" 1.5 0.5
        (:then
          (bind _alpha_2 (Timeline|rotationTimeline PlayFromStart)
            (:Update
              (Transformation|SetActorRotation (Math|Rotator|Lerp(Rotator) (Transformation|GetActorRotation) (Math|Rotator|FindLookatRotation (Transformation|GetActorLocation) (Transformation|GetActorLocation (Game|Player|GetPlayerPawn 0))) _alpha_2)))
            (:Finished
              (Math|Integer|IncrementInt (Variables|Default|GetdashCounter)
                (:%20%20
                  (if (< (Variables|Default|GetdashCounter) 2)
                    (goto _label)
                    (else
                      (Variables|Default|SetdashCounter 0)
                      (Variables|Default|Setdashing false))))))))))))

(event Custom|ResetHitBox
  (Utilities|FlowControl|DoOnce false) ; enters at Reset
)

(event Custom|pose
  (bind _returnvalue (Game|GetPlayerCharacter 0))
  (bind _returnvalue_2 (Math|Random|RandomFloatinRange 0.0 3.6e+02))
  (bind _teleportradius (Variables|Default|GetteleportRadius))
  (bind _returnvalue_3 (Transformation|GetActorLocation _returnvalue))
  (bind _returnvalue_4 (Math|Rotator|MakeRotator 0.0 0.0 _returnvalue_2))
  (bind _returnvalue_5 (Math|Vector|GetForwardVector _returnvalue_4))
  (bind _returnvalue_6 (* _returnvalue_5 _teleportradius))
  (bind _returnvalue_7 (+ _returnvalue_6 _returnvalue_3))
  (Variables|Default|SetposeAttackAnim true)
  (Transformation|SetActorRotation (Math|Rotator|MakeRotator 0.0 0.0 (.yaw (Math|Rotator|FindLookatRotation (Transformation|GetActorLocation) (Transformation|GetActorLocation (Variables|Default|GetplayerRef))))))
  (Variables|Default|SetteleportLocation (Math|Vector|MakeVector (.x _returnvalue_7) (.y _returnvalue_7) (Variables|Default|GetinitialHeight)) :!label _label)
  (bind _outhit (Collision|BoxTraceByChannel (Variables|Default|GetteleportLocation) (Variables|Default|GetteleportLocation) "100.000000,100.000000,100.000000" "0, 0, 0" "TraceTypeQuery2" false 0 "None"))
  (if (.bblockinghit _outhit)
    (goto _label)
    (else
      (Transformation|SetActorLocation (Variables|Default|GetteleportLocation) false false)
      (Utilities|Time|SetTimerbyEvent (delegate Custom|SwitchPose) 0.5 true))))

(event Custom|SwitchPose
  (bind _returnvalue (Game|GetPlayerCharacter 0))
  (bind _returnvalue_2 (Transformation|GetActorTransform))
  (bind _returnvalue_3 (Math|Random|RandomFloatinRange 0.0 3.6e+02))
  (bind _teleportradius (Variables|Default|GetteleportRadius))
  (bind _returnvalue_4 (Transformation|GetActorLocation _returnvalue))
  (bind _returnvalue_5 (Math|Rotator|MakeRotator 0.0 0.0 _returnvalue_3))
  (bind _returnvalue_6 (Math|Vector|GetForwardVector _returnvalue_5))
  (bind _returnvalue_7 (* _returnvalue_6 _teleportradius))
  (bind _returnvalue_8 (+ _returnvalue_7 _returnvalue_4))
  (Math|Integer|IncrementInt (Variables|Default|GetposeIndex)
    (:%20%20
      (if (> (Variables|Default|GetposeIndex) 5)
        (Variables|Default|SetposeIndex 1)
        (Variables|Default|SetteleportLocation (Math|Vector|MakeVector (.x _returnvalue_8) (.y _returnvalue_8) (Variables|Default|GetinitialHeight)) :!label _label)
        (bind _returnvalue_9 (Collision|BoxTraceByChannel (Variables|Default|GetteleportLocation) (Variables|Default|GetteleportLocation) "10.000000,10.000000,10.000000" "0, 0, 0" "TraceTypeQuery2" false 0 "None"))
        (if _returnvalue_9
          (goto _label)
          (else
            (Transformation|SetActorLocation (Variables|Default|GetteleportLocation) false false)
            (Transformation|SetActorRotation (Math|Rotator|MakeRotator 0.0 0.0 (.yaw (Math|Rotator|FindLookatRotation (Transformation|GetActorLocation) (Transformation|GetActorLocation (Variables|Default|GetplayerRef)))))))))
      (Game|SpawnActorfromClass "/Game/Core/AI/Bosses/Senjin/SenjinBoss_Clone_Projectile.SenjinBoss_Clone_Projectile_C" (Math|Transform|MakeTransform (+ (.location _returnvalue_2) (* (Transformation|GetActorForwardVector) 1e+02)) (Math|Rotator|MakeRotator 0.0 0.0 (+ (.Yaw (Math|Rotator|BreakRotator (.rotation _returnvalue_2))) (Utilities|Select :Index (Variables|Default|GetposeIndex) :Option%200 0.0 :Option%201 -2e+01 :Option%202 -1e+01 :Option%203 0.0 :Option%204 1e+01 :Option%205 2e+01)))) "AlwaysSpawn" 0 (Variables|Default|GetposeIndex) 0))))

(event Custom|move)

(event EventBeginPlay
  (Collision|SetCollisionEnabled (Variables|Default|GetBoxNoEscape) "NoCollision")
  (bind _asbp_wukong (Utilities|Casting|CastToBP_Wukong (Game|GetPlayerCharacter 0)))
  (Variables|Default|SetplayerRef _asbp_wukong)
  (bind _returnvalue (Actor|GetActorOfClass "/Script/Engine.TargetPoint"))
  (Variables|Default|SetmapCenter _returnvalue)
  (Variables|Default|SetinitialHeight (.z (Transformation|GetActorLocation)))
  (AI|Components|Blackboard|SetValueasObject (Variables|/Script/AIModule.AIController|GetBlackboard (AI|GetAIController self)) (Variables|Default|GetplayerKeyName) (Variables|Default|GetplayerRef)))

(fn ConstructionScript)