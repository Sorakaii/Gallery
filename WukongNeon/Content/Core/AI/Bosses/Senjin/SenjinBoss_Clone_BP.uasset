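; Senjin boss clone used in the boss's mirror phase, standing in until the player hits one.
; Any damage ends the mirror state, disables the boss's no-escape box, moves the boss to this clone, destroys all clones and plays a sped-up back-kick montage on the boss.
; The clone's own no-escape box has the boss push Wukong back to center on overlap.
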(event OnComponentBeginOverlap(BoxNoEscape)
  (params (OverlappedComponent :type Primitive%20Component%20Object%20Reference) (OtherActor :type Actor%20Object%20Reference) (OtherComp :type Primitive%20Component%20Object%20Reference) (OtherBodyIndex :type Integer) (bFromSweep :type Boolean) (SweepResult :type Hit%20Result%20Structure%20%28by%20ref%29))
  (bind _asbp_wukong (Utilities|Casting|CastToBP_Wukong OtherActor))
  (Default|PlayerPushBacktoCenter (Variables|Default|GetsenjinBossRef) _asbp_wukong))

(event EventBeginPlay)

(event Game|Damage|EventAnyDamage
  (params (Damage :type Float%20%28single-precision%29) (DamageType :type Damage%20Type%20Object%20Reference) (InstigatedBy :type Controller%20Object%20Reference) (DamageCauser :type Actor%20Object%20Reference))
  (bind _returnvalue (Game|GetPlayerCharacter 0))
  (bind _senjinbossref (Variables|Default|GetsenjinBossRef))
  (bind _senjinbossref_2 (Variables|Default|GetsenjinBossRef))
  (bind _returnvalue_2 (Transformation|GetActorLocation _senjinbossref_2))
  (bind _returnvalue_3 (Transformation|GetActorLocation _returnvalue))
  (bind _returnvalue_4 (Math|Rotator|FindLookatRotation _returnvalue_2 _returnvalue_3))
  (Variables|/Game/Core/AI/Bosses/Senjin/SenjinBoss_BP.SenjinBoss_BP_C|SetisInMirror _senjinbossref false)
  (Components|Movement|StopMovementImmediately (Variables|/Script/Engine.Character|GetCharacterMovement (Variables|Default|GetsenjinBossRef)))
  (Collision|SetCollisionEnabled (Variables|/Game/Core/AI/Bosses/Senjin/SenjinBoss_BP.SenjinBoss_BP_C|GetBoxNoEscape (Variables|Default|GetsenjinBossRef)) "NoCollision")
  (Transformation|SetActorLocationAndRotation (Variables|Default|GetsenjinBossRef) (Transformation|GetActorLocation) (Math|Rotator|MakeRotator (.roll _returnvalue_4) (.pitch _returnvalue_4) 0.0))
  (bind _outactors (Actor|GetAllActorsOfClass "SenjinBoss_Clone_BP_C"))
  (for _array_element _outactors
    (Actor|DestroyActor _array_element))
  (Animation|Montage|PlayMontage (Variables|/Script/Engine.Character|GetMesh _senjinbossref) "/Game/Characters/Bosses/Senjin/SenjinUpdate/animation/backKIck.backKIck" 2.0))

(fn ConstructionScript)