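; BP_Crystals is a hazard in the Thomas boss fight that orbits the boss and hurts BP_Wukong on contact.
; Each tick it circles Thomas around the Z axis, with the radius pulsing on a squared sine of the boss's Chrono value.
; Overlapping Wukong applies damage, plays an explosion sound and destroys the crystal.
; Any damage received also destroys it.
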(event OnComponentBeginOverlap(Box)
  (params (OverlappedComponent :type Primitive%20Component%20Object%20Reference) (OtherActor :type Actor%20Object%20Reference) (OtherComp :type Primitive%20Component%20Object%20Reference) (OtherBodyIndex :type Integer) (bFromSweep :type Boolean) (SweepResult :type Hit%20Result%20Structure%20%28by%20ref%29))
  (bind _asbp_wukong (Utilities|Casting|CastToBP_Wukong OtherActor))
  (Game|Damage|ApplyDamage _asbp_wukong 5.0 0 0)
  (Class|AkGameplayStatics|PostEvent "/Game/WwiseAudio/Events/Camille/Play_Explosion.Play_Explosion" (Game|Player|GetPlayerPawn 0))
  (Actor|DestroyActor))

(event EventBeginPlay
  (bind _returnvalue (Actor|GetActorOfClass "/Game/Core/AI/Bosses/Thomas/BP_Thomas.BP_Thomas_C"))
  (Variables|Default|SetThomas _returnvalue))

(event Collision|EventActorBeginOverlap
  (params (OtherActor :type Actor%20Object%20Reference)))

(event EventTick
  (params (DeltaSeconds :type Float%20%28single-precision%29))
  (Transformation|SetActorLocation (+ (Transformation|GetActorLocation (Variables|Default|GetThomas)) (Math|Vector|RotateVectorAroundAxis (Math|Vector|MakeVector (Variables|Default|GetRadiusLenght) 0.0 0.0) (Variables|Default|GetPositionAround) "0, 0,1.000000")) false false)
  (Variables|Default|SetPositionAround (+ (* DeltaSeconds (Variables|Default|GetSpeed)) (Variables|Default|GetPositionAround)))
  (Variables|Default|SetRadiusLenght (Math|Float|Lerp 7.5e+02 1.25e+03 (Math|Float|Power (Math|Trig|Sin(Degrees) (* (+ (Variables|/Game/Core/AI/Bosses/Thomas/BP_Thomas.BP_Thomas_C|GetChrono (Variables|Default|GetThomas)) 0.5) 1.8e+02)) 2.0))))

(event Game|Damage|EventAnyDamage
  (params (Damage :type Float%20%28single-precision%29) (DamageType :type Damage%20Type%20Object%20Reference) (InstigatedBy :type Controller%20Object%20Reference) (DamageCauser :type Actor%20Object%20Reference))
  (Actor|DestroyActor))

(fn ConstructionScript)