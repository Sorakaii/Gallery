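; Repeating shockwave for the Thomas boss that knocks the Wukong character away from its center.
; Tick grows the collision sphere from the fractional part of Ratio, which is not updated here, capping the radius and re-arming the push near each cycle's start.
; On overlap, a non-invincible Wukong gets a horizontal velocity-change impulse scaled by Strenght, then the push disarms until re-armed.
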(event OnComponentBeginOverlap(Sphere)
  (params (OverlappedComponent :type Primitive%20Component%20Object%20Reference) (OtherActor :type Actor%20Object%20Reference) (OtherComp :type Primitive%20Component%20Object%20Reference) (OtherBodyIndex :type Integer) (bFromSweep :type Boolean) (SweepResult :type Hit%20Result%20Structure%20%28by%20ref%29))
  (bind _asbp_wukong (Utilities|Casting|CastToBP_Wukong OtherActor))
  (if (not (Variables|/Game/Core/PlayerCharacter/BP_Wukong.BP_Wukong_C|GetIsInvincible _asbp_wukong))
    (if (Variables|Default|GetCanEject)
      (Physics|AddImpulse (Variables|/Script/Engine.Character|GetCharacterMovement _asbp_wukong) (Math|Vector|MakeVector (.x (* (+ (Math|Vector|GetForwardVector (Math|Rotator|FindLookatRotation (Transformation|GetWorldLocation (Variables|Default|GetSphere)) (Transformation|GetWorldLocation (Variables|/Script/Engine.Character|GetMesh _asbp_wukong)))) "0, 0, 0") (* (Variables|Default|GetStrenght) 1.0))) (.y (* (+ (Math|Vector|GetForwardVector (Math|Rotator|FindLookatRotation (Transformation|GetWorldLocation (Variables|Default|GetSphere)) (Transformation|GetWorldLocation (Variables|/Script/Engine.Character|GetMesh _asbp_wukong)))) "0, 0, 0") (* (Variables|Default|GetStrenght) 1.0))) 0.0) true)
      (Variables|Default|SetCanEject false))))

(event EventBeginPlay)

(event Collision|EventActorBeginOverlap
  (params (OtherActor :type Actor%20Object%20Reference)))

(event EventTick
  (params (DeltaSeconds :type Float%20%28single-precision%29))
  (Components|Sphere|SetSphereRadius (Variables|Default|GetSphere) (Math|Float|Clamp(Float) (* (Math|Float|%(Float) (Variables|Default|GetRatio) 1.0) 4.5e+03) 0.0 3e+03) true)
  (if (<= (Math|Float|%(Float) (Variables|Default|GetRatio) 1.0) 0.01)
    (Variables|Default|SetCanEject true)))

(fn ConstructionScript)