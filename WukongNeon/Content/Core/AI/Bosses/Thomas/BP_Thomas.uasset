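; Boss actor Thomas, which surrounds itself with BP_Crystals and respawns the set whenever its crystal array empties.
; A looping timer spawns crystals up to MaxNumber, offsetting each angle by elapsed time times speed to keep the moving ring evenly spaced.
; Dynamic materials show HP percentage on the mesh, refreshed every tick, and pass the boss's starting position to the landscape floor.
; Death destroys all crystals and the BP_Thomas_Pulse actor before calling the parent.
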(event Custom|SpawnPrism
  (if (< (Utilities|Array|Length (Variables|Default|GetCrystals)) (Variables|Default|GetMaxNumber))
    (bind _returnvalue (Game|SpawnActorfromClass "/Game/Core/AI/Bosses/Thomas/BP_Crystals.BP_Crystals_C" (Math|Transform|MakeTransform "0, 0, 0" "0, 0, 0" "1,1,1") "Undefined" 0 (+ (* (/ 3.6e+02 (Math|Conversions|ToFloat(Integer) (Variables|Default|GetMaxNumber))) (Variables|Default|GetNumero)) (* (Variables|Default|GetChrono) (Variables|Default|GetCrystalSpeed))) 1e+03 (Variables|Default|GetCrystalSpeed) 0))
    (Utilities|Array|Add (Variables|Default|GetCrystals) _returnvalue)
    (Variables|Default|SetNumero (+ (Variables|Default|GetNumero) 1.0))
    (else
      (Utilities|Time|ClearandInvalidateTimerbyHandle (Variables|Default|GetTimer)))))

(event Custom|InitSpawnPrism
  (Variables|Default|SetChrono 0.0)
  (bind _returnvalue (Utilities|Time|SetTimerbyEvent (delegate Custom|SpawnPrism) (Variables|Default|GetTime) true))
  (Variables|Default|SetTimer _returnvalue))

(event Custom|RefreshThomasMat
  (Rendering|Material|SetScalarParameterValue (Variables|Default|GetThomasMat) "HPPercent" (/ (Math|Conversions|ToFloat(Integer) (Variables|Default|Gethp)) (Math|Conversions|ToFloat(Integer) (Variables|Default|GetmaxHp))) :!class /Script/Engine.MaterialInstanceDynamic))

(event EventBeginPlay
  (bind _mesh (Variables|Character|GetMesh))
  (bind _returnvalue (Transformation|GetWorldLocation _mesh))
  (bind _returnvalue_2 (Rendering|Material|CreateDynamicMaterialInstance "/Game/Misc/Materials/Bosses/Thomas/MI_ThomasFloor.MI_ThomasFloor" "None" "None" :!class /Script/Engine.KismetMaterialLibrary))
  (bind _output_get (Variables|Default|SetBossFloorMat _returnvalue_2))
  (Variables|/Script/Landscape.LandscapeProxy|SetLandscapeMaterial (Variables|Default|GetBossFloor) _output_get)
  (CallFunction|InitSpawnPrism)
  (bind _returnvalue_3 (Rendering|Material|CreateDynamicMaterialInstance "/Game/Misc/Materials/Bosses/Thomas/M_Thomas.M_Thomas" "None" "None" :!class /Script/Engine.KismetMaterialLibrary))
  (bind _output_get_2 (Variables|Default|SetThomasMat _returnvalue_3))
  (Rendering|Material|SetMaterial (Variables|Character|GetMesh) 0 _output_get_2)
  (Rendering|Material|SetVectorParameterValue (Variables|Default|GetBossFloorMat) "Position" (Utilities|Struct|MakeLinearColor (.x _returnvalue) (.y _returnvalue) (.z _returnvalue) 1.0) :!class /Script/Engine.MaterialInstanceDynamic))

(event EventTick
  (params (DeltaSeconds :type Float%20%28single-precision%29))
  (Variables|Default|SetChrono (+ DeltaSeconds (Variables|Default|GetChrono)))
  (Utilities|FlowControl|Sequence
    (:then_0
      (if (and (== (Utilities|Array|Length (Variables|Default|GetCrystals)) 0) (not (Utilities|Time|IsTimerActivebyHandle (Variables|Default|GetTimer))))
        (CallFunction|InitSpawnPrism)))
    (:then_1
      (CallFunction|RefreshThomasMat))))

(fn ConstructionScript
  (bind _returnvalue (Rendering|Material|CreateDynamicMaterialInstance "/Game/Misc/Materials/Bosses/Thomas/M_Thomas.M_Thomas" "None" "None" :!class /Script/Engine.KismetMaterialLibrary))
  (Variables|Default|SetThomasMat _returnvalue)
  (CallFunction|RefreshThomasMat))

(fn Death
  (bind _outactors (Actor|GetAllActorsOfClass "/Game/Core/AI/Bosses/Thomas/BP_Crystals.BP_Crystals_C"))
  (Actor|DestroyActor _outactors)
  (bind _returnvalue (Actor|GetActorOfClass "/Game/Core/AI/Bosses/Thomas/BP_Thomas_Pulse.BP_Thomas_Pulse_C"))
  (Actor|DestroyActor _returnvalue)
  (|CallParentFunction))