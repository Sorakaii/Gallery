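; Room camera actor that, while activated, turns smoothly to follow the ThirdPersonCharacter_CameraTest player.
; Tick interpolates rotation toward the player and, beyond a fixed horizontal distance, narrows field of view as distance grows between DistanceMin and DistanceMax.
; The changeCamera event blends the player controller's view to this actor and registers it as the player's camera.
; The construction script draws persistent debug cylinders showing both distance radii.
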(event Custom|changeCamera
  (Game|Player|SetViewTargetwithBlend (Game|GetPlayerController 0) self 1.0 "VTBlend_EaseInOut" 1.0 true)
  (Variables|/Game/Blueprints/Player/ThirdPersonCharacter_CameraTest.ThirdPersonCharacter_CameraTest_C|Setcamera (Variables|Default|GetPlayer) self))

(event EventBeginPlay
  (bind _returnvalue (Actor|GetActorOfClass "/Game/Blueprints/Player/ThirdPersonCharacter_CameraTest.ThirdPersonCharacter_CameraTest_C"))
  (Variables|Default|SetPlayer _returnvalue))

(event Collision|EventActorBeginOverlap
  (params (OtherActor :type Actor%20Object%20Reference)))

(event EventTick
  (params (DeltaSeconds :type Float%20%28single-precision%29))
  (bind _returnvalue (Transformation|GetActorLocation))
  (bind _camera (Variables|Default|GetCamera))
  (bind _player (Variables|Default|GetPlayer))
  (bind _returnvalue_2 (Transformation|GetActorLocation _player))
  (if (Variables|Default|GetActivated)
    (Transformation|SetActorRotation (Math|Interpolation|RInterpTo (Transformation|GetActorRotation) (Math|Rotator|FindLookatRotation (Transformation|GetActorLocation) (Transformation|GetActorLocation (Variables|Default|GetPlayer))) (Utilities|Time|GetWorldDeltaSeconds) 1.0))
    (Variables|Default|SetdistancePlayerCamera (Math|Vector|VectorLength (Math|Vector|VectorGetAbs (- (Math|Vector|MakeVector (.x _returnvalue_2) (.y _returnvalue_2) 0.0) (Math|Vector|MakeVector (.x _returnvalue) (.y _returnvalue) 0.0)))))
    (if (> (Variables|Default|GetdistancePlayerCamera) 2e+03)
      (Camera|SetFieldOfView _camera (Math|Interpolation|FInterpTo (Variables|/Script/Engine.CameraComponent|GetFieldOfView _camera) (Math|Float|MapRangeClamped (Variables|Default|GetdistancePlayerCamera) (Variables|Default|GetDistanceMin) (Variables|Default|GetDistanceMax) 9e+01 35.0) (Utilities|Time|GetWorldDeltaSeconds) 1.2)))))

(fn ConstructionScript
  (bind _returnvalue (Transformation|GetActorLocation))
  (bind _distancemin (Variables|Default|GetDistanceMin))
  (bind _distancemax (Variables|Default|GetDistanceMax))
  (Rendering|Debug|FlushPersistentDebugLines)
  (Class|KismetSystemLibrary|DrawDebugCylinder (Math|Vector|MakeVector (.x _returnvalue) (.y _returnvalue) 0.0) (Math|Vector|MakeVector (.x _returnvalue) (.y _returnvalue) 3e+03) _distancemin (Math|Float|Truncate (/ _distancemin 5e+01)) "(R=0.000000,G=0.239841,B=1.000000,A=1.000000)" 1.0000000150474662e+29 0.0)
  (Class|KismetSystemLibrary|DrawDebugCylinder (Math|Vector|MakeVector (.x _returnvalue) (.y _returnvalue) 0.0) (Math|Vector|MakeVector (.x _returnvalue) (.y _returnvalue) 3e+03) _distancemax (Math|Float|Truncate (/ _distancemax 5e+01)) "(R=1.000000,G=0.000000,B=0.053850,A=1.000000)" 1.0000000150474662e+29 0.0))