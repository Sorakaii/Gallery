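; Trigger volume that toggles the third-person test character between its own camera and a linked room camera.
; Each time the character leaves the box, it checks the Activated flag on AfterTriggerCamera to choose the direction of the swap.
; Switching to the room camera disables the spring arm's pawn control rotation and calls ChangeCamera.
; Switching back restores that rotation, returns to the player camera and clears the input-change flags.
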(event OnComponentEndOverlap(Box)
  (params (OverlappedComponent :type Primitive%20Component%20Object%20Reference) (OtherActor :type Actor%20Object%20Reference) (OtherComp :type Primitive%20Component%20Object%20Reference) (OtherBodyIndex :type Integer))
  (bind _aftertriggercamera (Variables|Default|GetAfterTriggerCamera))
  (bind _asthird_person_character_camera_test (Utilities|Casting|CastToThirdPersonCharacter_CameraTest OtherActor))
  (Variables|Default|SetPlayer _asthird_person_character_camera_test)
  (if (not (Variables|/Game/Blueprints/Camera/RoomCamera/BP_Camera.BP_Camera_C|GetActivated (Variables|Default|GetAfterTriggerCamera)))
    (Variables|/Script/Engine.SpringArmComponent|SetbUsePawnControlRotation (Actor|GetComponentbyClass (Variables|Default|GetPlayer) "/Script/Engine.SpringArmComponent") false)
    (Default|ChangeCamera (Variables|Default|GetAfterTriggerCamera))
    (Variables|/Game/Blueprints/Camera/RoomCamera/BP_Camera.BP_Camera_C|SetActivated _aftertriggercamera true)
    (else
      (Variables|/Script/Engine.SpringArmComponent|SetbUsePawnControlRotation (Actor|GetComponentbyClass (Variables|Default|GetPlayer) "/Script/Engine.SpringArmComponent") true)
      (Default|GoBacktoPlayerCamera (Variables|Default|GetPlayer) 1.0)
      (Variables|/Game/Blueprints/Camera/RoomCamera/BP_Camera.BP_Camera_C|SetActivated _aftertriggercamera false)
      (Variables|/Game/Blueprints/Player/ThirdPersonCharacter_CameraTest.ThirdPersonCharacter_CameraTest_C|SetchangeInputX (Variables|Default|GetPlayer) false)
      (Variables|/Game/Blueprints/Player/ThirdPersonCharacter_CameraTest.ThirdPersonCharacter_CameraTest_C|SetchangeInputY (Variables|Default|GetPlayer) false))))

(event EventBeginPlay)

(event Collision|EventActorBeginOverlap
  (params (OtherActor :type Actor%20Object%20Reference)))

(event EventTick
  (params (DeltaSeconds :type Float%20%28single-precision%29)))

(fn ConstructionScript)