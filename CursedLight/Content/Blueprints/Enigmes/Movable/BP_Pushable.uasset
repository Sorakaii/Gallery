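; Puzzle object that an ALS character can push, with a box overlap toggling the character's CanPush flag.
; The construction script generates inward-facing push transforms on a square perimeter sized from the mesh bounds, shown as arrows.
; Interact passes the nearest transform to the character's PushComponent to lerp the player there, or otherwise ends the push.
; TraceForObstacle offers a box-trace check offset along the character's facing.
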(event OnComponentBeginOverlap(XBox)
  (params (OverlappedComponent :type Primitive%20Component%20Object%20Reference) (OtherActor :type Actor%20Object%20Reference) (OtherComp :type Primitive%20Component%20Object%20Reference) (OtherBodyIndex :type Integer) (bFromSweep :type Boolean) (SweepResult :type Hit%20Result%20Structure%20%28by%20ref%29))
  (bind _asals_anim_man_character_bp (Utilities|Casting|CastToALS_AnimMan_CharacterBP OtherActor))
  (Variables|/Game/Blueprints/Player/ThirdPersonCharacter.ThirdPersonCharacter_C|SetCanPush _asals_anim_man_character_bp true))

(event OnComponentEndOverlap(XBox)
  (params (OverlappedComponent :type Primitive%20Component%20Object%20Reference) (OtherActor :type Actor%20Object%20Reference) (OtherComp :type Primitive%20Component%20Object%20Reference) (OtherBodyIndex :type Integer))
  (bind _asals_anim_man_character_bp (Utilities|Casting|CastToALS_AnimMan_CharacterBP OtherActor))
  (Variables|/Game/Blueprints/Player/ThirdPersonCharacter.ThirdPersonCharacter_C|SetCanPush _asals_anim_man_character_bp false))

(event EventBeginPlay)

(event Collision|EventActorBeginOverlap
  (params (OtherActor :type Actor%20Object%20Reference)))

(event EventTick
  (params (DeltaSeconds :type Float%20%28single-precision%29)))

(event EventInteract
  (params (Player :type Third%20Person%20Character%20Object%20Reference))
  (if (and (Variables|/Game/Blueprints/Player/ThirdPersonCharacter.ThirdPersonCharacter_C|GetCanPush Player) (not (Variables|/Game/Blueprints/Player/ThirdPersonCharacter.ThirdPersonCharacter_C|GetPushing Player)))
    (bind _asals_anim_man_character_bp (Utilities|Casting|CastToALS_AnimMan_CharacterBP Player))
    (bind _output_get (Variables|Default|SetCharacterREF _asals_anim_man_character_bp))
    (Variables|Default|SetCharacterPrevTransform (Transformation|GetActorTransform _output_get))
    (bind _bestindex (CallFunction|FindClosestPushTransformIndex (Math|Conversions|ToVector2D(Vector) (Transformation|GetActorLocation (Variables|Default|GetCharacterREF))) (Variables|/Game/Blueprints/Enigmes/Movable/PushComponent.PushComponent_C|GetPushRange (Variables|/Game/Blueprints/Player/ThirdPersonCharacter.ThirdPersonCharacter_C|GetPushComponent (Variables|Default|GetCharacterREF)))))
    (bind _output_get_2 (Variables|Default|SetClosestPushTransform (Math|Transform|ComposeTransforms (Utilities|Array|Get(acopy) (Variables|Default|GetPushTransforms) _bestindex) (Transformation|GetActorTransform))))
    (Default|LerpPlayertoTransform (Variables|/Game/Blueprints/Player/ThirdPersonCharacter.ThirdPersonCharacter_C|GetPushComponent (Variables|Default|GetCharacterREF)) _output_get_2 self)
    (else
      (bind _characterref (Variables|Default|GetCharacterREF)
        (:then
          (Default|EndPush (Variables|/Game/Blueprints/Player/ThirdPersonCharacter.ThirdPersonCharacter_C|GetPushComponent _characterref)))
        (:else)))))

(fn ConstructionScript
  (bind _staticmesh (Variables|Default|GetStaticMesh))
  (bind _sphereradius (Collision|GetComponentBounds _staticmesh))
  (bind _returnvalue (/ _sphereradius 7.5))
  (Variables|Default|SetRadius (* (.SphereRadius (Collision|GetComponentBounds (Variables|Default|GetStaticMesh))) (/ (Math|Trig|GetPI) 2.0)))
  (Components|Box|SetBoxExtent (Variables|Default|GetXBox) (* (Math|Vector|MakeVector 1.0 1.0 1.0) 132.5) true)
  (Utilities|Array|Clear (Variables|Default|GetPushTransforms))
  (for _index (range -5 5)
    (for _index_2 (range -5 5)
      (if (Math|Boolean|ORBoolean (== (Math|Conversions|ToFloat(Integer) _index) 5.0) (== (Math|Conversions|ToFloat(Integer) _index) -5.0) (== (Math|Conversions|ToFloat(Integer) _index_2) 5.0) (== (Math|Conversions|ToFloat(Integer) _index_2) -5.0))
        (Utilities|Array|Add (Variables|Default|GetPushTransforms) (Math|Transform|MakeTransform (Math|Vector|MakeVector (* (Math|Conversions|ToFloat(Integer) _index_2) _returnvalue) (* _returnvalue (Math|Conversions|ToFloat(Integer) _index)) 0.0) (Math|Rotator|FindLookatRotation (Math|Vector|MakeVector (* (Math|Conversions|ToFloat(Integer) _index_2) _returnvalue) (* _returnvalue (Math|Conversions|ToFloat(Integer) _index)) 0.0) (Math|Vector|MakeVector 0.0 0.0 0.0)) "1.000000,1.000000,1.000000")))))
  (for _array_element (Variables|Default|GetPushTransforms)
    (AddComponent|AddArrowComponent false _array_element)))

(fn FindClosestPushTransformIndex
  (params (CharacterLocation :type Vector%202D%20Structure) (PushRange :type Float%20%28double-precision%29))
  (for (_array_element _array_index) (Variables|Default|GetPushTransforms)
    (LocalVariables|SetcurrentTransformIndex _array_index)
    (bind _output_get (LocalVariables|SetcurrentDistanceSq (Class|KismetMathLibrary|DistanceSquared2D (Math|Conversions|ToVector2D(Vector) (Math|Transform|TransformLocation (Transformation|GetActorTransform) (.location _array_element))) CharacterLocation)))
    (if (< _output_get (Math|Float|Square PushRange))
      (if (or (< (LocalVariables|GetcurrentDistanceSq) (LocalVariables|GetclosestDistanceSq)) (< (LocalVariables|GetcurrentTransformIndex) 0))
        (LocalVariables|SetclosestTransformIndex (LocalVariables|GetcurrentTransformIndex))
        (LocalVariables|SetclosestDistanceSq (LocalVariables|GetcurrentDistanceSq)))))
  (return (LocalVariables|GetclosestTransformIndex)))

(fn TraceforObstacle
  (params (Distance :type Float%20%28single-precision%29) (DrawDebugType :type EDrawDebugTrace%20Enum :default "None") (ActorsToIgnore :type Array%20of%20Actor%20Object%20References))
  (bind _linetracescene (Variables|Default|GetLineTraceScene))
  (bind _characterref (Variables|Default|GetCharacterREF))
  (bind _staticmesh (Variables|Default|GetStaticMesh))
  (bind _returnvalue (Transformation|GetWorldLocation _linetracescene))
  (bind _returnvalue_2 (Math|Vector|GetUpVector _staticmesh))
  (bind _returnvalue_3 (Transformation|GetActorForwardVector _characterref))
  (bind _returnvalue_4 (* _returnvalue_3 Distance))
  (bind _returnvalue_5 (* _returnvalue_2 5e+01))
  (bind _returnvalue_6 (+ _returnvalue _returnvalue_4))
  (bind _returnvalue_7 (+ _returnvalue_6 _returnvalue_5))
  (bind _outhit (Collision|BoxTraceByChannel _returnvalue_7 _returnvalue_7 "10.000000,75.000000,16.000000" (Transformation|GetActorRotation (Variables|Default|GetCharacterREF)) "TraceTypeQuery1" false ActorsToIgnore DrawDebugType))
  (return _outhit (.bBlockingHit (Collision|BreakHitResult _outhit))))