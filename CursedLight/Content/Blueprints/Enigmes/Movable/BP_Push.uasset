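; Pushable puzzle object that the player shoves along a spline, from its start to input key 1.
; The first Interact snaps the player to the push point, attaches them to the mesh and locks movement; later presses advance a target key in small steps.
; Tick eases the mesh's XY toward that key, blends the ALS push stride while moving, and prints animation debug.
; Interacting at the end releases the player.
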(event OnComponentBeginOverlap(Box)
  (params (OverlappedComponent :type Primitive%20Component%20Object%20Reference) (OtherActor :type Actor%20Object%20Reference) (OtherComp :type Primitive%20Component%20Object%20Reference) (OtherBodyIndex :type Integer) (bFromSweep :type Boolean) (SweepResult :type Hit%20Result%20Structure%20%28by%20ref%29))
  (bind _playerref (Variables|Default|GetPlayerRef))
  ;[0.8104 1 0] Overlap
  (if (== OtherActor _playerref)
    (Variables|/Game/Blueprints/Player/ThirdPersonCharacter.ThirdPersonCharacter_C|SetCanPush _playerref true)))

(event EventBeginPlay
  ;[0 1 0.2733] BeginPlay
  (bind _asthird_person_character (Utilities|Casting|CastToThirdPersonCharacter (Game|GetPlayerCharacter 0)))
  (Variables|Default|SetPlayerRef _asthird_person_character))

(event EventInteract
  (params (Player :type Third%20Person%20Character%20Object%20Reference))
  (bind _playerref (Variables|Default|GetPlayerRef))
  (bind _pushpoint (Variables|Default|GetPushPoint))
  (bind _returnvalue (Transformation|GetWorldLocation _pushpoint))
  ;[0.06709 1 0] Interact for push
  (if (>= (Variables|Default|GetIn%20Key) 1.0)
    (CallFunction|ResetPush)
    (elif (and (Variables|/Game/Blueprints/Player/ThirdPersonCharacter.ThirdPersonCharacter_C|GetCanPush Player) (not (Variables|/Game/Blueprints/Player/ThirdPersonCharacter.ThirdPersonCharacter_C|GetPushing Player)))
      (bind _asabp_main_chara_child_als (Utilities|Casting|CastToABP_MainChara_ChildALS (Components|SkeletalMesh|GetAnimInstance (Variables|/Script/Engine.Character|GetMesh (Variables|Default|GetPlayerRef)))))
      (Variables|Default|SetAnimInstRef _asabp_main_chara_child_als)
      (Variables|/Game/Characters/ALS/ALS_AnimBP.ALS_AnimBP_C|SetisPushing (Variables|Default|GetAnimInstRef) true)
      (Components|MoveComponentTo (Variables|/Script/Engine.Character|GetCapsuleComponent _playerref) (Math|Vector|MakeVector (.x _returnvalue) (.y _returnvalue) (.z (Transformation|GetActorLocation _playerref))) "0.000000,-90.000000,0.000000" false false 0.2 false)
      (Transformation|AttachComponentToComponent (Variables|Default|GetPlayerRef) (Variables|Default|GetStaticMesh) "None" "KeepWorld" "KeepWorld" "KeepWorld" true)
      (Variables|/Game/Blueprints/Player/ThirdPersonCharacter.ThirdPersonCharacter_C|SetPushing (Variables|Default|GetPlayerRef) true)
      (Default|SetMovementCapabilities (Variables|Default|GetPlayerRef) false false false)
      (elif (< (- (Variables|Default|Getcount) (Variables|Default|GetIn%20Key)) 0.05)
        (Variables|Default|Setcount (+ (Variables|Default|Getcount) 0.05))))))

(event EventTick
  (params (DeltaSeconds :type Float%20%28single-precision%29))
  (bind _spline (Variables|Default|GetSpline))
  (bind _in_key (Variables|Default|GetIn%20Key))
  (bind _returnvalue (Class|SplineComponent|GetLocationatSplineInputKey _spline _in_key "Local"))
  ;[0 0.8706 1] Tick
  (Utilities|FlowControl|Sequence
    (:then_0
      ;;[1 0 0.8023] Debug
      (Development|PrintString (Utilities|String|EnumtoString (Variables|/Game/Characters/ALS/ALS_AnimBP.ALS_AnimBP_C|GetGroundedEntryState (.AsALS%20Anim%20BP (Utilities|Casting|CastToALS_AnimBP (Components|SkeletalMesh|GetAnimInstance (Variables|/Script/Engine.Character|GetMesh (Variables|Default|GetPlayerRef))))))) true true "(R=0.000000,G=0.660000,B=1.000000,A=1.000000)" 0.0)
      (Development|PrintString (Utilities|GetDisplayName (Animation|GetCurrentMontage (Variables|Default|GetPlayerRef) :!class /Script/Engine.Character)) true true "(R=0.000000,G=0.660000,B=1.000000,A=1.000000)" 0.0)
      (Development|PrintString (Utilities|String|ToString(Float) (Class|SkeletalMeshComponent|GetPosition (Variables|/Script/Engine.Character|GetMesh (Variables|Default|GetPlayerRef)))) true true "(R=1.000000,G=0.000000,B=0.780794,A=1.000000)" 0.0))
    (:then_1
      ;;[0 1 0.1467] Set position mesh along spline
      (CallFunction|SetStrideCustPush DeltaSeconds)
      (CallFunction|SetinKey DeltaSeconds)
      (Transformation|SetRelativeLocationAndRotation (Variables|Default|GetStaticMesh) (Math|Vector|MakeVector (.x _returnvalue) (.y _returnvalue) 0.0) "0, 0, 0" false false))))

(fn ConstructionScript
  (bind _spline (Variables|Default|GetSpline))
  (Transformation|SetRelativeLocationAndRotation (Variables|Default|GetStaticMesh) (Spline|GetLocationatDistanceAlongSpline _spline 0.0 "Local") (Spline|GetRotationatDistanceAlongSpline _spline 0.0 "Local") false false))

(fn SetStrideCustPush
  (params (DeltaTime :type Float%20%28single-precision%29))
  (bind _animinstref (Variables|Default|GetAnimInstRef)
    (:then
      (Variables|/Game/Characters/ALS/ALS_AnimBP.ALS_AnimBP_C|SetStrideCustomPush _animinstref (Math|Interpolation|FInterptoConstant (Variables|/Game/Characters/ALS/ALS_AnimBP.ALS_AnimBP_C|GetStrideCustomPush (Variables|Default|GetAnimInstRef)) (Math|Float|SelectFloat 0.0 1.0 (Math|Float|NearlyEqual(Float) (Variables|Default|Getcount) (Variables|Default|GetIn%20Key) 0.0001)) DeltaTime 5.0)))
    (:else)))

(fn SetinKey
  (params (DeltaTime :type Float%20%28double-precision%29))
  (Variables|Default|SetIn%20Key (Math|Interpolation|FInterptoConstant (Variables|Default|GetIn%20Key) (Variables|Default|Getcount) DeltaTime 0.1)))

(fn ResetPush
  (bind _playerref (Variables|Default|GetPlayerRef))
  (Variables|/Game/Characters/ALS/ALS_AnimBP.ALS_AnimBP_C|SetisPushing (Variables|Default|GetAnimInstRef) false)
  (Variables|/Game/Blueprints/Player/ThirdPersonCharacter.ThirdPersonCharacter_C|SetPushing (Variables|Default|GetPlayerRef) false)
  (Default|SetMovementCapabilities _playerref true true true)
  (Transformation|DetachFromActor _playerref "KeepWorld" "KeepWorld" "KeepWorld"))