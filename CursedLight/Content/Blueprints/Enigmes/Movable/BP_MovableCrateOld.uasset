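; Legacy movable crate for puzzles, meant to be pushed by the player, but its push logic is disconnected.
; The construction script adds an arrow component for each push transform.
; Interact only validates the player and its PushComponent, calling an empty PushFailed otherwise.
; Unreachable nodes hold the old player snapping with floor, room and wall traces, plus a BeginPush call noted as broken; FindClosestPushTransformIndex is empty.
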(event EventBeginPlay)

(event Collision|EventActorBeginOverlap
  (params (OtherActor :type Actor%20Object%20Reference)))

(event EventTick
  (params (DeltaSeconds :type Float%20%28single-precision%29)))

(event EventInteract
  (params (Player :type Third%20Person%20Character%20Object%20Reference))
  (CallFunction|HandleInteraction Player))

(fn ConstructionScript
  (for _array_element (Variables|Default|GetPushTransforms)
    (AddComponent|AddArrowComponent false _array_element)))

(fn HandleInteraction
  (params (Player :type Third%20Person%20Character%20Object%20Reference))
  (Utilities|IsValid Player
    (:Is%20Valid
      (bind _output_get (LocalVariables|SetPushComponent (Actor|GetComponentbyClass Player "/Game/Blueprints/Enigmes/Movable/PushComponent.PushComponent_C")))
      (Utilities|IsValid _output_get
        (:Is%20Not%20Valid
          (Utilities|PushFailed "Character doesn't have push component"))))
    (:Is%20Not%20Valid
      (Utilities|PushFailed "Character is invalid"))))

(fn FindClosestPushTransformIndex
  (params (CharacterLocation :type Vector%202D%20Structure) (PushRange :type Float%20%28double-precision%29)))