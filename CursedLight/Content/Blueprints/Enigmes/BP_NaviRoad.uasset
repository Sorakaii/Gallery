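; Wall puzzle where the player, on interacting, steers a spawned BP_NaviPuzzle through three roads of rising difficulty to open the doors of a linked wall.
; Interaction locks the camera into a waiting cinematic; chained timelines slide each road in and scale the goal.
; Each goal overlap advances Index and swaps roads, with the last triggering the doors and restoring camera control.
; Tick only debug-prints; the block-moving logic never runs.
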(event OnComponentBeginOverlap(Sphere)
  (params (OverlappedComponent :type Primitive%20Component%20Object%20Reference) (OtherActor :type Actor%20Object%20Reference) (OtherComp :type Primitive%20Component%20Object%20Reference) (OtherBodyIndex :type Integer) (bFromSweep :type Boolean) (SweepResult :type Hit%20Result%20Structure%20%28by%20ref%29))
  (bind _wallref (Variables|Default|GetWallRef))
  (bind _playerref (Variables|Default|GetPlayerRef))
  (bind _asbp_navi_puzzle (Utilities|Casting|CastToBP_NaviPuzzle OtherActor))
  (Utilities|FlowControl|DoOnce false
    (:Completed
      (bind _result (Math|Integer|IncrementInt (Variables|Default|GetIndex))
        (:%20%20
          (if (== _result 3)
            (Variables|/Script/Engine.NavMovementComponent|SetNavAgentProps (Variables|/Script/Engine.Character|GetCharacterMovement _playerref) (Variables|/Game/Blueprints/Player/ThirdPersonCharacter.ThirdPersonCharacter_C|GetinitialMovementCapabilities _playerref))
            (Rendering|SetVisibility (Variables|/Game/Blueprints/Navi/BP_NaviPawn.BP_NaviPawn_C|GetCollision (Variables|/Game/Blueprints/Player/ThirdPersonCharacter.ThirdPersonCharacter_C|GetnaviRef (Variables|Default|GetPlayerRef))) true true)
            (Default|NextWaitingCinematicCamera (Variables|Default|GetcamManagerRef))
            (Default|MakeNotTargetable (Variables|Default|GetC_Interactible))
            (Utilities|FlowControl|Delay 1.0)
            (Default|MoveDoors _wallref)
            (Collision|SetCollisionEnabled (Variables|/Game/Blueprints/Enigmes/BP_Wall.BP_Wall_C|GetWallCollision _wallref) "NoCollision")
            (Utilities|FlowControl|Delay 1.0)
            (Default|NextWaitingCinematicCamera (Variables|Default|GetcamManagerRef))
            (Variables|/Game/Blueprints/Player/ThirdPersonCharacter.ThirdPersonCharacter_C|SetcanMoveCamera (Variables|Default|GetPlayerRef) true)
            (Utilities|FlowControl|Delay 0.1)
            (Actor|DestroyActor _asbp_navi_puzzle)
            (else
              (Variables|/Game/Blueprints/Navi/BP_NaviPuzzle.BP_NaviPuzzle_C|SetcanMove (Variables|Default|GetNaviPuzzleRef) false)
              (CallFunction|ChangePosition))))))))

(event InteractwithOwner(C_Interactible)
  (bind _goal (Variables|Default|GetGoal))
  (bind _roadsimple (Variables|Default|GetRoadSimple))
  (bind _wallref (Variables|Default|GetWallRef))
  (bind _camera (Variables|Default|GetCamera))
  (bind _relativelocation (Variables|/Script/Engine.SceneComponent|GetRelativeLocation _roadsimple))
  (bind _cinematiccam (Variables|/Game/Blueprints/Enigmes/BP_Wall.BP_Wall_C|GetCinematicCam _wallref))
  (Utilities|FlowControl|DoOnce false
    (:Completed
      (Rendering|SetVisibility (Variables|/Game/Blueprints/Navi/BP_NaviPawn.BP_NaviPawn_C|GetCollision (Variables|/Game/Blueprints/Player/ThirdPersonCharacter.ThirdPersonCharacter_C|GetnaviRef (Variables|Default|GetPlayerRef))) false true)
      (bind _returnvalue (Game|SpawnActorfromClass "/Game/Blueprints/Navi/BP_NaviPuzzle.BP_NaviPuzzle_C" (Math|Transform|MakeTransform (Transformation|GetWorldLocation (Variables|Default|GetSpawn)) "0,90.000000, 0" "1.000000,1.000000,1.000000") "AlwaysSpawn" 0 self 0 0))
      (Variables|Default|SetNaviPuzzleRef _returnvalue)
      (Variables|/Game/Blueprints/Navi/BP_NaviPuzzle.BP_NaviPuzzle_C|SetIsWallPuzzle (Variables|Default|GetNaviPuzzleRef) true)
      (Variables|/Game/Blueprints/Player/ThirdPersonCharacter.ThirdPersonCharacter_C|SetcanMoveCamera (Variables|Default|GetPlayerRef) false)
      (Default|StartPuzzle (Variables|Default|GetNaviPuzzleRef))
      (Default|WaitingCinematic (Variables|Default|GetcamManagerRef) (Utilities|Array|MakeArray (Math|Transform|MakeTransform (Transformation|GetWorldLocation _camera) (Transformation|GetWorldRotation _camera) "1.000000,1.000000,1.000000") (Math|Transform|MakeTransform (Transformation|GetWorldLocation _cinematiccam) (Transformation|GetWorldRotation _cinematiccam) "1.000000,1.000000,1.000000")))
      (Default|MakeNotTargetable (Variables|Default|GetC_Interactible))
      (Variables|Default|SetRelativeLocationBase _relativelocation)
      (Variables|Default|SetRelativeLocationEnd (+ _relativelocation "0,67.000000,0"))
      (bind _location (Timeline|Timeline0Location PlayFromStart)
        (:Update
          (Transformation|SetRelativeLocation _roadsimple (Math|Vector|Lerp(Vector) (Variables|Default|GetRelativeLocationBase) (Variables|Default|GetRelativeLocationEnd) _location) false false))
        (:Finished
          (Transformation|SetWorldLocation (Variables|Default|GetGoal) (Utilities|Array|Get(acopy) (Variables|Default|GetLocationArray) (Variables|Default|GetIndex)) false false)
          (bind _scale (Timeline|TimelineScaleStart PlayFromStart)
            (:Update
              (Transformation|SetWorldScale3D _goal (Math|Vector|Lerp(Vector) (Transformation|GetWorldScale _goal) "0.250000,0.250000,0.250000" _scale)))
            (:Finished
              (Variables|/Game/Blueprints/Navi/BP_NaviPuzzle.BP_NaviPuzzle_C|SetcanMove (Variables|Default|GetNaviPuzzleRef) true))))))))

(event Custom|ChangePosition
  (bind _goal (Variables|Default|GetGoal))
  (bind _goal_2 (Variables|Default|GetGoal))
  (bind _goal_3 (Variables|Default|GetGoal))
  (bind _goal_4 (Variables|Default|GetGoal))
  (bind _roadmedium (Variables|Default|GetRoadMedium))
  (bind _roadhard (Variables|Default|GetRoadHard))
  (bind _relativelocation (Variables|/Script/Engine.SceneComponent|GetRelativeLocation _roadhard))
  (bind _relativelocation_2 (Variables|/Script/Engine.SceneComponent|GetRelativeLocation _roadmedium))
  (switch int (Variables|Default|GetIndex)
    (:1
      (bind _scale (Timeline|Scale0Timeline PlayFromStart)
        (:Update
          (Transformation|SetWorldScale3D _goal_3 (Math|Vector|Lerp(Vector) (Transformation|GetWorldScale _goal_3) "0, 0, 0" _scale)))
        (:Finished
          (Transformation|SetWorldLocation (Variables|Default|GetSphere) (Utilities|Array|Get(acopy) (Variables|Default|GetLocationArray) (Variables|Default|GetIndex)) false false)
          (bind _location (Timeline|TimelineLocationChangeStart PlayFromStart)
            (:Update
              (Transformation|SetRelativeLocation (Variables|Default|GetRoadSimple) (Math|Vector|Lerp(Vector) (Variables|Default|GetRelativeLocationEnd) (Variables|Default|GetRelativeLocationBase) _location) false false))
            (:Finished
              (Variables|Default|SetRelativeLocationBase _relativelocation_2)
              (Variables|Default|SetRelativeLocationEnd (+ _relativelocation_2 "0,67.000000,0"))
              (bind _location_2 (Timeline|TimelineLocationChangeEnd PlayFromStart)
                (:Update
                  (Transformation|SetRelativeLocation (Variables|Default|GetRoadMedium) (Math|Vector|Lerp(Vector) (Variables|Default|GetRelativeLocationBase) (Variables|Default|GetRelativeLocationEnd) _location_2) false false))
                (:Finished
                  (bind _scale_2 (Timeline|Scale1Timeline PlayFromStart)
                    (:Update
                      (Transformation|SetWorldScale3D _goal_4 (Math|Vector|Lerp(Vector) (Transformation|GetWorldScale _goal_4) "0.250000,0.250000,0.250000" _scale_2)))
                    (:Finished
                      (CallFunction|ResetDoOnce)
                      (Variables|/Game/Blueprints/Navi/BP_NaviPuzzle.BP_NaviPuzzle_C|SetcanMove (Variables|Default|GetNaviPuzzleRef) true))))))))))
    (:2
      (bind _scale_3 (Timeline|Timeline_0 PlayFromStart)
        (:Update
          (Transformation|SetWorldScale3D _goal (Math|Vector|Lerp(Vector) (Transformation|GetWorldScale _goal) "0, 0, 0" _scale_3)))
        (:Finished
          (Transformation|SetWorldLocation (Variables|Default|GetSphere) (Utilities|Array|Get(acopy) (Variables|Default|GetLocationArray) (Variables|Default|GetIndex)) false false)
          (bind _location_3 (Timeline|Timeline_2 PlayFromStart)
            (:Update
              (Transformation|SetRelativeLocation (Variables|Default|GetRoadMedium) (Math|Vector|Lerp(Vector) (Variables|Default|GetRelativeLocationEnd) (Variables|Default|GetRelativeLocationBase) _location_3) false false))
            (:Finished
              (Variables|Default|SetRelativeLocationBase _relativelocation)
              (Variables|Default|SetRelativeLocationEnd (+ _relativelocation "0,67.000000,0"))
              (bind _location_4 (Timeline|Timeline_3 PlayFromStart)
                (:Update
                  (Transformation|SetRelativeLocation (Variables|Default|GetRoadHard) (Math|Vector|Lerp(Vector) (Variables|Default|GetRelativeLocationBase) (Variables|Default|GetRelativeLocationEnd) _location_4) false false))
                (:Finished
                  (bind _scale_4 (Timeline|Timeline_1 PlayFromStart)
                    (:Update
                      (Transformation|SetWorldScale3D _goal_2 (Math|Vector|Lerp(Vector) (Transformation|GetWorldScale _goal_2) "0.250000,0.250000,0.250000" _scale_4)))
                    (:Finished
                      (CallFunction|ResetDoOnce)
                      (Variables|/Game/Blueprints/Navi/BP_NaviPuzzle.BP_NaviPuzzle_C|SetcanMove (Variables|Default|GetNaviPuzzleRef) true))))))))))))

(event Custom|ResetDoOnce
  (bind _wallref (Variables|Default|GetWallRef))
  (bind _playerref (Variables|Default|GetPlayerRef))
  (Utilities|FlowControl|DoOnce false) ; enters at Reset
)

(event EventBeginPlay
  (bind _asthird_person_character (Utilities|Casting|CastToThirdPersonCharacter (Game|GetPlayerCharacter 0)))
  (Variables|Default|SetPlayerRef _asthird_person_character)
  (Variables|Default|SetLocationArray (Utilities|Array|MakeArray (Transformation|GetWorldLocation (Variables|Default|GetGLocation)) (Transformation|GetWorldLocation (Variables|Default|GetGLocation2)) (Transformation|GetWorldLocation (Variables|Default|GetGLocation3))))
  (bind _asals_player_camera_manager (Utilities|Casting|CastToALS_PlayerCameraManager (Game|GetPlayerCameraManager 0)))
  (Variables|Default|SetcamManagerRef _asals_player_camera_manager)
  (Variables|Default|SetBlockArray (Utilities|Array|MakeArray 0 (Variables|Default|GetBlock2) (Variables|Default|GetBlock3) (Variables|Default|GetBlock4) (Variables|Default|GetBlock5) (Variables|Default|GetBlock6))))

(event Collision|EventActorBeginOverlap
  (params (OtherActor :type Actor%20Object%20Reference))
  ;[1 1 1] old
)

(event EventTick
  (params (DeltaSeconds :type Float%20%28single-precision%29))
  (Development|PrintString (Utilities|String|ToString(Integer) (Variables|Default|GetNumBlock)) true true "(R=0.000000,G=1.000000,B=0.547668,A=1.000000)" 0.0))

(fn ConstructionScript
  (Default|CreateComponents (Variables|Default|GetSC_BoxAndMesh)))