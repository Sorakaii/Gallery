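; BP_SwitchSimon is an interactible switch for what appears to be a Simon-style puzzle, starting untargetable unless Debug is set.
; ActivateSwitch, skipped in Debug, disables targeting, lights the flakes' material and spins them on a timeline.
; Player interaction reports the switch to Wall as an answer; activations without an answer restore the gold material instead.
; Each finished spin completes a latent action buffer, then renews it, signalling anything awaiting the switch.
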(event InteractwithOwner(C_Interactible)
  ;[0 1 0.3289] ActivateSwitch
  ;;[0 1 0] NaviActivate
  (CallFunction|ActivateSwitch true))

(event Custom|ActivateSwitch
  (params (ShouldUpdatePlayerAnswer :type Boolean))
  ;[0 1 0.3289] ActivateSwitch
  (if (not (Variables|Default|Getdebug))
    (Default|MakeNotTargetable (Variables|Default|GetC_Interactible))
    ;;[0.5 1 0] Feedback
    (CallFunction|UpdateFlakesMat true)
    (Variables|Default|SetstartRelativeRot (.yaw (Variables|/Script/Engine.SceneComponent|GetRelativeRotation (Variables|Default|GetFlakes))))
    (bind _factorrot (Timeline|Rotation PlayFromStart)
      (:Update
        (Transformation|SetRelativeRotation (Variables|Default|GetFlakes) (Math|Rotator|MakeRotator 0.0 0.0 (Math|Float|Lerp (Variables|Default|GetstartRelativeRot) -3.6e+02 _factorrot)) false false))
      (:Finished
        (if ShouldUpdatePlayerAnswer
          (Default|UpdatePlayerAnswer (Variables|Default|GetWall) self)
          (else
            (CallFunction|UpdateFlakesMat false)))
        (Class|LowEntryLatentActionNone|Done (Variables|Default|GetSwitchActivatedBuffer))
        (Variables|Default|SetSwitchActivatedBuffer 0)
        (bind _latentaction (Class|LowEntryExtendedStandardLibrary|LatentActionCreateNone))
        (Variables|Default|SetSwitchActivatedBuffer _latentaction)))))

(event EventBeginPlay
  ;[0 0 1] Init
  (bind _latentaction (Class|LowEntryExtendedStandardLibrary|LatentActionCreateNone))
  (Variables|Default|SetSwitchActivatedBuffer _latentaction)
  (Default|MakeNotTargetable (Variables|Default|GetC_Interactible))
  (bind _asthird_person_character (Utilities|Casting|CastToThirdPersonCharacter (Game|GetPlayerCharacter 0)))
  (Variables|Default|SetPlayerRef _asthird_person_character)
  (CallFunction|FDebug))

(fn ConstructionScript)

(fn UpdateFlakesMat
  (params (Lit :type Boolean))
  (for (_ _array_index) (Rendering|Material|GetMaterials (Variables|Default|GetFlakes))
    (Rendering|Material|SetMaterial (Variables|Default|GetFlakes) _array_index (select Lit "/Game/FX/Materials/MI_EmissiveLight.MI_EmissiveLight" "/Game/Assets/Materials/MasterMaterials/M_Metal_Gold.M_Metal_Gold")))
  (return))

(fn FDebug
  (if (Variables|Default|Getdebug)
    (Default|MakeTargetable (Variables|Default|GetC_Interactible))))