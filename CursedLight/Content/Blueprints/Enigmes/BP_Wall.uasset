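; Puzzle wall that blocks the player, configured by PuzzleType as a Simon sequence or a Labyrinth double door.
; In Simon, it shuffles its switches at BeginPlay, and a trigger overlap starts a camera cinematic replaying that order, one switch per second.
; Player input is compared once complete: success plays a cinematic and drops the wall, failure resets and replays the sequence.
; In Labyrinth, MoveDoors slides both doors apart on a timeline.
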(event OnComponentBeginOverlap(TriggerCinematic)
  (params (OverlappedComponent :type Primitive%20Component%20Object%20Reference) (OtherActor :type Actor%20Object%20Reference) (OtherComp :type Primitive%20Component%20Object%20Reference) (OtherBodyIndex :type Integer) (bFromSweep :type Boolean) (SweepResult :type Hit%20Result%20Structure%20%28by%20ref%29))
  (bind _cinematiccam (Variables|Default|GetCinematicCam))
  (bind _returnvalue (Transformation|GetWorldTransform _cinematiccam))
  ;[1 0 1] Simon
  ;;[0.1366 0 1] StartCinematic
  (Collision|SetCollisionEnabled (Variables|Default|GetTriggerCinematic) "NoCollision")
  (Default|CustomDisableInput (Variables|Default|GetPlayerRef))
  (Default|WaitingCinematic (Variables|Default|GetcamManagerRef) (Utilities|Array|MakeArray (Math|Transform|MakeTransform (.location _returnvalue) (.rotation _returnvalue) "1.000000,1.000000,1.000000")))
  (CallFunction|ShowAnswer true))

(event Custom|MoveDoors
  ;[1 0.9394 0.4187] Doors Labyrinth
  (bind _newtrack_0 (Timeline|OpenDoorTimeline PlayFromStart)
    (:Update
      (Transformation|SetRelativeLocation (Variables|Default|GetDoorL) (Math|Vector|Lerp(Vector) "-150.000000, 0, 0" "-420.000000, 0, 0" _newtrack_0) false false)
      (Transformation|SetRelativeLocation (Variables|Default|GetDoorR) (Math|Vector|Lerp(Vector) "150.000000, 0, 0" "420.000000, 0, 0" _newtrack_0) false false))))

(event Custom|ShowAnswer
  (params (Cinematic :type Boolean) (SwitchBuffer :type Low%20Entry%20Latent%20Action%20None%20Object%20Reference))
  ;[1 0 1] Simon
  ;;[0 0.7209 1] ShowAnswer
  (if Cinematic
    _
    (else
      (Class|LowEntryLatentActionNone|WaitTillDone SwitchBuffer)))
  (bind _tick (Class|LowEntryExtendedStandardLibrary|TickSeconds (+ (Utilities|Array|Length (Variables|Default|GetSolutionArray)) 1) 1.0))
  (if (>= (- _tick 1) (Utilities|Array|Length (Variables|Default|GetSolutionArray)))
    (if Cinematic
      (Default|NextWaitingCinematicCamera (Variables|Default|GetcamManagerRef)))
    (for _array_element (Variables|Default|GetSolutionArray)
      (Default|MakeTargetable (Variables|/Game/Blueprints/Enigmes/BP_SwitchSimon.BP_SwitchSimon_C|GetC_Interactible _array_element)))
    (Class|LowEntryLatentActionNone|WaitTillDone (Variables|/Game/Blueprints/Camera/ALS/ALS_PlayerCameraManager.ALS_PlayerCameraManager_C|GetreverseMoveCamAction (Variables|Default|GetcamManagerRef)))
    (Input|EnableInput (Game|GetPlayerCharacter 0) (Game|GetPlayerController 0))
    (else
      (Default|ActivateSwitch (Utilities|Array|Get(acopy) (Variables|Default|GetSolutionArray) (- _tick 1)) false))))

(event Custom|SimonWinCinematic
  (bind _cinematiccam (Variables|Default|GetCinematicCam))
  (bind _returnvalue (Transformation|GetWorldTransform _cinematiccam))
  ;[1 0 1] Simon
  ;;[0.3169 1 0] SimonWinCinematic
  (for _array_element (Variables|Default|GetSolutionArray)
    (Default|ActivateSwitch _array_element false))
  (Utilities|FlowControl|Delay 1.5)
  (Components|Activation|Deactivate (Variables|Default|GetWallVFX))
  (Collision|SetCollisionEnabled (Variables|Default|GetWallCollision) "NoCollision")
  (Transformation|SetRelativeLocationAndRotation _cinematiccam "0.000000,-2000.000000,500.000000" "0,90.000000, 0" false false)
  (Default|Cinematic (Variables|Default|GetcamManagerRef) (Utilities|Array|MakeArray (Math|Transform|MakeTransform (.location _returnvalue) (.rotation _returnvalue) "1.000000,1.000000,1.000000")) (Utilities|Array|MakeArray 1.0 4.5))
  (Class|LowEntryLatentActionNone|WaitTillDone (Variables|/Game/Blueprints/Camera/ALS/ALS_PlayerCameraManager.ALS_PlayerCameraManager_C|GetreverseMoveCamAction (Variables|Default|GetcamManagerRef)))
  (Input|EnableInput (Game|GetPlayerCharacter 0) (Game|GetPlayerController 0)))

(event EventBeginPlay
  ;[0 0 1] Init : Set switches ref + randomize solution
  (bind _asthird_person_character (Utilities|Casting|CastToThirdPersonCharacter (Game|GetPlayerCharacter 0)))
  (Variables|Default|SetPlayerRef _asthird_person_character)
  (bind _asals_player_camera_manager (Utilities|Casting|CastToALS_PlayerCameraManager (Game|GetPlayerCameraManager 0)))
  (Variables|Default|SetcamManagerRef _asals_player_camera_manager)
  (switch Utilities|FlowControl|Switch|SwitchonEPuzzle (Variables|Default|GetpuzzleType)
    (:NewEnumerator0
      (Components|Activation|Activate (Variables|Default|GetWallVFX) false)
      (for _array_element (Variables|Default|GetSolutionArray)
        (Variables|/Game/Blueprints/Enigmes/BP_SwitchSimon.BP_SwitchSimon_C|SetWall _array_element self))
      (Utilities|Array|Shuffle (Variables|Default|GetSolutionArray)))
    (:NewEnumerator1
      (Development|SetHiddeninGame (Variables|Default|GetDoorR) false false)
      (Collision|SetCollisionEnabled (Variables|Default|GetTriggerCinematic) "NoCollision"))))

(fn ConstructionScript)

(fn UpdatePlayerAnswer
  (params (switchToAdd :type BP%20Switch%20Simon%20Object%20Reference))
  (bind _playeranswerarray (Variables|Default|GetPlayerAnswerArray))
  (Utilities|Array|AddUnique _playeranswerarray switchToAdd)
  (if (!= (Utilities|Array|Length _playeranswerarray) (Utilities|Array|Length (Variables|Default|GetSolutionArray)))
    _
    (else
      (CallFunction|CheckPlayerAnswer)))
  (return))

(fn CheckPlayerAnswer
  (bind _playeranswerarray (Variables|Default|GetPlayerAnswerArray))
  (if (Utilities|Array|Identical (Variables|Default|GetPlayerAnswerArray) (Variables|Default|GetSolutionArray))
    (CallFunction|SimonWinCinematic)
    (else
      (for _array_element _playeranswerarray
        (Default|UpdateFlakesMat _array_element false))
      (LocalVariables|SetlastSwitch (Utilities|Array|Get(acopy) _playeranswerarray (Utilities|Array|LastIndex _playeranswerarray)))
      (Utilities|Array|Clear (Variables|Default|GetPlayerAnswerArray))
      (CallFunction|ShowAnswer false (Variables|/Game/Blueprints/Enigmes/BP_SwitchSimon.BP_SwitchSimon_C|GetSwitchActivatedBuffer (LocalVariables|GetlastSwitch)))))
  (return))