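; BP_Root is a puzzle actor for a root puzzle, made of eight cube pieces that glide toward target positions.
; BeginPlay caches the third-person player, collects the cubes, and records their relative locations as both initial and target arrays.
; While the player's InRootPuzzle flag is set, Tick eases each cube toward its target with VInterpTo.
; Nothing in this Blueprint changes the targets after BeginPlay.
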(event EventBeginPlay
  (bind _cube2 (Variables|Default|GetCube2))
  (bind _cube1 (Variables|Default|GetCube1))
  (bind _cube7 (Variables|Default|GetCube7))
  (bind _cube (Variables|Default|GetCube))
  (bind _cube4 (Variables|Default|GetCube4))
  (bind _cube5 (Variables|Default|GetCube5))
  (bind _cube6 (Variables|Default|GetCube6))
  (bind _cube3 (Variables|Default|GetCube3))
  (bind _asthird_person_character (Utilities|Casting|CastToThirdPersonCharacter (Game|GetPlayerCharacter 0)))
  (Variables|Default|SetPlayerRef _asthird_person_character)
  (Variables|Default|SetRootArray (Utilities|Array|MakeArray _cube _cube1 _cube2 _cube3 _cube4 _cube5 _cube6 _cube7))
  (bind _output_get (Variables|Default|SetRootTargetLocation (Utilities|Array|MakeArray (Variables|/Script/Engine.SceneComponent|GetRelativeLocation _cube) (Variables|/Script/Engine.SceneComponent|GetRelativeLocation _cube1) (Variables|/Script/Engine.SceneComponent|GetRelativeLocation _cube2) (Variables|/Script/Engine.SceneComponent|GetRelativeLocation _cube3) (Variables|/Script/Engine.SceneComponent|GetRelativeLocation _cube4) (Variables|/Script/Engine.SceneComponent|GetRelativeLocation _cube5) (Variables|/Script/Engine.SceneComponent|GetRelativeLocation _cube6) (Variables|/Script/Engine.SceneComponent|GetRelativeLocation _cube7))))
  (Variables|Default|SetRootInitialLocation _output_get)
  (Actor|Tick|SetActorTickEnabled true))

(event Collision|EventActorBeginOverlap
  (params (OtherActor :type Actor%20Object%20Reference)))

(event EventTick
  (params (DeltaSeconds :type Float%20%28single-precision%29))
  (if (Variables|/Game/Blueprints/Player/ThirdPersonCharacter.ThirdPersonCharacter_C|GetinRootPuzzle (Variables|Default|GetPlayerRef))
    (for (_array_element _array_index) (Variables|Default|GetRootArray)
      (Transformation|SetRelativeLocation _array_element (Math|Interpolation|VInterpTo (Variables|/Script/Engine.SceneComponent|GetRelativeLocation _array_element) (Utilities|Array|Get(acopy) (Variables|Default|GetRootTargetLocation) _array_index) DeltaSeconds 5.0) false false))))

(fn ConstructionScript)