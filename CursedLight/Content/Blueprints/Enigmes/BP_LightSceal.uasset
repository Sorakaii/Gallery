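; BP_LightSceal is an interactible puzzle actor that starts a Navi-controlled root puzzle for the player.
; BeginPlay caches the player character and ALS camera manager.
; On interaction it disables targeting, hides the player's Navi collision component, and spawns a non-wall BP_NaviPuzzle at its sphere.
; It hands puzzle, root and seal references to the player, starts the puzzle, and passes its camera transform to the camera manager's WaitingCinematic.
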(event InteractwithOwner(C_Interactible)
  (bind _playerref (Variables|Default|GetPlayerRef))
  (bind _camera (Variables|Default|GetCamera))
  (Default|MakeNotTargetable (Variables|Default|GetC_Interactible))
  (Rendering|SetVisibility (Variables|/Game/Blueprints/Navi/BP_NaviPawn.BP_NaviPawn_C|GetCollision (Variables|/Game/Blueprints/Player/ThirdPersonCharacter.ThirdPersonCharacter_C|GetnaviRef (Variables|Default|GetPlayerRef))) false true)
  (bind _returnvalue (Game|SpawnActorfromClass "/Game/Blueprints/Navi/BP_NaviPuzzle.BP_NaviPuzzle_C" (Math|Transform|MakeTransform (Transformation|GetWorldLocation (Variables|Default|GetSphere)) "0, 0, 0" "2.000000,2.000000,2.000000") "Undefined" 0 0 self 0))
  (Variables|/Game/Blueprints/Navi/BP_NaviPuzzle.BP_NaviPuzzle_C|SetIsWallPuzzle _returnvalue false)
  (Variables|/Game/Blueprints/Player/ThirdPersonCharacter.ThirdPersonCharacter_C|SetinRootPuzzle _playerref true)
  (Variables|/Game/Blueprints/Player/ThirdPersonCharacter.ThirdPersonCharacter_C|SetrootPuzzleNaviPuzzleRef _playerref _returnvalue)
  (Variables|/Game/Blueprints/Player/ThirdPersonCharacter.ThirdPersonCharacter_C|SetrootPuzzleRootRef _playerref (Variables|Default|GetRootRef))
  (Variables|/Game/Blueprints/Player/ThirdPersonCharacter.ThirdPersonCharacter_C|SetrootPuzzleLightScealRef _playerref self)
  (Default|StartPuzzle _returnvalue)
  (Default|WaitingCinematic (Variables|Default|GetCamManagerRef) (Utilities|Array|MakeArray (Math|Transform|MakeTransform (Transformation|GetWorldLocation _camera) (Transformation|GetWorldRotation _camera) "1.000000,1.000000,1.000000"))))

(event EventBeginPlay
  (bind _asthird_person_character (Utilities|Casting|CastToThirdPersonCharacter (Game|GetPlayerCharacter 0)))
  (Variables|Default|SetPlayerRef _asthird_person_character)
  (bind _asals_player_camera_manager (Utilities|Casting|CastToALS_PlayerCameraManager (Game|GetPlayerCameraManager 0)))
  (Variables|Default|SetCamManagerRef _asals_player_camera_manager))

(event Collision|EventActorBeginOverlap
  (params (OtherActor :type Actor%20Object%20Reference)))

(event EventTick
  (params (DeltaSeconds :type Float%20%28single-precision%29)))

(fn ConstructionScript)