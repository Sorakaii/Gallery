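; BP_SwitchFindable is a one-shot puzzle switch that lights its indexed part of a linked Wall when interacted with.
; Interaction makes it untargetable, resets the player's control rotation to the character's yaw, and swaps the Flakes mesh materials from gold to emissive.
; A timeline then spins the Flakes in yaw as feedback.
; A sound call exists but is never executed.
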(event InteractwithOwner(C_Interactible)
  ;[0 1 0.3289] ActivateSwitch
  ;;[0 1 0] NaviActivate
  (CallFunction|ActivateSwitch))

(event Custom|ActivateSwitch
  ;[0 1 0.3289] ActivateSwitch
  (Default|MakeNotTargetable (Variables|Default|GetC_Interactible))
  (Pawn|SetControlRotation (Game|GetPlayerController 0) (Math|Rotator|MakeRotator 0.0 0.0 (.yaw (Transformation|GetActorRotation (Variables|Default|GetPlayerRef)))))
  ;;[0.5 1 0] Feedback
  (CallFunction|UpdateFlakesMat true)
  (Variables|Default|SetstartRelativeRot (.yaw (Variables|/Script/Engine.SceneComponent|GetRelativeRotation (Variables|Default|GetFlakes))))
  (Default|Lighton (Variables|Default|GetWall) (Variables|Default|GetIndex))
  (bind _factorrot (Timeline|Rotation PlayFromStart)
    (:Update
      (Transformation|SetRelativeRotation (Variables|Default|GetFlakes) (Math|Rotator|MakeRotator 0.0 0.0 (Math|Float|Lerp (Variables|Default|GetstartRelativeRot) -3.6e+02 _factorrot)) false false))))

(event EventBeginPlay
  ;[0 0 1] Init
  (bind _asthird_person_character (Utilities|Casting|CastToThirdPersonCharacter (Game|GetPlayerCharacter 0)))
  (Variables|Default|SetPlayerRef _asthird_person_character))

(fn ConstructionScript)

(fn UpdateFlakesMat
  (params (Lit :type Boolean))
  (for (_ _array_index) (Rendering|Material|GetMaterials (Variables|Default|GetFlakes))
    (Rendering|Material|SetMaterial (Variables|Default|GetFlakes) _array_index (select Lit "/Game/FX/Materials/MI_EmissiveLight.MI_EmissiveLight" "/Game/Assets/Materials/MasterMaterials/M_Metal_Gold.M_Metal_Gold")))
  (return))