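; Puzzle wall that opens once its four indicator lights are lit.
; LightOn swaps the indexed light to an emissive material and counts calls; the fourth disables the player's walk and jump and removes wall collision.
; A transition widget's black-screen callbacks then chain the sequence: the ALS camera manager cuts to CinematicCam as the wall VFX deactivates, then reverses back and restores movement.
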(event Custom|LightOn
  (params (Num :type Integer))
  (Rendering|Material|SetMaterial (Utilities|Array|Get(acopy) (Variables|Default|GetSphereArray) Num) 0 "/Game/Blueprints/Enigmes/M_Emissive.M_Emissive")
  (bind _result (Math|Integer|IncrementInt (Variables|Default|Getcount))
    (:%20%20
      (if (== _result 4)
        (Default|SetMovementCapabilities (Variables|Default|GetPlayerRef) false false true)
        (Utilities|FlowControl|Delay 1.0)
        (Collision|SetCollisionEnabled (Variables|Default|GetWallCollision) "NoCollision")
        (bind _returnvalue (UserInterface|CreateWidget "/Game/Blueprints/UI/WBP_Transition.WBP_Transition_C" 0 true))
        (UserInterface|Viewport|AddtoViewport _returnvalue 0)
        (EventDispatchers|BindEventtoIsBlack _returnvalue (delegate Custom|StartCine))))))

(event Custom|StartCine
  (bind _cinematiccam (Variables|Default|GetCinematicCam))
  (bind _returnvalue (Transformation|GetWorldTransform _cinematiccam))
  (Components|Activation|Deactivate (Variables|Default|GetWallVFX))
  (Default|Cinematic (Variables|Default|GetcamManagerRef) (Utilities|Array|MakeArray (Math|Transform|MakeTransform (.location _returnvalue) (.rotation _returnvalue) "1.000000,1.000000,1.000000")) (Utilities|Array|MakeArray 0.0 2.5) true)
  (Utilities|FlowControl|Delay 1.5)
  (bind _returnvalue_2 (UserInterface|CreateWidget "/Game/Blueprints/UI/WBP_Transition.WBP_Transition_C"))
  (UserInterface|Viewport|AddtoViewport _returnvalue_2 0)
  (EventDispatchers|BindEventtoIsBlack _returnvalue_2 (delegate Custom|ReturnCine)))

(event Custom|ReturnCine
  (Class|LowEntryLatentActionNone|WaitTillDone (Variables|/Game/Blueprints/Camera/ALS/ALS_PlayerCameraManager.ALS_PlayerCameraManager_C|GetreverseMoveCamAction (Variables|Default|GetcamManagerRef)))
  (Default|ReverseFade (stale Custom|StartCine _returnvalue_2))
  (Default|SetMovementCapabilities (Variables|Default|GetplayerRef) true true true))

(event EventBeginPlay
  (Variables|Default|SetSphereArray (Utilities|Array|MakeArray (Variables|Default|GetLight1) (Variables|Default|GetLight2) (Variables|Default|GetLight3) (Variables|Default|GetLight4)))
  (bind _asthird_person_character (Utilities|Casting|CastToThirdPersonCharacter (Game|GetPlayerCharacter 0)))
  (Variables|Default|SetPlayerRef _asthird_person_character)
  (bind _asals_player_camera_manager (Utilities|Casting|CastToALS_PlayerCameraManager (Game|GetPlayerCameraManager 0)))
  (Variables|Default|SetcamManagerRef _asals_player_camera_manager)
  (Components|Activation|Activate (Variables|Default|GetWallVFX) false))

(event Collision|EventActorBeginOverlap
  (params (OtherActor :type Actor%20Object%20Reference)))

(event EventTick
  (params (DeltaSeconds :type Float%20%28single-precision%29)))

(fn ConstructionScript)