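; Component that makes its owning actor a focusable lock-on target for the ThirdPersonCharacter, marked by a spinning arrow.
; On BeginPlay it creates a query-only overlap box sized to the actor's bounds and a hidden arrow mesh, which focus events show or hide.
; Targetability switches the box's collision object type and toggles actor collision, disabling only when no sibling component remains focusable.
; Re-enabling also calls the player's lock search.
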(event Custom|isFocused
  (params (OldComp :type C%20Interactible%20Object%20Reference))
  (Utilities|IsValid OldComp
    (:Is%20Valid
      (Rendering|SetVisibility (Variables|C_Interactible_C|GetarrowMeshComp OldComp) false false)
      (Rendering|SetVisibility (Variables|Default|GetarrowMeshComp) true false))))

(event Custom|Unfocused
  (Rendering|SetVisibility (Variables|Default|GetarrowMeshComp) false false))

(event Custom|MakeNotTargetable
  (if (Utilities|Enum|NotEqual(Enum) (Collision|GetCollisionObjectType (Variables|Default|GetCollider)) "ECC_GameTraceChannel4")
    (Variables|Default|SetcanFocus false)
    (bind _ownerhasfocusable (CallFunction|CheckBrothers))
    (if (not _ownerhasfocusable)
      (Collision|SetCollisionObjectType (Variables|Default|GetCollider) "ECC_GameTraceChannel4")
      (Collision|SetActorEnableCollision (Components|GetOwner) false)
      (Collision|SetActorEnableCollision (Components|GetOwner) true))))

(event Custom|MakeTargetable
  (Variables|Default|SetcanFocus true)
  (Collision|SetCollisionObjectType (Variables|Default|GetCollider) "ECC_GameTraceChannel3")
  (Collision|SetActorEnableCollision (Components|GetOwner) false)
  (Default|FSearchLock (Variables|Default|GetplayerRef) false)
  (Collision|SetActorEnableCollision (Components|GetOwner) true))

(event EventBeginPlay
  (bind _returnvalue (Components|GetOwner))
  (bind _asthird_person_character (Utilities|Casting|CastToThirdPersonCharacter (Game|GetPlayerCharacter 0)))
  (bind _output_get (Variables|Default|SetplayerRef _asthird_person_character))
  (Variables|Default|SetnaviRef (Variables|/Game/Blueprints/Player/ThirdPersonCharacter.ThirdPersonCharacter_C|GetnaviRef _output_get))
  (bind _returnvalue_2 (Game|AddComponentbyClass _returnvalue "/Script/Engine.BoxComponent" false))
  (Variables|Default|SetCollider _returnvalue_2)
  (Collision|SetCollisionEnabled (Variables|Default|GetCollider) "QueryOnly")
  (Collision|SetCollisionResponsetoAllChannels (Variables|Default|GetCollider) "ECR_Overlap")
  (Collision|SetCollisionObjectType (Variables|Default|GetCollider) "ECC_GameTraceChannel3")
  (Components|Box|SetBoxExtent (Variables|Default|GetCollider) (.BoxExtent (Collision|GetActorBounds _returnvalue false false)) true)
  (bind _returnvalue_3 (Game|AddComponentbyClass (Components|GetOwner) "/Script/Engine.StaticMeshComponent" false (Math|Transform|MakeTransform "0, 0, 0" "0.000000, 0,-90.000000" "1.000000,1.000000,1.000000")))
  (Variables|Default|SetarrowMeshComp _returnvalue_3)
  (Collision|SetCollisionEnabled (Variables|Default|GetarrowMeshComp) "NoCollision")
  (Components|StaticMesh|SetStaticMesh (Variables|Default|GetarrowMeshComp) "/Game/Blueprints/UI/SM_LockArrow.SM_LockArrow")
  (Transformation|SetWorldLocation (Variables|Default|GetarrowMeshComp) (+ (Transformation|GetWorldLocation) "0,0,50.000000") false false)
  (Transformation|AttachComponentToComponent (Variables|Default|GetarrowMeshComp) self "None" "KeepWorld" "KeepWorld" "KeepWorld" false)
  (CallFunction|Unfocused)
  (Components|Tick|SetComponentTickEnabled true))

(event EventTick
  (params (DeltaSeconds :type Float%20%28single-precision%29))
  (bind _arrowmeshcomp (Variables|Default|GetarrowMeshComp))
  (CallFunction|Debug)
  (Transformation|AddWorldRotation (Variables|Default|GetarrowMeshComp) "0,-1.000000, 0" false false)
  (Transformation|SetWorldRotation _arrowmeshcomp (Math|Rotator|MakeRotator -9e+01 0.0 (.yaw (Transformation|GetWorldRotation _arrowmeshcomp))) false false))

(fn Debug)

(fn CheckBrothers
  (for _array_element (Actor|GetComponentsByClass (Components|GetOwner) "C_Interactible_C")
    (if (Variables|C_Interactible_C|GetcanFocus _array_element)
      (return true)))
  (return false))