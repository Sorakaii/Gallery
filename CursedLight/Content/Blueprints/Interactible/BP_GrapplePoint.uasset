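; Grapple point the player can target within a mid-range distance band and pull themselves to.
; Tick checks player distance to toggle the interactible component's targetability and its Niagara effect.
; Interacting restricts movement and plays a grapple montage, whose notify starts a timeline extending the grapple end to the point.
; The capsule then moves above the point and the grapple hides, while montage completion or interruption restores movement.
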(event InteractwithOwner(C_Interactible)
  (bind _playerref (Variables|Default|GetplayerRef))
  (Default|LockUpdate (Variables|Default|GetplayerRef) false)
  (Default|SetMovementCapabilities (Variables|Default|GetPlayerRef) false false true)
  (Pawn|SetControlRotation (Game|GetPlayerController 0) (Transformation|GetActorRotation (Variables|Default|GetPlayerref)))
  (Animation|Montage|PlayMontage (Variables|/Script/Engine.Character|GetMesh (Variables|Default|GetplayerRef)) "/Game/Characters/Player/Animations/AM_Player_Grappling.AM_Player_Grappling"
    (:OnCompleted
      (Default|SetMovementCapabilities (Variables|Default|GetplayerRef) true true true :!label _label))
    (:OnInterrupted
      (goto _label))
    (:OnNotifyBegin
      (Rendering|SetVisibility (Variables|/Game/Blueprints/Player/ThirdPersonCharacter.ThirdPersonCharacter_C|GetGrapple (Variables|Default|GetplayerRef)) true false)
      (Audio|PlaySound2D "/Game/FX/Audio/Magical_light_transition__Sound_Effects_.Magical_light_transition__Sound_Effects_" 1.0 1.0 0.0 0 0)
      (Variables|Default|SetWorldLocationInteractible (Transformation|GetWorldLocation (Variables|Default|GetC_Interactible)))
      (Variables|Default|SetWorldLocationGrappleEnd (Transformation|GetWorldLocation (Variables|/Game/Blueprints/Player/ThirdPersonCharacter.ThirdPersonCharacter_C|GetGrappleEnd (Variables|Default|GetplayerRef))))
      (bind _newtrack_0 (Timeline|GrappleTimeline PlayFromStart)
        (:Update
          (Transformation|SetWorldLocation (Variables|/Game/Blueprints/Player/ThirdPersonCharacter.ThirdPersonCharacter_C|GetGrappleEnd (Variables|Default|GetplayerRef)) (Math|Vector|Lerp(Vector) (Variables|Default|GetWorldLocationGrappleEnd) (Variables|Default|GetWorldLocationInteractible) _newtrack_0) false false))
        (:Finished
          (Components|MoveComponentTo (Variables|/Script/Engine.Character|GetCapsuleComponent (Variables|Default|GetplayerRef)) (+ (Transformation|GetActorLocation) "0,0,200.000000") "0, 0, 0" false false 0.2 false)
          (Transformation|SetWorldLocation (Variables|/Game/Blueprints/Player/ThirdPersonCharacter.ThirdPersonCharacter_C|GetGrappleEnd _playerref) (Transformation|GetActorLocation _playerref) false false)
          (Rendering|SetVisibility (Variables|/Game/Blueprints/Player/ThirdPersonCharacter.ThirdPersonCharacter_C|GetGrapple (Variables|Default|GetplayerRef)) false false))))))

(event EventBeginPlay
  (bind _asthird_person_character (Utilities|Casting|CastToThirdPersonCharacter (Game|GetPlayerCharacter 0)))
  (Variables|Default|SetplayerRef _asthird_person_character))

(event EventTick
  (params (DeltaSeconds :type Float%20%28single-precision%29))
  (bind _self self)
  (bind _playerref (Variables|Default|GetplayerRef))
  (bind _c_interactible (Variables|Default|GetC_Interactible))
  (bind _returnvalue (Transformation|GetDistanceTo _playerref _self))
  (bind _canfocus (Variables|/Game/Blueprints/Interactible/C_Interactible.C_Interactible_C|GetcanFocus _c_interactible))
  (if (or (< _returnvalue 5e+02) (> _returnvalue 1.5e+03))
    (if _canfocus
      (Default|MakeNotTargetable _c_interactible)
      (else
        (Components|Activation|Deactivate (Variables|Default|GetNS_GrapplinPoint))))
    (elif (not _canfocus)
      (Default|MakeTargetable _c_interactible)
      (else
        (Components|Activation|Activate (Variables|Default|GetNS_GrapplinPoint) false)))))

(fn ConstructionScript)