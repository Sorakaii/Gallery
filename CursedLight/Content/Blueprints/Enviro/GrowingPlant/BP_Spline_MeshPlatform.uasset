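; Growing plant actor that extends a randomized spline-mesh stem, with a platform-like tip mesh riding its growing end.
; LaunchAnim scatters spline points along the forward axis within random bounds, then builds hidden spline mesh sections, the last using a tip mesh.
; A random-rate timeline reveals each section in turn, lerping its end position and tangent.
; Tick keeps the added static mesh at the growing end until the final section.
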(event Custom|TimelineLaunch
  (bind _returnvalue (Transformation|GetActorRotation))
  (bind _splinemeshinfo (Variables|Default|GetSplineMeshInfo))
  (bind _splinemeshinfo_2 (Variables|Default|GetSplineMeshInfo))
  (bind _splinepartnumber (Variables|Default|GetsplinePartNumber))
  (bind _splinepartnumber_2 (Variables|Default|GetsplinePartNumber))
  (bind (_roll _pitch _yaw) (Math|Rotator|BreakRotator _returnvalue))
  (bind _output (Utilities|Array|Get(acopy) _splinemeshinfo _splinepartnumber))
  (bind _output_2 (Utilities|Array|Get(acopy) _splinemeshinfo_2 _splinepartnumber_2))
  (Rendering|SetVisibility (.splinemesh (Utilities|Array|Get(acopy) (Variables|Default|GetSplineMeshInfo) (Variables|Default|GetsplinePartNumber))) true false :!label _label)
  (Variables|Default|SetcachedRelative (Math|Rotator|MakeRotator _roll _pitch _yaw))
  (bind _alpha (Timeline|timelineAlongSplineMesh PlayFromStart)
    (:Update
      (Variables|Default|SetendPos (Math|Vector|Lerp(Vector) (.startpos _output) (.endpos _output) _alpha))
      (SplineMesh|SetEndPosition (.splinemesh _output) (Variables|Default|GetendPos) true)
      (SplineMesh|SetEndTangent (.splinemesh _output_2) (Math|Vector|Lerp(Vector) (.starttan _output_2) (.endtan _output_2) _alpha) true :!class /Script/Engine.SplineMeshComponent))
    (:Finished
      (Math|Integer|IncrementInt (Variables|Default|GetsplinePartNumber)
        (:%20%20
          (if (< (Variables|Default|GetsplinePartNumber) (Utilities|Array|Length (Variables|Default|GetSplineMeshInfo)))
            (goto _label)))))))

(event Custom|moveTip
  (Transformation|SetRelativeLocation (Variables|Default|GettipRef) (Variables|Default|GetendPos) false false)
  (if (not (< (Variables|Default|GetsplinePartNumber) (- (Utilities|Array|Length (Variables|Default|GetSplineMeshInfo)) 1)))
    (Actor|Tick|SetActorTickEnabled false)))

(event Custom|LaunchAnim
  (Variables|Default|SetplayRate (Math|Random|RandomFloatinRange (Variables|Default|GetspeedRangeMin) (Variables|Default|GetspeedRangeMax)))
  (Components|Timeline|SetPlayRate (Variables|Default|GettimelineAlongSplineMesh) (Math|Random|RandomFloatinRange (Variables|Default|GetspeedRangeMin) (Variables|Default|GetspeedRangeMax)))
  (for _index (range 0 (Variables|Default|GetdividerNumber))
    (Variables|Default|SetdivindingIndex _index)
    (Variables|Default|SetpointPosition (Math|Vector|Lerp(Vector) (Transformation|GetWorldLocation (Variables|Default|GetSpline)) (+ (* (Math|Vector|GetForwardVector (Variables|Default|GetSpline)) 1e+03) (Transformation|GetWorldLocation (Variables|Default|GetSpline))) (/ (Math|Conversions|ToFloat(Integer) (+ (Variables|Default|GetdivindingIndex) 1)) (Math|Conversions|ToFloat(Integer) (Variables|Default|GetdividerNumber)))))
    (if (< (Variables|Default|GetdivindingIndex) (Variables|Default|GetdividerNumber))
      ;[1 1 1] square
      (Variables|Default|SetpointPosition (Math|Random|RandomPointinBoundingBox (Variables|Default|GetpointPosition) (Variables|Default|GetsquareSpawnBoundHalfSize)))
      ;[1 1 1] round
      (Variables|Default|SetpointPosition (.RandomLocation (CallFunction|GetRandomPointinSphere (Variables|Default|GetpointPosition) (Variables|Default|GetsphereSpawnBoundMin) (Variables|Default|GetsphereSpawnBoundMax)))))
    (Spline|AddSplinePoint (Variables|Default|GetSpline) (Variables|Default|GetpointPosition) "World" true))
  (Variables|Default|SetsectionLength (* (.x (Transformation|GetActorScale3D)) (Variables|Default|GetsectionLength)))
  (for _index_2 (range 0 (Math|Float|Truncate (/ (Spline|GetSplineLength (Variables|Default|GetSpline)) (Variables|Default|GetsectionLength))))
    (Variables|Default|SetpointIndex _index_2)
    (bind _returnvalue (Game|AddComponentbyClass "/Script/Engine.SplineMeshComponent" false))
    (Utilities|Array|Add (Variables|Default|GetSplineMeshInfo) (Utilities|Struct|MakeSplineMeshInfos _returnvalue (Spline|GetLocationatDistanceAlongSpline (Variables|Default|GetSpline) (* (Variables|Default|GetpointIndex) (Variables|Default|GetsectionLength)) "Local") (Math|Vector|ClampVectorSize (Spline|GetTangentatDistanceAlongSpline (Variables|Default|GetSpline) (* (Variables|Default|GetpointIndex) (Variables|Default|GetsectionLength)) "Local") 0.0 (Variables|Default|GetsectionLength)) (Spline|GetLocationatDistanceAlongSpline (Variables|Default|GetSpline) (* (+ (Variables|Default|GetpointIndex) 1) (Variables|Default|GetsectionLength)) "Local") (Math|Vector|ClampVectorSize (Spline|GetTangentatDistanceAlongSpline (Variables|Default|GetSpline) (* (+ (Variables|Default|GetpointIndex) 1) (Variables|Default|GetsectionLength)) "Local") 0.0 (Variables|Default|GetsectionLength))))
    (Transformation|SetMobility (.splinemesh (Utilities|Array|Get(acopy) (Variables|Default|GetSplineMeshInfo) (Variables|Default|GetpointIndex))) "Movable")
    (SplineMesh|SetStartandEnd (.splinemesh (Utilities|Array|Get(acopy) (Variables|Default|GetSplineMeshInfo) (Variables|Default|GetpointIndex))) (.startpos (Utilities|Array|Get(acopy) (Variables|Default|GetSplineMeshInfo) (Variables|Default|GetpointIndex))) (.starttan (Utilities|Array|Get(acopy) (Variables|Default|GetSplineMeshInfo) (Variables|Default|GetpointIndex))) (.endpos (Utilities|Array|Get(acopy) (Variables|Default|GetSplineMeshInfo) (Variables|Default|GetpointIndex))) (.endtan (Utilities|Array|Get(acopy) (Variables|Default|GetSplineMeshInfo) (Variables|Default|GetpointIndex))) true :!class /Script/Engine.SplineMeshComponent)
    (if (>= (Variables|Default|GetpointIndex) (Math|Float|Truncate (/ (Spline|GetSplineLength (Variables|Default|GetSpline)) (Variables|Default|GetsectionLength))))
      (Components|StaticMesh|SetStaticMesh (.splinemesh (Utilities|Array|Get(acopy) (Variables|Default|GetSplineMeshInfo) (Variables|Default|GetpointIndex))) (Variables|Default|GettipMesh))
      (Rendering|Material|SetMaterial (.splinemesh (Utilities|Array|Get(acopy) (Variables|Default|GetSplineMeshInfo) (Variables|Default|GetpointIndex))) 0 (Variables|Default|GettipMaterial))
      (else
        (Components|StaticMesh|SetStaticMesh (.splinemesh (Utilities|Array|Get(acopy) (Variables|Default|GetSplineMeshInfo) (Variables|Default|GetpointIndex))) (Variables|Default|GetmeshSection))
        (Rendering|Material|SetMaterial (.splinemesh (Utilities|Array|Get(acopy) (Variables|Default|GetSplineMeshInfo) (Variables|Default|GetpointIndex))) 0 (Variables|Default|GetsectionMaterial))))
    (SplineMesh|SetForwardAxis (.splinemesh (Utilities|Array|Get(acopy) (Variables|Default|GetSplineMeshInfo) (Variables|Default|GetpointIndex))) (Variables|Default|GetmeshForwardAxis) true)
    (Class|SplineMeshComponent|SetStartRoll (.splinemesh (Utilities|Array|Get(acopy) (Variables|Default|GetSplineMeshInfo) (Variables|Default|GetpointIndex))) (Math|Trig|DegreesToRadians (Class|SplineComponent|GetRollatDistanceAlongSpline (Variables|Default|GetSpline) (* (Variables|Default|GetpointIndex) (Variables|Default|GetsectionLength)) "Local")) true)
    (Class|SplineMeshComponent|SetEndRoll (.splinemesh (Utilities|Array|Get(acopy) (Variables|Default|GetSplineMeshInfo) (Variables|Default|GetpointIndex))) (Math|Trig|DegreesToRadians (Class|SplineComponent|GetRollatDistanceAlongSpline (Variables|Default|GetSpline) (* (+ (Variables|Default|GetpointIndex) 1) (Variables|Default|GetsectionLength)) "Local")) true)
    (Rendering|SetVisibility (.splinemesh (Utilities|Array|Get(acopy) (Variables|Default|GetSplineMeshInfo) (Variables|Default|GetpointIndex))) false false))
  (CallFunction|TimelineLaunch)
  (Actor|Tick|SetActorTickEnabled true))

(event EventBeginPlay
  (bind _returnvalue (AddComponent|AddStaticMeshComponent false (Math|Transform|MakeTransform "0, 0, 0" "90.000000, 0, 0" "1.000000,1.000000,1.000000")))
  (bind _output_get (Variables|Default|SettipRef _returnvalue))
  (Transformation|SetMobility _output_get "Movable"))

(event EventTick
  (params (DeltaSeconds :type Float%20%28single-precision%29))
  (CallFunction|MoveTip))

(fn ConstructionScript)