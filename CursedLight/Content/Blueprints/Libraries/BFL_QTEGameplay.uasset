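; Blueprint function library for QTE gameplay, with a helper that places a QTE widget above a target component.
; It creates a WidgetComponent on the instigator actor, then detaches it and snaps it onto the given parent component.
; The component gets a fixed draw size, a raised relative position and the caller's already-created widget, then returns along with that widget.
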(fn AddQTEWidgetonTarget
  (params (InstigatorTemp :type Actor%20Object%20Reference) (ParentComponent :type Scene%20Component%20Object%20Reference) (WidgetCreated :type User%20Widget%20Object%20Reference))
  (bind _returnvalue (Game|AddComponentbyClass InstigatorTemp "/Script/UMG.WidgetComponent" false))
  (LocalVariables|SetQTEWidgetComp _returnvalue)
  (Transformation|DetachFromComponent (LocalVariables|GetQTEWidgetComp) "KeepRelative" "KeepRelative" "KeepRelative" true)
  (Transformation|AttachComponentToComponent (LocalVariables|GetQTEWidgetComp) ParentComponent "None" "SnapToTarget" "SnapToTarget" "SnapToTarget" true)
  (Class|WidgetComponent|SetDrawSize (LocalVariables|GetQTEWidgetComp) "(X=100.000000,Y=100.000000)")
  (Transformation|SetRelativeLocation (LocalVariables|GetQTEWidgetComp) "0, 0,200.000000" false false)
  (UserInterface|SetWidget (LocalVariables|GetQTEWidgetComp) WidgetCreated)
  (return (LocalVariables|GetQTEWidgetComp) (UserInterface|GetWidget (LocalVariables|GetQTEWidgetComp))))