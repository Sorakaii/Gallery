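; BP_BossCL is an AI boss that targets the player through its blackboard and can be killed by damage.
; BeginPlay stores left and right arm locations in the blackboard and caches the player.
; Entering its Box sets the player as target and binds target clearing to player death; leaving does not clear it.
; At zero health it clears the target, plays a timeline rotation as a placeholder death, then destroys itself.
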(event OnComponentBeginOverlap(Box)
  (params (OverlappedComponent :type Primitive%20Component%20Object%20Reference) (OtherActor :type Actor%20Object%20Reference) (OtherComp :type Primitive%20Component%20Object%20Reference) (OtherBodyIndex :type Integer) (bFromSweep :type Boolean) (SweepResult :type Hit%20Result%20Structure%20%28by%20ref%29))
  (if (== OtherActor (Variables|Default|GetplayerRef))
    (AI|Components|Blackboard|SetValueasObject (AI|GetBlackboard 0) (Variables|Default|GettargetKeyName) (Game|GetPlayerCharacter 0))
    (EventDispatchers|BindEventtoPlayerDeathDispatcher (Variables|Default|GetplayerRef) (delegate Custom|StopFighting))))

(event OnComponentEndOverlap(Box)
  (params (OverlappedComponent :type Primitive%20Component%20Object%20Reference) (OtherActor :type Actor%20Object%20Reference) (OtherComp :type Primitive%20Component%20Object%20Reference) (OtherBodyIndex :type Integer)))

(event Custom|StopFighting
  (AI|Components|Blackboard|ClearValue (AI|GetBlackboard 0) (Variables|Default|GettargetKeyName)))

(event EventBeginPlay
  (AI|Components|Blackboard|SetValueasObject (AI|GetBlackboard 0) (Variables|Default|GetleftArmKeyName) (Variables|Default|GetLeftArmLocation))
  (AI|Components|Blackboard|SetValueasObject (AI|GetBlackboard 0) (Variables|Default|GetrightArmKeyName) (Variables|Default|GetRightArmLocation))
  (bind _asthird_person_character (Utilities|Casting|CastToThirdPersonCharacter (Game|GetPlayerCharacter 0)))
  (Variables|Default|SetplayerRef _asthird_person_character))

(event Game|Damage|EventAnyDamage
  (params (Damage :type Float%20%28single-precision%29) (DamageType :type Damage%20Type%20Object%20Reference) (InstigatedBy :type Controller%20Object%20Reference) (DamageCauser :type Actor%20Object%20Reference))
  (bind _output_get (Variables|Default|SetHealth (- (Variables|Default|GetHealth) Damage)))
  (if (<= _output_get 0.0)
    (AI|Components|Blackboard|ClearValue (AI|GetBlackboard 0) (Variables|Default|GettargetKeyName))
    (Variables|Default|SetRotBoss (Transformation|GetActorRotation))
    (bind _alpha (Timeline|TempDeath PlayFromStart)
      (:Update
        (Transformation|SetActorRotation (Math|Rotator|Lerp(Rotator) (Variables|Default|GetRotBoss) (Math|Rotator|MakeRotator (.Roll (Math|Rotator|BreakRotator (Variables|Default|GetRotBoss))) (.Pitch (Math|Rotator|BreakRotator (Variables|Default|GetRotBoss))) (* (.Yaw (Math|Rotator|BreakRotator (Variables|Default|GetRotBoss))) 4.0)) _alpha)))
      (:Finished
        (Actor|DestroyActor)))))

(event EventTick
  (params (DeltaSeconds :type Float%20%28single-precision%29)))

(fn ConstructionScript)