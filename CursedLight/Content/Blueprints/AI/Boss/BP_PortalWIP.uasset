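; Work-in-progress boss portal that thrusts an arm at a given player location and retracts it.
; PortalAttack drives the arm on the Movement timeline, which reverses and then calls EndAttack.
; A sphere trace at the Scene component damages the third-person character through a DoOnce that is never reset.
; The Dissolve component's position and scale feed MPC_Data on construction, BeginPlay and Tick, which also draws a debug box.
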(event Custom|PortalAttack
  (params (PlayerLoc :type Vector))
  (bind _movement (Variables|Default|GetMovement))
  (bind _scene (Variables|Default|GetScene))
  (bind _returnvalue (Transformation|GetWorldLocation _scene))
  (Variables|Default|SetPlayerLocation PlayerLoc)
  (bind _alpha (Timeline|Movement PlayFromStart)
    (:Update
      (Transformation|SetRelativeLocation (Variables|Default|GetArm) (Math|Vector|Lerp(Vector) (Variables|Default|GetArmLoc) (Variables|Default|GetPlayerLocation) _alpha) false false)
      (bind _outhit (Collision|SphereTraceByChannel _returnvalue _returnvalue 26.0 "TraceTypeQuery1" false 0 "None"))
      (bind _asthird_person_character (Utilities|Casting|CastToThirdPersonCharacter (.HitActor (Collision|BreakHitResult _outhit))))
      (Utilities|FlowControl|DoOnce false
        (:Completed
          (Game|Damage|ApplyDamage _asthird_person_character 2.0 0 0))))
    (:Finished
      (if (!= (Components|Timeline|GetPlaybackPosition _movement) 0.0)
        (Components|Timeline|ReversefromEnd _movement)
        (else
          (Default|CallEndAttack))))))

(event EventTick
  (params (DeltaSeconds :type Float%20%28single-precision%29))
  (bind _dissolve (Variables|Default|GetDissolve))
  (Rendering|Material|SetVectorParameterValue "/Game/FX/Materials/DissolvePortal/MPC_Data.MPC_Data" "Bounds" (Math|Conversions|ToLinearColor(Vector) (Transformation|GetWorldScale (Variables|Default|GetDissolve))) :!class /Script/Engine.KismetMaterialLibrary)
  (Rendering|Material|SetVectorParameterValue "/Game/FX/Materials/DissolvePortal/MPC_Data.MPC_Data" "Position" (Math|Conversions|ToLinearColor(Vector) (Transformation|GetWorldLocation (Variables|Default|GetDissolve))) :!class /Script/Engine.KismetMaterialLibrary)
  (Rendering|Debug|DrawDebugBox (Transformation|GetWorldLocation _dissolve) "250.000000,30.000000,30.000000" "(R=0.000000,G=1.000000,B=0.118339,A=1.000000)" (Transformation|GetWorldRotation _dissolve) 0.0 1e+01))

(event EventBeginPlay
  (bind _dissolve (Variables|Default|GetDissolve))
  (Variables|Default|SetArmLoc (Variables|/Script/Engine.SceneComponent|GetRelativeLocation (Variables|Default|GetArm)))
  (Rendering|Material|SetVectorParameterValue "/Game/FX/Materials/DissolvePortal/MPC_Data.MPC_Data" "Position" (Math|Conversions|ToLinearColor(Vector) (Transformation|GetWorldLocation _dissolve)) :!class /Script/Engine.KismetMaterialLibrary)
  (Rendering|Material|SetVectorParameterValue "/Game/FX/Materials/DissolvePortal/MPC_Data.MPC_Data" "Bounds" (Math|Conversions|ToLinearColor(Vector) (Transformation|GetWorldScale _dissolve)) :!class /Script/Engine.KismetMaterialLibrary))

(fn ConstructionScript
  (bind _dissolve (Variables|Default|GetDissolve))
  (Rendering|Material|SetVectorParameterValue "/Game/FX/Materials/DissolvePortal/MPC_Data.MPC_Data" "Position" (Math|Conversions|ToLinearColor(Vector) (Transformation|GetWorldLocation _dissolve)) :!class /Script/Engine.KismetMaterialLibrary)
  (Rendering|Material|SetVectorParameterValue "/Game/FX/Materials/DissolvePortal/MPC_Data.MPC_Data" "Bounds" (Math|Conversions|ToLinearColor(Vector) (Transformation|GetWorldScale _dissolve)) :!class /Script/Engine.KismetMaterialLibrary))