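; Boss arm actor that lunges at a given player location for the PortalAttack, then retracts.
; A timeline lerps it from its BeginPlay position to the target, reverses on reaching the end, and calls EndAttack once back at the start.
; Each update sphere-traces at the Scene component and damages a hit ThirdPersonCharacter through a DoOnce that is never reset, so only the first hit deals damage.
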(event Custom|PortalAttack
  (params (PlayerLoc :type Vector))
  (bind _movement (Variables|Default|GetMovement))
  (bind _scene (Variables|Default|GetScene))
  (bind _returnvalue (Transformation|GetWorldLocation _scene))
  (Variables|Default|SetPlayerLocation PlayerLoc)
  (bind _alpha (Timeline|Movement PlayFromStart)
    (:Update
      (Transformation|SetActorLocation (Math|Vector|Lerp(Vector) (Variables|Default|GetArmLoc) (Variables|Default|GetPlayerLocation) _alpha) false false)
      (bind _outhit (Collision|SphereTraceByChannel _returnvalue _returnvalue 26.0 "TraceTypeQuery1" false 0 "None"))
      (bind _asthird_person_character (Utilities|Casting|CastToThirdPersonCharacter (.HitActor (Collision|BreakHitResult _outhit))))
      (Utilities|FlowControl|DoOnce false
        (:Completed
          (Game|Damage|ApplyDamage _asthird_person_character 2.0 0 0))))
    (:Finished
      (if (!= (Components|Timeline|GetPlaybackPosition _movement) 0.0)
        (Components|Timeline|ReversefromEnd _movement)
        (else
          (Default|CallEndAttack))))))

(event Collision|EventActorBeginOverlap
  (params (OtherActor :type Actor%20Object%20Reference)))

(event EventTick
  (params (DeltaSeconds :type Float%20%28single-precision%29)))

(event EventBeginPlay
  (Variables|Default|SetArmLoc (Transformation|GetActorLocation)))

(fn ConstructionScript)