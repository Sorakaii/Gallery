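; Tutorial kamikaze enemy character that feeds its type, player reference and attack availability to an AI Blackboard.
; When its KamikazeFX finishes, a sphere trace damages a hit ThirdPersonCharacter and destroys the enemy.
; Navi interaction applies damage with directional FX; each hit removes one health, then briefly stuns it or destroys it at zero.
; Helpers handle attack montages, player focus and timeline-driven rotation toward a target.
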(event InteractwithOwner(C_Interactible)
  (bind _damagefx (Variables|Default|GetDamageFX))
  (bind _c_interactible (Variables|Default|GetC_Interactible))
  (bind _naviref (Variables|/Game/Blueprints/Interactible/C_Interactible.C_Interactible_C|GetnaviRef _c_interactible))
  (if (not (Variables|/Game/Blueprints/Navi/BP_NaviPawn.BP_NaviPawn_C|GethasAppliedDamage _naviref))
    (Game|Damage|ApplyDamage self 1.0 (AI|GetAIController _naviref) _naviref)
    (Effects|Components|ParticleSystem|SetVectorParameter _damagefx "User.DamageAngle" (Math|Vector|GetForwardVector (Math|Rotator|FindLookatRotation (Transformation|GetActorLocation _naviref) (Transformation|GetActorLocation self))))
    (Components|Activation|Activate _damagefx false)
    (Development|PrintString "Hello")))

(event OnSystemFinished(KamikazeFX)
  (params (PSystem :type Niagara%20Component%20Object%20Reference))
  (bind _returnvalue (Transformation|GetActorLocation))
  (bind (_outhit _returnvalue_2) (Collision|SphereTraceByChannel _returnvalue _returnvalue 2.5e+02 "TraceTypeQuery3" false 0 "ForDuration"))
  (if _returnvalue_2
    (bind _asthird_person_character (Utilities|Casting|CastToThirdPersonCharacter (.HitActor (Collision|BreakHitResult _outhit))))
    (Game|Damage|ApplyDamage _asthird_person_character 3.0 (Pawn|GetController) self)
    (Actor|DestroyActor)))

(event Custom|Restore%20Speed%20Value
  (CallFunction|UpdateWalkSpeed (Variables|Default|GetOld%20Move%20Speed)))

(event Custom|PlayMontageAttack
  (params (MontageToPlay :type Anim%20Montage%20Object%20Reference))
  (Variables|Default|SetcanAttack false)
  (Animation|Montage|PlayMontage (Variables|Character|GetMesh) MontageToPlay))

(event Custom|Rotate%20To%20Face%20Target
  (params (Target :type Actor%20Object%20Reference))
  (Components|Timeline|SetPlayRate (Variables|Default|GetTimeline_Rotation) 2.0)
  (bind _alpha (Timeline|Timeline_Rotation PlayFromStart)
    (:Update
      (Transformation|SetActorRotation (Math|Rotator|Lerp(Rotator) (Transformation|GetActorRotation) (Math|Rotator|FindLookatRotation (Transformation|GetActorLocation) (Transformation|GetActorLocation Target)) _alpha)))))

(event EventBeginPlay
  (Variables|Default|SetTransformRef (Transformation|GetActorTransform))
  (AI|Components|Blackboard|SetValueasEnum (AI|GetBlackboard 0) (Variables|Default|GetTypeName) (Variables|Default|GetType)))

(event Game|Damage|EventAnyDamage
  (params (Damage :type Float%20%28single-precision%29) (DamageType :type Damage%20Type%20Object%20Reference) (InstigatedBy :type Controller%20Object%20Reference) (DamageCauser :type Actor%20Object%20Reference))
  (if (not (Variables|Default|GetisDead))
    (Math|Float|DecrementFloat (Variables|Default|GetHealth)
      (:%20%20
        (if (<= (Variables|Default|GetHealth) 0.0)
          (Pawn|Components|CharacterMovement|DisableMovement (Variables|Character|GetCharacterMovement))
          (Default|MakeNotTargetable (Variables|Default|GetC_Interactible))
          (Class|LowEntryExtendedStandardLibrary|DelayFrames 1)
          (Variables|Default|SetisDead true)
          (Actor|DestroyActor)
          (else
            (CallFunction|UpdateWalkSpeed 0.0)
            (Utilities|Time|SetTimerbyEvent (delegate Custom|Restore%20Speed%20Value) (Variables|Default|GetHitStun))))))))

(event EventTick
  (params (DeltaSeconds :type Float%20%28single-precision%29)))

(event Collision|EventActorBeginOverlap
  (params (OtherActor :type Actor%20Object%20Reference)))

(fn ConstructionScript)

(fn UpdateWalkSpeed
  (params (Max%20Walk%20Speed :type Float%20%28single-precision%29))
  (bind _charactermovement (Variables|Character|GetCharacterMovement))
  (Variables|Default|SetOld%20Move%20Speed (Variables|/Script/Engine.CharacterMovementComponent|GetMaxWalkSpeed _charactermovement))
  (Variables|/Script/Engine.CharacterMovementComponent|SetMaxWalkSpeed _charactermovement Max%20Walk%20Speed))

(fn SetPlayerREF
  (params (Player :type Third%20Person%20Character%20Object%20Reference))
  (AI|Components|Blackboard|SetValueasObject (AI|GetBlackboard 0) (LocalVariables|GetPlayerREF) Player)
  (if (Utilities|IsValid Player)
    (AI|SetFocus (AI|GetAIController self) Player)))

(fn ResetAttackCooldown
  (CallFunction|SetCanAttack true))

(fn SetCanAttack
  (params (canAttack :type Boolean))
  (bind _output_get (Variables|Default|SetcanAttack canAttack))
  (AI|Components|Blackboard|SetValueasBool (AI|GetBlackboard 0) (LocalVariables|GetcanAttackName) _output_get))