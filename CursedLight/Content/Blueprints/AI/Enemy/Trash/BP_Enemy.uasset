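; Base AI enemy character, configured at construction from an EnemyType asset as Kamikaze, Melee or Range, feeding its blackboard and attack state.
; Navi interactions apply damage with directional FX.
; Each hit removes one health and briefly stops movement, while death refills the player's health and destroys the enemy.
; When the kamikaze FX finishes, a sphere trace damages the player and destroys the enemy if the player is hit.
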(event InteractwithOwner(C_Interactible)
  (bind _returnvalue (Utilities|Name|MakeLiteralName "naviMovementAnchorLocation"))
  (bind _c_interactible (Variables|Default|GetC_Interactible))
  (bind _naviattackbox (Variables|Default|GetNaviAttackBox))
  (bind _c_interactible_2 (Variables|Default|GetC_Interactible))
  (bind _naviref (Variables|/Game/Blueprints/Interactible/C_Interactible.C_Interactible_C|GetnaviRef _c_interactible_2))
  (bind _naviref_2 (Variables|/Game/Blueprints/Interactible/C_Interactible.C_Interactible_C|GetnaviRef _c_interactible))
  (bind _returnvalue_2 (AI|GetBlackboard _naviref))
  (bind _returnvalue_3 (AI|Components|Blackboard|GetValueasVector _returnvalue_2 _returnvalue))
  (if (not (Variables|/Game/Blueprints/Navi/BP_NaviPawn.BP_NaviPawn_C|GethasAppliedDamage _naviref_2))
    (Game|Damage|ApplyDamage self 1.0 (AI|GetAIController _naviref_2) _naviref_2)
    (bind _returnvalue_4 (Niagara|SpawnSystemAttached "/Game/FX/NiagaraSystem/NS_ExploNavi.NS_ExploNavi" _naviattackbox "None" _returnvalue_3 "0, 0, 0" "KeepRelativeOffset" false false))
    (Variables|Default|SetdamageFX _returnvalue_4)
    (Effects|Components|ParticleSystem|SetVectorParameter (Variables|Default|GetdamageFX) "User.DamageAngle" (Math|Vector|GetForwardVector (Math|Rotator|FindLookatRotation (Transformation|GetActorLocation (Variables|/Game/Blueprints/Interactible/C_Interactible.C_Interactible_C|GetnaviRef (Variables|Default|GetC_Interactible))) (+ (+ (Variables|/Script/Engine.SceneComponent|GetRelativeLocation _naviattackbox) _returnvalue_3) (Transformation|GetActorLocation self)))))
    (Components|Activation|Activate (Variables|Default|GetdamageFX) false)))

(event OnSystemFinished(KamikazeFX)
  (params (PSystem :type Niagara%20Component%20Object%20Reference))
  (bind _returnvalue (Transformation|GetActorLocation))
  (bind (_outhit _returnvalue_2) (Collision|SphereTraceByChannel _returnvalue _returnvalue 3e+02 "TraceTypeQuery3" false 0 "ForDuration"))
  (if _returnvalue_2
    (bind _asthird_person_character (Utilities|Casting|CastToThirdPersonCharacter (.HitActor (Collision|BreakHitResult _outhit))))
    (Game|Damage|ApplyDamage _asthird_person_character 3.0 (Pawn|GetController) self)
    (Actor|DestroyActor)))

(event Custom|Restore%20Speed%20Value
  (CallFunction|UpdateWalkSpeed (Variables|Default|GetOld%20Move%20Speed)))

(event Custom|PlayMontageAttack
  (params (MontageToPlay :type Anim%20Montage%20Object%20Reference))
  (Variables|Default|SetcanAttack false)
  (Animation|Montage|PlayMontage (Variables|Character|GetMesh) MontageToPlay
    (:OnCompleted
      (Variables|Default|SetcanAttack true))))

(event Custom|Rotate%20To%20Face%20Target
  (params (Target :type Actor%20Object%20Reference))
  (Components|Timeline|SetPlayRate (Variables|Default|GetTimeline_Rotation) 2.0)
  (bind _alpha (Timeline|Timeline_Rotation PlayFromStart)
    (:Update
      (Transformation|SetActorRotation (Math|Rotator|Lerp(Rotator) (Transformation|GetActorRotation) (Math|Rotator|FindLookatRotation (Transformation|GetActorLocation) (Transformation|GetActorLocation Target)) _alpha)))))

(event EventBeginPlay
  (Variables|Default|SetTransformRef (Transformation|GetActorTransform))
  (AI|Components|Blackboard|SetValueasEnum (AI|GetBlackboard 0) (Variables|Default|GetTypeName) (Variables|Default|GetType))
  (bind _asthird_person_character (Utilities|Casting|CastToThirdPersonCharacter (Game|GetPlayerCharacter 0)))
  (Variables|Default|SetplayerRef _asthird_person_character))

(event Game|Damage|EventAnyDamage
  (params (Damage :type Float%20%28single-precision%29) (DamageType :type Damage%20Type%20Object%20Reference) (InstigatedBy :type Controller%20Object%20Reference) (DamageCauser :type Actor%20Object%20Reference))
  (bind _playerref (Variables|Default|GetplayerRef))
  (if (not (Variables|Default|GetisDead))
    (Math|Float|DecrementFloat (Variables|Default|GetHealth)
      (:%20%20
        (if (<= (Variables|Default|GetHealth) 0.0)
          (Pawn|Components|CharacterMovement|DisableMovement (Variables|Character|GetCharacterMovement))
          (Default|MakeNotTargetable (Variables|Default|GetC_Interactible))
          (Class|LowEntryExtendedStandardLibrary|DelayFrames 1)
          (Variables|Default|SetisDead true)
          (Variables|/Game/Blueprints/Player/ThirdPersonCharacter.ThirdPersonCharacter_C|SetHealth _playerref (Variables|/Game/Blueprints/Player/ThirdPersonCharacter.ThirdPersonCharacter_C|GetmaxHealth _playerref))
          (Actor|DestroyActor)
          (else
            (CallFunction|UpdateWalkSpeed 0.0)
            (Utilities|Time|SetTimerbyEvent (delegate Custom|Restore%20Speed%20Value) (Variables|Default|GetHitStun))))))))

(event EventTick
  (params (DeltaSeconds :type Float%20%28single-precision%29)))

(event Collision|EventActorBeginOverlap
  (params (OtherActor :type Actor%20Object%20Reference)))

(fn ConstructionScript
  (bind _enemy_type (Variables|Default|GetEnemy%20Type)
    (:then
      (Components|SkinnedMesh|SetSkinnedAssetandUpdate (Variables|Character|GetMesh) (Variables|/Game/Blueprints/AI/Enemy/Trash/DataAssets/PDA_Enemy.PDA_Enemy_C|GetMesh _enemy_type) true)
      (Class|SkeletalMeshComponent|SetAnimClass (Variables|Character|GetMesh) (Variables|/Game/Blueprints/AI/Enemy/Trash/DataAssets/PDA_Enemy.PDA_Enemy_C|GetABP (Variables|Default|GetEnemy%20Type)))
      (Variables|Default|SetType (Variables|/Game/Blueprints/AI/Enemy/Trash/DataAssets/PDA_Enemy.PDA_Enemy_C|GetEnemy%20Class (Variables|Default|GetEnemy%20Type)))
      (Variables|Default|SetAttack%20Range (Variables|/Game/Blueprints/AI/Enemy/Trash/DataAssets/PDA_Enemy.PDA_Enemy_C|GetAttack%20Range (Variables|Default|GetEnemy%20Type)))
      (Variables|Default|SetHealth (Variables|/Game/Blueprints/AI/Enemy/Trash/DataAssets/PDA_Enemy.PDA_Enemy_C|GetHealth (Variables|Default|GetEnemy%20Type)))
      (Components|Capsule|SetCapsuleHalfHeight (Variables|Collision|GetCapsuleComponent) (Utilities|Select :Index (Variables|Default|GetType) :NewEnumerator0 44.0 :NewEnumerator1 88.0 :NewEnumerator2 88.0) true)
      (Transformation|SetRelativeLocation (Variables|Character|GetMesh) (Math|Vector|MakeVector 0.0 0.0 (* (Variables|/Script/Engine.CapsuleComponent|GetCapsuleHalfHeight (Variables|Collision|GetCapsuleComponent)) -1.0)) false false)
      (Rendering|Material|SetMaterial (Variables|Character|GetMesh) 0 "/Game/Assets/GA_Assets/TextureMobShade/m_BodyEffect_Inst.m_BodyEffect_Inst")
      (Transformation|SetRelativeLocation (Variables|Default|GetC_Interactible) (Math|Vector|MakeVector 0.0 0.0 (- (Variables|/Script/Engine.CapsuleComponent|GetCapsuleHalfHeight (Variables|Collision|GetCapsuleComponent)) 2.0)) false false))
    (:else)))

(fn UpdateWalkSpeed
  (params (Max%20Walk%20Speed :type Float%20%28single-precision%29))
  (bind _charactermovement (Variables|Character|GetCharacterMovement))
  (Variables|Default|SetOld%20Move%20Speed (Variables|/Script/Engine.CharacterMovementComponent|GetMaxWalkSpeed _charactermovement))
  (Variables|/Script/Engine.CharacterMovementComponent|SetMaxWalkSpeed _charactermovement Max%20Walk%20Speed))

(fn SetPlayerREF
  (params (Player :type Third%20Person%20Character%20Object%20Reference))
  (AI|Components|Blackboard|SetValueasObject (AI|GetBlackboard 0) (LocalVariables|GetPlayerRefKeyName) Player)
  (if (Utilities|IsValid Player)
    (AI|SetFocus (AI|GetAIController self) Player)))

(fn ResetAttackCooldown
  (CallFunction|SetCanAttack true))

(fn SetCanAttack
  (params (canAttack :type Boolean))
  (bind _output_get (Variables|Default|SetcanAttack canAttack))
  (AI|Components|Blackboard|SetValueasBool (AI|GetBlackboard 0) (LocalVariables|GetcanAttackName) _output_get))