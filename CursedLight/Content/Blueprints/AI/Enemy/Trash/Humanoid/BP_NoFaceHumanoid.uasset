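; Humanoid trash enemy configured from a data asset (range, health, type, material), passing range and type to its AI Blackboard.
; Perceiving an ALS player-character class sets the player as Blackboard target.
; Each hit removes one health, briefly halting movement with a hit montage, or at zero playing a montage before destruction.
; A custom Explosion event sphere-traces after a short delay, damages a hit ALS character and destroys the enemy.
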(event OnTargetPerceptionUpdated(AIPerception)
  (params (Actor :type Actor%20Object%20Reference) (Stimulus :type AI%20Stimulus%20Structure))
  (if (== (Utilities|GetClass Actor) "/Game/Blueprints/ALS/Blueprints/CharacterLogic/ALS_AnimMan_CharacterBP.ALS_AnimMan_CharacterBP_C")
    (AI|Components|Blackboard|SetValueasObject (Variables|/Script/AIModule.AIController|GetBlackboard (AI|GetAIController self)) (Variables|AI|GettargetKeyName) (Game|GetPlayerCharacter 0))))

(event Custom|Explosion
  (bind _returnvalue (Transformation|GetActorLocation))
  (Utilities|FlowControl|Delay 0.2)
  (bind _outhit (Collision|SphereTraceByChannel _returnvalue _returnvalue 5e+02 "TraceTypeQuery1" false 0 "ForDuration"))
  (bind _asals_anim_man_character_bp (Utilities|Casting|CastToALS_AnimMan_CharacterBP (.HitActor (Collision|BreakHitResult _outhit)))
    (:then
      (Game|Damage|ApplyDamage _asals_anim_man_character_bp 1.0 (Pawn|GetController) self))
    (:CastFailed
      _))
  (Actor|DestroyActor))

(event EventBeginPlay
  (AI|Components|Blackboard|SetValueasFloat (Variables|/Script/AIModule.AIController|GetBlackboard (AI|GetAIController self)) (Variables|Ai|GetattackRangeKeyName) (Variables|Default|GetattackRange))
  (bind _asthird_person_character (Utilities|Casting|CastToThirdPersonCharacter (Game|GetPlayerCharacter 0)))
  (Variables|Default|SetplayerRef _asthird_person_character)
  (Variables|Default|SetCachedWalkSpeed (Variables|/Script/Engine.CharacterMovementComponent|GetMaxWalkSpeed (Variables|Character|GetCharacterMovement)))
  (AI|Components|Blackboard|SetValueasEnum (AI|GetBlackboard 0) (Utilities|Name|MakeLiteralName "type") (Variables|Default|GetAITypes)))

(event Game|Damage|EventAnyDamage
  (params (Damage :type Float%20%28single-precision%29) (DamageType :type Damage%20Type%20Object%20Reference) (InstigatedBy :type Controller%20Object%20Reference) (DamageCauser :type Actor%20Object%20Reference))
  (if (not (Variables|Default|GetIsDead))
    (Math|Float|DecrementFloat (Variables|Default|GetHealth)
      (:%20%20
        (if (<= (Variables|Default|GetHealth) 0.0)
          (Pawn|Components|CharacterMovement|DisableMovement (Variables|Character|GetCharacterMovement))
          (Variables|Default|SetIsDead true)
          (Animation|Montage|PlayMontage (Variables|Character|GetMesh) "/Game/Characters/Mannequin/Animations/AM_ReleaseStunNoFace4UE4.AM_ReleaseStunNoFace4UE4"
            (:then
              (Utilities|FlowControl|Delay 1.0)
              (Actor|DestroyActor)))
          (else
            (Utilities|FlowControl|Sequence
              (:then_0
                (Variables|/Script/Engine.CharacterMovementComponent|SetMaxWalkSpeed (Variables|Character|GetCharacterMovement) 0.0)
                (Animation|Montage|PlayMontage (Variables|Character|GetMesh) "/Game/Characters/Mannequin/Animations/AM_Hit.AM_Hit"))
              (:then_1
                (Utilities|FlowControl|RetriggerableDelay 1.0)
                (Variables|/Script/Engine.CharacterMovementComponent|SetMaxWalkSpeed (Variables|Character|GetCharacterMovement) (Variables|Default|GetCachedWalkSpeed))))))))))

(fn ConstructionScript
  (bind _aidataassets (Variables|Default|GetAIDataAssets))
  (if (Utilities|IsValid (Variables|Default|GetAIDataAssets))
    (Variables|Default|SetattackRange (Variables|/Game/Blueprints/AI/Enemy/Trash/Humanoid/DataAssets/PDA_AIEnnemyBase.PDA_AIEnnemyBase_C|GetAttackRange _aidataassets))
    (Variables|Default|SetHealth (Variables|/Game/Blueprints/AI/Enemy/Trash/Humanoid/DataAssets/PDA_AIEnnemyBase.PDA_AIEnnemyBase_C|GetHealth _aidataassets))
    (Variables|Default|SetAITypes (Variables|/Game/Blueprints/AI/Enemy/Trash/Humanoid/DataAssets/PDA_AIEnnemyBase.PDA_AIEnnemyBase_C|GetAIType _aidataassets))
    (Rendering|Material|SetMaterial (Variables|Character|GetMesh) 0 (Variables|/Game/Blueprints/AI/Enemy/Trash/Humanoid/DataAssets/PDA_AIEnnemyBase.PDA_AIEnnemyBase_C|GetMI _aidataassets))))