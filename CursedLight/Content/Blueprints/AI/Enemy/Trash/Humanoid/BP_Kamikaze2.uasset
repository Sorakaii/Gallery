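; Kamikaze humanoid enemy that punches, then blows itself up, with its AI type written to the blackboard on BeginPlay.
; MeleeAttack stops movement and plays a left punch montage for its first two calls, tracked by AttackCount.
; When a punch completes, walking resumes, and after a short delay an explosion montage plays, calling Explosion on blend out.
; Left-hand overlaps damage any ALS_AnimMan_CharacterBP, independent of the attack state.
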(event OnComponentBeginOverlap(LeftHand)
  (params (OverlappedComponent :type Primitive%20Component%20Object%20Reference) (OtherActor :type Actor%20Object%20Reference) (OtherComp :type Primitive%20Component%20Object%20Reference) (OtherBodyIndex :type Integer) (bFromSweep :type Boolean) (SweepResult :type Hit%20Result%20Structure%20%28by%20ref%29))
  (bind _asals_anim_man_character_bp (Utilities|Casting|CastToALS_AnimMan_CharacterBP OtherActor))
  (Game|Damage|ApplyDamage _asals_anim_man_character_bp 1.0 0 0))

(event EventBeginPlay
  (|CallParentFunction)
  (AI|Components|Blackboard|SetValueasEnum (AI|GetBlackboard 0) (Utilities|Name|MakeLiteralName "type") (Variables|Default|GetAI_Type)))

(event EventTick
  (params (DeltaSeconds :type Float%20%28single-precision%29))
  (|CallParentFunction DeltaSeconds) ; This node is disabled and will not be called.\nDrag off pins to build functionality.
)

(event EventMeleeAttack
  (bind _charactermovement (Variables|Character|GetCharacterMovement))
  (Pawn|Components|CharacterMovement|DisableMovement _charactermovement)
  (switch int (Variables|Default|GetAttackCount)
    (:0
      (Variables|Default|SetAttackCount 1)
      (Animation|Montage|PlayMontage (Variables|Character|GetMesh) "/Game/Characters/Mannequin/Animations/AM_Fists_Punch_L_Montage.AM_Fists_Punch_L_Montage"
        (:OnCompleted
          _)))
    (:1
      (Variables|Default|SetAttackCount 2)
      (Animation|Montage|PlayMontage (Variables|Character|GetMesh) "/Game/Characters/Mannequin/Animations/AM_Fists_Punch_L_Montage.AM_Fists_Punch_L_Montage"
        (:OnCompleted
          _))))
  (Pawn|Components|CharacterMovement|SetMovementMode _charactermovement "MOVE_Walking" 0)
  (Utilities|FlowControl|Delay 2.5)
  (Animation|Montage|PlayMontage (Variables|Character|GetMesh) "/Game/Characters/Mannequin/Animations/AM_Explosion.AM_Explosion"
    (:OnBlendOut
      (CallFunction|Explosion))))

(fn ConstructionScript
  (|CallParentFunction))