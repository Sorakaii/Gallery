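; Close-combat humanoid enemy AI character that writes its AI type to the blackboard on BeginPlay and provides a Punch attack.
; Punch box-traces from the right hand to damage a pawn immediately, then disables movement during the punch montage and restores walking on completion.
; A Sphere hit handler also damages the ALS character, but compares its own hit component to that character's capsule.
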(event OnComponentBeginOverlap(Sphere)
  (params (OverlappedComponent :type Primitive%20Component%20Object%20Reference) (OtherActor :type Actor%20Object%20Reference) (OtherComp :type Primitive%20Component%20Object%20Reference) (OtherBodyIndex :type Integer) (bFromSweep :type Boolean) (SweepResult :type Hit%20Result%20Structure%20%28by%20ref%29)))

(event OnComponentHit(Sphere)
  (params (HitComponent :type Primitive%20Component%20Object%20Reference) (OtherActor :type Actor%20Object%20Reference) (OtherComp :type Primitive%20Component%20Object%20Reference) (NormalImpulse :type Vector :default "0, 0, 0") (Hit :type Hit%20Result%20Structure%20%28by%20ref%29))
  (bind _asals_anim_man_character_bp (Utilities|Casting|CastToALS_AnimMan_CharacterBP OtherActor))
  (if (== HitComponent (Variables|/Script/Engine.Character|GetCapsuleComponent _asals_anim_man_character_bp))
    (Game|Damage|ApplyDamage _asals_anim_man_character_bp 1.0 0 0)))

(event EventBeginPlay
  (|CallParentFunction)
  (AI|Components|Blackboard|SetValueasEnum (AI|GetBlackboard 0) (Utilities|Name|MakeLiteralName "type") (Variables|Default|GetAI_Type)))

(event Collision|EventActorBeginOverlap
  (params (OtherActor :type Actor%20Object%20Reference)))

(event EventTick
  (params (DeltaSeconds :type Float%20%28single-precision%29))
  (|CallParentFunction DeltaSeconds) ; This node is disabled and will not be called.\nDrag off pins to build functionality.
)

(event EventPunch
  (bind _charactermovement (Variables|Character|GetCharacterMovement))
  (CallFunction|HitMarker)
  (Pawn|Components|CharacterMovement|DisableMovement _charactermovement)
  (Animation|Montage|PlayMontage (Variables|Character|GetMesh) "/Game/Characters/Mannequin/Animations/AM_StrongPunch.AM_StrongPunch"
    (:OnCompleted
      (Pawn|Components|CharacterMovement|SetMovementMode _charactermovement "MOVE_Walking" 0))))

(fn ConstructionScript
  (|CallParentFunction))

(fn HitMarker
  (bind _mesh (Variables|Character|GetMesh))
  (bind _returnvalue (Math|Vector|GetForwardVector _mesh))
  (bind _returnvalue_2 (Transformation|GetSocketLocation _mesh "hand_r"))
  (bind (_outhit _returnvalue_3) (Class|KismetSystemLibrary|BoxTraceSingleforObjects _returnvalue_2 (+ _returnvalue_2 (* _returnvalue 3e+01)) "25.000000,65.000000,25.000000" (Math|Conversions|RotationFromXVector _returnvalue) (Utilities|Array|MakeArray "ObjectTypeQuery3") true 0 "None" true))
  (if _returnvalue_3
    (Game|Damage|ApplyDamage (.HitActor (Collision|BreakHitResult _outhit)) 1.0 0 0)))