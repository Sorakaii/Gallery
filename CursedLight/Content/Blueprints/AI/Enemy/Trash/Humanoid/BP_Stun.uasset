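; Humanoid trash enemy that stuns the player when its capsule overlaps the third-person character.
; On BeginPlay it writes its AI type to the blackboard and binds to the player's QTE result dispatcher.
; When that dispatcher fires, it plays a release montage, waits out the fall duration, plays a stand-up montage and restarts its AI brain logic on blend out.
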(event OnComponentBeginOverlap(CapsuleComponent)
  (params (OverlappedComponent :type Primitive%20Component%20Object%20Reference) (OtherActor :type Actor%20Object%20Reference) (OtherComp :type Primitive%20Component%20Object%20Reference) (OtherBodyIndex :type Integer) (bFromSweep :type Boolean) (SweepResult :type Hit%20Result%20Structure%20%28by%20ref%29))
  (bind _asthird_person_character (Utilities|Casting|CastToThirdPersonCharacter OtherActor))
  (Variables|/Game/Blueprints/Player/ThirdPersonCharacter.ThirdPersonCharacter_C|SetIsStun _asthird_person_character true))

(event Custom|PlayerFreed
  (Animation|Montage|PlayMontage (Variables|Character|GetMesh) "/Game/Characters/Mannequin/Animations/AM_ReleaseStunNoFace4UE4.AM_ReleaseStunNoFace4UE4"
    (:then
      (Utilities|FlowControl|Delay (Variables|Default|GetfallDuration))
      (Animation|Montage|PlayMontage (Variables|Character|GetMesh) "/Game/Characters/Mannequin/Animations/AM_StandUpNoFace4UE4.AM_StandUpNoFace4UE4"
        (:OnBlendOut
          (Class|BrainComponent|RestartLogic (Variables|/Script/AIModule.AIController|GetBrainComponent (AI|GetAIController self))))))))

(event EventBeginPlay
  (|CallParentFunction)
  (AI|Components|Blackboard|SetValueasEnum (AI|GetBlackboard 0) (Utilities|Name|MakeLiteralName "type") (Variables|Default|GetAITypes))
  (EventDispatchers|BindEventtoQTEResultDispatcher (Variables|Default|GetplayerRef) (delegate Custom|PlayerFreed)))

(event Collision|EventActorBeginOverlap
  (params (OtherActor :type Actor%20Object%20Reference)))

(event EventTick
  (params (DeltaSeconds :type Float%20%28single-precision%29)))

(event Game|Damage|EventAnyDamage
  (params (Damage :type Float%20%28single-precision%29) (DamageType :type Damage%20Type%20Object%20Reference) (InstigatedBy :type Controller%20Object%20Reference) (DamageCauser :type Actor%20Object%20Reference))
  (|CallParentFunction Damage DamageType InstigatedBy DamageCauser))

(fn ConstructionScript)