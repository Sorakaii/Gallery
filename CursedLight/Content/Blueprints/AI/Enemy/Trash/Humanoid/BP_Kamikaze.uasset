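; Kamikaze humanoid trash enemy that blows itself up to damage an ALS character nearby.
; On BeginPlay it writes its AI type to the blackboard's "type" key.
; The Explosion event, not called within this graph, starts a Niagara effect, waits briefly, then runs a single-hit sphere trace at its own location.
; It applies damage only if that hit is an ALS_AnimMan_CharacterBP, then destroys itself either way.
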(event Custom|Explosion
  (bind _returnvalue (Transformation|GetActorLocation))
  (Components|Activation|Activate (Variables|Default|GetNiagara_0) false)
  (Utilities|FlowControl|Delay 2.0)
  (bind _outhit (Collision|SphereTraceByChannel _returnvalue _returnvalue 5e+02 "TraceTypeQuery1" false 0 "None"))
  (bind _asals_anim_man_character_bp (Utilities|Casting|CastToALS_AnimMan_CharacterBP (.HitActor (Collision|BreakHitResult _outhit)))
    (:then
      (bind _returnvalue_2 (Game|Damage|ApplyDamage _asals_anim_man_character_bp 1.0 (Pawn|GetController) self)))
    (:CastFailed
      _))
  (Actor|DestroyActor))

(event EventBeginPlay
  (|CallParentFunction)
  (AI|Components|Blackboard|SetValueasEnum (AI|GetBlackboard 0) (Utilities|Name|MakeLiteralName "type") (Variables|Default|GetAITypes)))

(event Game|Damage|EventAnyDamage
  (params (Damage :type Float%20%28single-precision%29) (DamageType :type Damage%20Type%20Object%20Reference) (InstigatedBy :type Controller%20Object%20Reference) (DamageCauser :type Actor%20Object%20Reference))
  (|CallParentFunction Damage DamageType InstigatedBy DamageCauser))

(fn ConstructionScript)