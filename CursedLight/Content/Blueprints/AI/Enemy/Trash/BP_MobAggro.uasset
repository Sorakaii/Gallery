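; BP_MobAggro is a group aggro trigger that alerts nearby enemies when the player enters its sphere.
; On overlap with a ThirdPersonCharacter, it stores that character as PlayerREF and runs a near zero-length multi sphere trace matching the sphere's radius.
; Each BP_Enemy hit receives the player reference through SetPlayerREF, so enemies in range gain their target together.
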(event OnComponentBeginOverlap(Sphere)
  (params (OverlappedComponent :type Primitive%20Component%20Object%20Reference) (OtherActor :type Actor%20Object%20Reference) (OtherComp :type Primitive%20Component%20Object%20Reference) (OtherBodyIndex :type Integer) (bFromSweep :type Boolean) (SweepResult :type Hit%20Result%20Structure%20%28by%20ref%29))
  (bind _returnvalue (Transformation|GetActorLocation))
  (bind _asthird_person_character (Utilities|Casting|CastToThirdPersonCharacter OtherActor))
  (Variables|Default|SetPlayer%20REF _asthird_person_character)
  (bind _outhits (Collision|MultiSphereTraceByChannel _returnvalue (+ _returnvalue "0,0,1.000000") (Variables|/Script/Engine.SphereComponent|GetSphereRadius (Variables|Default|GetSphere)) "TraceTypeQuery4" false 0 "None"))
  (for _array_element _outhits
    (bind _asbp_enemy (Utilities|Casting|CastToBP_Enemy (.HitActor (Collision|BreakHitResult _array_element))))
    (Default|SetPlayerREF _asbp_enemy (Variables|Default|GetPlayer%20REF))))

(event EventBeginPlay)

(event Collision|EventActorBeginOverlap
  (params (OtherActor :type Actor%20Object%20Reference)))

(event EventTick
  (params (DeltaSeconds :type Float%20%28single-precision%29)))

(fn ConstructionScript)