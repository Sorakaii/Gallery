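; Enemy homing projectile that detonates on the player, used by a trash enemy.
; An overlap on DetectPlayer sets the player as homing target, and proximity on Tick or a five-second timer triggers a one-shot explosion.
; Timelines lower max speed and ramp the sphere's material displacement before Niagara activates.
; That activation sphere-traces to damage the player and re-enables the owner's attack; the actor is destroyed when the effect finishes.
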(event OnComponentBeginOverlap(DetectPlayer)
  (params (OverlappedComponent :type Primitive%20Component%20Object%20Reference) (OtherActor :type Actor%20Object%20Reference) (OtherComp :type Primitive%20Component%20Object%20Reference) (OtherBodyIndex :type Integer) (bFromSweep :type Boolean) (SweepResult :type Hit%20Result%20Structure%20%28by%20ref%29))
  ;[0.1273 0 0.1406] Start Homing
  (bind _asthird_person_character (Utilities|Casting|CastToThirdPersonCharacter OtherActor))
  (Variables|Default|SetPlayer%20REF _asthird_person_character)
  (Variables|/Script/Engine.ProjectileMovementComponent|SetHomingTargetComponent (Variables|Default|GetProjectileMovement) (Variables|/Game/Blueprints/Player/ThirdPersonCharacter.ThirdPersonCharacter_C|GettargetableCollision (Variables|Default|GetPlayer%20REF))))

(event OnSystemFinished(Niagara)
  (params (PSystem :type Niagara%20Component%20Object%20Reference))
  (Actor|DestroyActor))

(event OnComponentActivated(Niagara)
  (params (Component :type Actor%20Component%20Object%20Reference) (bReset :type Boolean))
  (bind _returnvalue (Transformation|GetActorLocation))
  (bind _outhit (Collision|SphereTraceByChannel _returnvalue _returnvalue 1e+02 "TraceTypeQuery3" false 0 "None"))
  (Default|SetCanAttack (Variables|Default|GetOwner%20REF) true)
  (bind _asthird_person_character (Utilities|Casting|CastToThirdPersonCharacter (.HitActor (Collision|BreakHitResult _outhit))))
  (Game|Damage|ApplyDamage _asthird_person_character 3.0 0 0))

(event Custom|Explosion
  (Utilities|FlowControl|DoOnce false
    (:Completed
      (CallFunction|SetMaterialParametersValue))))

(event Custom|SetMaterialParametersValue
  (CallFunction|SetSpeedValue)
  (bind _alpha (Timeline|Timeline_0 PlayFromStart)
    (:Update
      (Rendering|Material|SetScalarParameterValueonMaterials (Variables|Default|GetSphere) "DispAmount" (Math|Float|Lerp 2.0 1e+01 _alpha))
      (Rendering|Material|SetScalarParameterValueonMaterials (Variables|Default|GetSphere) "Speed" (Math|Float|Lerp 1e+01 3e+01 _alpha)))
    (:Finished
      (Components|Activation|Activate (Variables|Default|GetNiagara) false)
      (Rendering|SetVisibility (Variables|Default|GetSphere) false false))))

(event Custom|Set%20Speed%20Value
  (bind _alpha (Timeline|Timeline_1 PlayFromStart)
    (:Update
      (Variables|/Script/Engine.ProjectileMovementComponent|SetMaxSpeed (Variables|Default|GetProjectileMovement) (Math|Float|Lerp 2.5e+02 1e+02 _alpha)))))

(event EventBeginPlay
  (Utilities|Time|SetTimerbyEvent (delegate Custom|Explosion) 5.0))

(event EventTick
  (params (DeltaSeconds :type Float%20%28single-precision%29))
  ;[1 0.1673 0] Player Detection
  (bind _player_ref (Variables|Default|GetPlayer%20REF)
    (:then
      (if (<= (Transformation|GetDistanceTo _player_ref) (Variables|Default|GetDetectionExplosion))
        (CallFunction|Explosion)))
    (:else)))

(fn ConstructionScript)