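; Tutorial kamikaze enemy that wakes when the player targets it, then charges and self-destructs on contact.
; Tick polls the player's target, then triggers a camera cinematic on itself, locking player movement until the camera returns.
; It then chases via AIMoveTo, retrying failed requests.
; Sphere overlap stops it and plays a headbutt montage, whose end activates the Kamikaze component, damages the player and destroys the actor.
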(event OnComponentBeginOverlap(Sphere)
  (params (OverlappedComponent :type Primitive%20Component%20Object%20Reference) (OtherActor :type Actor%20Object%20Reference) (OtherComp :type Primitive%20Component%20Object%20Reference) (OtherBodyIndex :type Integer) (bFromSweep :type Boolean) (SweepResult :type Hit%20Result%20Structure%20%28by%20ref%29))
  (if (== OtherActor (Variables|Default|GetplayerRef))
    (Components|Movement|StopMovementImmediately (Variables|Character|GetCharacterMovement))
    (Animation|Montage|PlayMontage (Variables|Character|GetMesh) "/Game/Assets/GA_Assets/Mobs/TrashMob_A/Animations/AM_Headbutt_Attack.AM_Headbutt_Attack"
      (:OnCompleted
        _)
      (:OnBlendOut
        _)
      (:OnInterrupted
        _))
    (Components|Activation|Activate (Variables|Default|GetKamikaze) false)
    (Game|Damage|ApplyDamage (Variables|Default|GetplayerRef) 1e+01 0 0)
    (Actor|DestroyActor)))

(event Custom|ActivateAI
  (bind _playerref (Variables|Default|GetplayerRef))
  (bind _camera (Variables|Default|GetCamera))
  (bind _returnvalue (Transformation|GetWorldTransform _camera))
  (bind _cameramanagerref (Variables|/Game/Blueprints/Player/ThirdPersonCharacter.ThirdPersonCharacter_C|GetCameraManagerRef _playerref))
  (Default|SetMovementCapabilities (Variables|Default|GetplayerRef) false false false)
  (Transformation|SetRelativeLocationAndRotation _camera "0.000000,-500.000000,300.000000" (Math|Rotator|FindLookatRotation (Math|Vector|MakeVector 0.0 -5e+02 3e+02) (Variables|/Script/Engine.SceneComponent|GetRelativeLocation (Variables|Character|GetMesh))) false false)
  (Default|Cinematic _cameramanagerref (Utilities|Array|MakeArray (Math|Transform|MakeTransform (.location _returnvalue) (.rotation _returnvalue) "1.000000,1.000000,1.000000")) (Utilities|Array|MakeArray 1.0 2.0) false)
  (Class|LowEntryLatentActionNone|WaitTillDone (Variables|/Game/Blueprints/Camera/ALS/ALS_PlayerCameraManager.ALS_PlayerCameraManager_C|GetreverseMoveCamAction _cameramanagerref))
  (Default|SetMovementCapabilities (Variables|Default|GetplayerRef) true true true)
  (CallFunction|Move))

(event Custom|Move
  (AI|AIMoveTo (AI|GetAIController self) "0, 0, 0" (Variables|Default|GetplayerRef) -1.0 "Default" "Default" true true
    (:then
      (Transformation|SetActorRotation (Math|Rotator|FindLookatRotation (Transformation|GetActorLocation) (Transformation|GetActorLocation (Variables|Default|GetplayerRef)))))
    (:OnRequestFailed
      (CallFunction|Move))))

(event EventBeginPlay
  (bind _asthird_person_character (Utilities|Casting|CastToThirdPersonCharacter (Game|GetPlayerCharacter 0)))
  (Variables|Default|SetplayerRef _asthird_person_character))

(event Collision|EventActorBeginOverlap
  (params (OtherActor :type Actor%20Object%20Reference)))

(event EventTick
  (params (DeltaSeconds :type Float%20%28single-precision%29))
  (if (== (Default|GetTargetedActor (Variables|Default|GetplayerRef)) self)
    (CallFunction|ActivateAI)
    (Actor|Tick|SetActorTickEnabled false)))

(fn ConstructionScript)