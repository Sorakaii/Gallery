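; Navi companion pawn that rides an attach actor and attacks the player's locked-on target.
; Movement states go to the AI blackboard, whose points feed timeline-driven Bezier paths with a floor-height clamp and drag slowdown.
; Attacks include trail slashes, combo projectiles and a QTE ultimate that slows BP_NoFaceHumanoid actors, then on success fires timed bursts.
; A dynamic material shared with the trail handles color fades.
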(event Custom|SlowMoQte
  ;[1 0 0.007763] QTEThings TOREFACTOR
  (bind _outactors (Actor|GetAllActorsOfClass "/Game/Blueprints/AI/Enemy/Trash/Humanoid/BP_NoFaceHumanoid.BP_NoFaceHumanoid_C"))
  (Utilities|FlowControl|FlipFlop
    (:A
      (for _array_element _outactors
        (Variables|/Script/Engine.Actor|SetCustomTimeDilation _array_element 0.2)))
    (:B
      (for _array_element_2 _outactors
        (Variables|/Script/Engine.Actor|SetCustomTimeDilation _array_element_2 1.0)))))

(event Custom|SlashAttack
  ;[0 0.3084 1] New Attack Navi
  (Variables|Default|SethasAppliedDamage true)
  (Components|Activation|Activate (Variables|Default|GetAttackTrail) true))

(event Custom|playerLockUpdate
  ;[0 0.04589 1] BeginPlay
  (CallFunction|FPlayerLockUpdate))

(event Custom|BurstUlt
  (bind _playerref (Variables|Refs|GetplayerRef))
  ;[0 0.3084 1] New Attack Navi
  (if (and (Variables|/Game/Blueprints/Player/ThirdPersonCharacter.ThirdPersonCharacter_C|GetisLock _playerref) (< (Variables|burstUlt|GetburstUltCount) 500))
    (if (Utilities|ClassIsChildOf (Utilities|GetClass (Default|GetTargetedActor _playerref)) "/Script/Engine.Character")
      (bind _returnvalue (Game|SpawnActorfromClass "/Game/Blueprints/Navi/UltBurst/BP_Burst.BP_Burst_C" (Math|Transform|MakeTransform (.location (Transformation|GetActorTransform self)) "0, 0, 0" "1.000000,1.000000,1.000000") "AlwaysSpawn" 0 1 0))
      (Default|Attack _returnvalue self (Default|GetTargetedActor (Variables|Refs|GetplayerRef)))
      (Math|Integer|IncrementInt (Variables|burstUlt|GetburstUltCount)))
    (else
      (Variables|burstUlt|SetburstUltCount 0)
      (Utilities|Time|ClearandInvalidateTimerbyHandle (Variables|burstUlt|GetburstUltTimer))
      (Utilities|FlowControl|Delay 1.0)
      (Actor|DestroyActor (Default|GetTargetedActor (Variables|Refs|GetplayerRef))))))

(event Custom|Ult
  ;[0 0.3084 1] New Attack Navi
  (bind _returnvalue (Utilities|Time|SetTimerbyEvent (delegate Custom|BurstUlt) 0.005 true))
  (Variables|burstUlt|SetburstUltTimer _returnvalue))

(event Custom|QteUlt
  ;[1 0 0.007763] QTEThings TOREFACTOR
  (bind _returnvalue (UserInterface|CreateWidget "/Game/Blueprints/UI/QTE/WBP_QTEUlt.WBP_QTEUlt_C" 0 self))
  (bind _output_get (Variables|burstUlt|SetburstUltQTEWidget _returnvalue))
  (UserInterface|Viewport|AddtoViewport _output_get 0)
  (Default|SetMovementCapabilities (Variables|Refs|GetplayerRef) false false true)
  (CallFunction|SlowMoQte))

(event Custom|MainMovementEvent
  (params (playRate :type Float%20%28double-precision%29) (Drag :type Float%20%28double-precision%29) (BezierCurveType :type EBezierCurveType%20Enum :default "NewEnumerator0"))
  ;[0 1 0.08878] NaviMovement
  (Variables|Default|SethasAppliedDamage false)
  (Components|Timeline|SetPlayRate (Variables|Default|GetMainMovementTimeline) playRate)
  (bind _alpha (Timeline|MainMovementTimeline PlayFromStart)
    (:Update
      (bind _output_get (Variables|NaviMovement|SetalphaMainMovementTimeline _alpha))
      (CallFunction|FUpdateNaviLocationinTimeline _output_get Drag BezierCurveType))
    (:Finished
      (Default|CallOnMovementTimelineFinished))))

(event Custom|DeactivateNiag
  ;[0 0.3084 1] New Attack Navi
  (Utilities|FlowControl|Delay 0.2)
  (Components|Activation|Deactivate (Variables|Default|GetAttackTrail))
  (Variables|Default|SethasAppliedDamage false))

(event Custom|QTESucess
  ;[1 0 0.007763] QTEThings TOREFACTOR
  (CallFunction|Ult)
  (CallFunction|SlowMoQte)
  (Default|SetMovementCapabilities (Variables|Refs|GetplayerRef) true true true)
  (Widget|RemovefromParent (Variables|burstUlt|GetburstUltQTEWidget))
  (Variables|burstUlt|SetburstUltQTEWidget 0)
  (Utilities|Platform|CollectGarbage)
  (Utilities|FlowControl|Delay 1.0)
  (if (Variables|/Game/Blueprints/Player/ThirdPersonCharacter.ThirdPersonCharacter_C|GetisLock (Variables|Refs|GetplayerRef))
    (CallFunction|UpdateMovementTypeinBlackboard "NewEnumerator4")
    (else
      (CallFunction|UpdateMovementTypeinBlackboard "NewEnumerator0"))))

(event Custom|attackThreeCombo
  (bind _self self)
  (bind _self_2 self)
  (bind _self_3 self)
  (bind _returnvalue (Transformation|GetActorTransform _self))
  (bind _returnvalue_2 (Transformation|GetActorTransform _self_2))
  (bind _returnvalue_3 (Transformation|GetActorTransform _self_3))
  ;[0 1 0.9378] AttackThreeCombo
  (Utilities|Time|ClearandInvalidateTimerbyHandle (Variables|AttackCombo|GetattackThreeComboResetComboTimer))
  (if (and (Variables|AttackCombo|GetattackThreeComboCanAttack) (Utilities|ClassIsChildOf (Utilities|GetClass (Default|GetTargetedActor (Variables|Refs|GetplayerRef))) "/Script/Engine.Character"))
    (bind _returnvalue_4 (Utilities|Time|SetTimerbyEvent (delegate Custom|ResetCombo) 0.5))
    (Variables|AttackCombo|SetattackThreeComboResetComboTimer _returnvalue_4)
    (if (not (> (Variables|AttackCombo|GetattackThreeComboCountAttack) 3))
      _
      (else
        (Variables|AttackCombo|SetattackThreeComboCountAttack 0)))
    (switch int (Variables|AttackCombo|GetattackThreeComboIteration)
      (:0
        (bind _returnvalue_5 (Game|SpawnActorfromClass "/Game/Blueprints/Navi/ThreeComboAttack/BP_ProjectileAttack.BP_ProjectileAttack_C" (Math|Transform|MakeTransform (.location _returnvalue) (.rotation _returnvalue) "1.000000,1.000000,1.000000") "Undefined" 0 (Variables|AttackCombo|GetattackThreeComboCountAttack) 0 :!label _label))
        (Utilities|FlowControl|Sequence
          (:then_0
            (Default|Attack _returnvalue_5 self (Default|GetTargetedActor (Variables|Refs|GetplayerRef)))
            (Math|Integer|IncrementInt (Variables|AttackCombo|GetattackThreeComboCountAttack)))
          (:then_1
            (Utilities|FlowControl|Delay (Utilities|Select :Index (Variables|AttackCombo|GetattackThreeComboCountAttack) :Option%200 0.1 :Option%201 0.15 :Option%202 0.75))
            (Variables|AttackCombo|SetattackThreeComboCanAttack true))))
      (:1
        (if (< (Variables|AttackCombo|GetattackThreeComboCountAttack) 2) :!label _label_2
          (goto _label)
          (else
            (for _index (range 0 (Variables|AttackCombo|GetattackThreeComboIteration))
              (bind _returnvalue_6 (Game|SpawnActorfromClass "/Game/Blueprints/Navi/ThreeComboAttack/BP_ProjectileAttack.BP_ProjectileAttack_C" (Math|Transform|MakeTransform (.location _returnvalue_3) (.rotation _returnvalue_3) "1.000000,1.000000,1.000000") "Undefined" 0 _index 0))
              (Default|Attack _returnvalue_6 self (Default|GetTargetedActor (Variables|Refs|GetplayerRef)))
              (Math|Integer|IncrementInt (Variables|AttackCombo|GetattackThreeComboCountAttack)))
            (Utilities|FlowControl|Delay 0.75)
            (Variables|AttackCombo|SetattackThreeComboCanAttack true)
            (Variables|AttackCombo|SetattackThreeComboCountAttack 0))))
      (:2
        (goto _label_2))
      (:3
        (Variables|AttackCombo|SetattackThreeComboCanAttack false)
        (for _index_2 (range 0 (Math|Integer|Clamp(Integer) (Variables|AttackCombo|GetattackThreeComboCountAttack) 0 8))
          (bind _returnvalue_7 (Game|SpawnActorfromClass "/Game/Blueprints/Navi/ThreeComboAttack/BP_ProjectileAttack.BP_ProjectileAttack_C" (Math|Transform|MakeTransform (.location _returnvalue_2) (.rotation _returnvalue_2) "1.000000,1.000000,1.000000") "Undefined" 0 _index_2 0))
          (Default|BigAttack _returnvalue_7 self (Default|GetTargetedActor (Variables|Refs|GetplayerRef))))
        (Utilities|FlowControl|Delay 0.75)
        (Variables|AttackCombo|SetattackThreeComboCanAttack true)
        (if (not (Utilities|Time|IsValidTimerHandle (Variables|AttackCombo|GetattackThreeComboResetComboTimer)))
          (Math|Integer|IncrementInt (Variables|AttackCombo|GetattackThreeComboCountAttack)
            (:%20%20
              (CallFunction|AttackThreeCombo)))
          (else
            (Variables|AttackCombo|SetattackThreeComboCountAttack 0)))))))

(event Custom|EndQTE
  ;[1 0 0.007763] QTEThings TOREFACTOR
  (CallFunction|SlowMoQte)
  (Default|SetMovementCapabilities (Variables|Refs|GetplayerRef) true true true)
  (Widget|RemovefromParent (Variables|burstUlt|GetburstUltQTEWidget))
  (Variables|burstUlt|SetburstUltQTEWidget 0)
  (Utilities|Platform|CollectGarbage)
  (Utilities|FlowControl|Delay 1.0)
  (if (Variables|/Game/Blueprints/Player/ThirdPersonCharacter.ThirdPersonCharacter_C|GetisLock (Variables|Refs|GetplayerRef))
    (CallFunction|UpdateMovementTypeinBlackboard "NewEnumerator4")
    (else
      (CallFunction|UpdateMovementTypeinBlackboard "NewEnumerator0"))))

(event Custom|ResetCombo
  ;[0 1 0.9378] AttackThreeCombo
  (Variables|AttackCombo|SetattackThreeComboCountAttack 0))

(event Custom|changeColor
  (params (Color :type Linear%20Color%20Structure :default "(R=0.000000,G=0.000000,B=1.000000,A=1.000000)") (Str :type Float%20%28double-precision%29) (Speed :type Float%20%28double-precision%29))
  ;[1 0.8288 0] ChangeColor
  (Components|Timeline|SetPlayRate (Variables|Default|GetcolorChangeTimeline) Speed)
  (bind _returnvalue (Rendering|Material|GetScalarParameterValue (Variables|colorUpdate|GetdynamicMat) "Strength" :!class /Script/Engine.MaterialInstanceDynamic))
  (Variables|colorUpdate|SetdynamicMatCurrentColorStrength _returnvalue)
  (bind _returnvalue_2 (Rendering|Material|GetVectorParameterValue (Variables|colorUpdate|GetdynamicMat) "Emissive" :!class /Script/Engine.MaterialInstanceDynamic))
  (Variables|ColorUpdate|SetdynamicMatCurrentColor _returnvalue_2)
  (bind _alpha (Timeline|colorChangeTimeline PlayFromStart)
    (:Update
      (Rendering|Material|SetVectorParameterValue (Variables|colorUpdate|GetdynamicMat) "Emissive" (Math|Color|Lerp(LinearColor) (Variables|ColorUpdate|GetdynamicMatCurrentColor) Color _alpha) :!class /Script/Engine.MaterialInstanceDynamic)
      (Rendering|Material|SetScalarParameterValue (Variables|colorUpdate|GetdynamicMat) "Strength" (Math|Float|Lerp (Variables|colorUpdate|GetdynamicMatCurrentColorStrength) Str _alpha) :!class /Script/Engine.MaterialInstanceDynamic))))

(event Custom|StrongAttack
  (CallFunction|SlashAttack)
  ;[0 0.3084 1] New Attack Navi
  (Components|Timeline|SetPlayRate (Variables|Default|GetTEST) 1.0)
  (Timeline|TEST PlayFromStart
    (:Update
      (Transformation|SetActorRelativeLocation (+ (Variables|/Script/Engine.SceneComponent|GetRelativeLocation (Variables|Default|GetCollision)) (* (Math|Random|RandomUnitVector) (Math|Random|RandomFloatinRange 1.0 5.0)))))))

(event EventBeginPlay
  ;[0 0.04589 1] BeginPlay
  (CallFunction|UpdateMovementTypeinBlackboard "NewEnumerator0")
  (bind _asthird_person_character (Utilities|Casting|CastToThirdPersonCharacter (Game|GetPlayerCharacter 0)))
  (Variables|Refs|SetplayerRef _asthird_person_character)
  (bind _returnvalue (Game|SpawnActorfromClass "/Game/Blueprints/Navi/BP_NaviAttachPoint.BP_NaviAttachPoint_C" (Math|Transform|MakeTransform "0, 0, 0" "0, 0, 0" "1.000000,1.000000,1.000000") "Undefined" 0 self 0))
  (Variables|NaviMovement|SetNaviAttachActor _returnvalue)
  (Transformation|SetAbsolute (Variables|/Script/Engine.Actor|GetRootComponent (Variables|NaviMovement|GetNaviAttachActor)) false true true)
  (Transformation|AttachActorToActor (Variables|NaviMovement|GetNaviAttachActor) "None" "SnapToTarget" "KeepWorld" "KeepWorld" false)
  (Transformation|SetAbsolute (Variables|Default|GetCollision) false true true)
  (bind _returnvalue_2 (Rendering|Material|CreateDynamicMaterialInstance "/Game/FX/Materials/M_Navi.M_Navi" "None" "None" :!class /Script/Engine.KismetMaterialLibrary))
  (Variables|colorUpdate|SetdynamicMat _returnvalue_2)
  (Class|NiagaraComponent|SetVariableMaterial (Variables|Default|GetTrail) "CustomMat" (Variables|colorUpdate|GetdynamicMat))
  (EventDispatchers|BindEventtoLockUpdateDispatcher (Variables|Refs|GetplayerRef) (delegate Custom|playerLockUpdate))
  (AI|Components|Blackboard|SetValueasObject (AI|GetBlackboard 0) (Utilities|Name|MakeLiteralName "playerRef") (Variables|Refs|GetplayerRef)))

(event EventTick
  (params (DeltaSeconds :type Float%20%28single-precision%29))
  ;[1 0 0] Tick
  (Variables|Default|SetActorVelocity (- (Transformation|GetActorLocation) (Variables|Default|GetActorVelocity))))

(fn ConstructionScript)

(fn FPlayerLockUpdate
  (CallFunction|UpdateMovementTypeinBlackboard "NewEnumerator12")
  (return))

(fn UpdateMovementTypeinBlackboard
  (params (movementType :type ENaviState%20Enum :default "NewEnumerator0"))
  (AI|Components|Blackboard|SetValueasEnum (AI|GetBlackboard 0) (Utilities|Name|MakeLiteralName "newNaviState") movementType)
  (Default|CallOnMovementTypeUpdateinBlackboard)
  (return))

(fn FUpdateNaviLocationinTimeline
  (params (time :type Float%20%28double-precision%29) (Drag :type Float%20%28double-precision%29) (CurveType :type EBezierCurveType%20Enum :default "NewEnumerator3"))
  (bind _playerref (Variables|Refs|GetplayerRef))
  (bind _actor (Default|GetTargetedActor _playerref))
  (bind _asbp_enemy (Utilities|Casting|CastToBP_Enemy _actor))
  (LocalVariables|SetLTime time)
  (LocalVariables|SetLDrag Drag)
  (LocalVariables|SetLCurveType CurveType)
  (switch Utilities|FlowControl|Switch|SwitchonEBezierCurveType (LocalVariables|GetLCurveType)
    (:NewEnumerator3
      (Transformation|SetActorRelativeLocation (.ReturnValue (CallFunction|GetLocationBezier (AI|Components|Blackboard|GetValueasVector (AI|GetBlackboard 0) (Utilities|Name|MakeLiteralName "naviMovementStartLocation")) (AI|Components|Blackboard|GetValueasVector (AI|GetBlackboard 0) (Utilities|Name|MakeLiteralName "naviMovementAnchorLocation")) (AI|Components|Blackboard|GetValueasVector (AI|GetBlackboard 0) (Utilities|Name|MakeLiteralName "naviMovementEndLocation")) (LocalVariables|GetLTime) 0 0 self (LocalVariables|GetLCurveType) 0.0 "0, 0, 0" 500))))
    (:NewEnumerator0
      (if (== (LocalVariables|GetLTime) 0.0) :!label _label ; FirstTick
        (CallFunction|UpdateMaxMinHeight)
        (Variables|NaviMovement|SetmainMovementPoints (.Points (CallFunction|GetLocationBezier (AI|Components|Blackboard|GetValueasVector (AI|GetBlackboard 0) (Utilities|Name|MakeLiteralName "naviMovementStartLocation")) (AI|Components|Blackboard|GetValueasVector (AI|GetBlackboard 0) (Utilities|Name|MakeLiteralName "naviMovementAnchorLocation")) (AI|Components|Blackboard|GetValueasVector (AI|GetBlackboard 0) (Utilities|Name|MakeLiteralName "naviMovementEndLocation")) (LocalVariables|GetLTime) 0 0 (Default|GetTargetedActor (Variables|Refs|GetplayerRef)) (LocalVariables|GetLCurveType) 0.0 "0, 0, 0" 500))))
      (Transformation|SetActorRelativeLocation (Math|Vector|MakeVector (.x (Utilities|Array|Get(acopy) (Variables|NaviMovement|GetmainMovementPoints) (Math|Float|Truncate (* (Math|Conversions|ToFloat(Integer) (Utilities|Array|LastIndex (Variables|NaviMovement|GetmainMovementPoints))) (LocalVariables|GetLTime))))) (.y (Utilities|Array|Get(acopy) (Variables|NaviMovement|GetmainMovementPoints) (Math|Float|Truncate (* (Math|Conversions|ToFloat(Integer) (Utilities|Array|LastIndex (Variables|NaviMovement|GetmainMovementPoints))) (LocalVariables|GetLTime))))) (Math|Float|Clamp(Float) (.z (Utilities|Array|Get(acopy) (Variables|NaviMovement|GetmainMovementPoints) (Math|Float|Truncate (* (Math|Conversions|ToFloat(Integer) (Utilities|Array|LastIndex (Variables|NaviMovement|GetmainMovementPoints))) (LocalVariables|GetLTime))))) (Variables|NaviMovement|GetmainMovementMinHeight) (Variables|NaviMovement|GetmainMovementMaxHeight))))
      (Rendering|SetActorHiddenInGame (and (>= (LocalVariables|GetLTime) 0.0) (< (LocalVariables|GetLTime) 0.02))))
    (:NewEnumerator1
      (goto _label))
    (:NewEnumerator2
      (goto _label))
    (:NewEnumerator4
      (goto _label))
    (:NewEnumerator5
      (goto _label))
    (:NewEnumerator6
      (if (Utilities|Operators|EqualEqual :A (Variables|/Script/Engine.SceneComponent|GetRelativeLocation (Variables|Default|GetCollision)) :ErrorTolerance 1e+01)
        (bind _targetedinteractiblecomponent (Variables|/Game/Blueprints/Player/ThirdPersonCharacter.ThirdPersonCharacter_C|GetTargetedInteractibleComponent (Variables|Refs|GetplayerRef))
          (:then
            (Variables|/Game/Blueprints/AI/Enemy/Trash/BP_Enemy.BP_Enemy_C|SetImpactFxRelativeLocation _asbp_enemy (.location (Math|Transform|MakeRelativeTransform (Math|Transform|MakeTransform (Transformation|GetActorLocation)) (Math|Transform|MakeTransform (Transformation|GetActorLocation _asbp_enemy)))))
            (Default|CallInteractwithOwner _targetedinteractiblecomponent)
            (goto _label))
          (:else
            (goto _label)))
        (else
          (goto _label)))))
  (if (> (LocalVariables|GetLTime) 0.53) ; 1/2Ticks
    (if (> (LocalVariables|GetLDrag) 0.0)
      (Components|Timeline|SetPlayRate (Variables|Default|GetMainMovementTimeline) (/ (Math|Float|MapRangeClamped (Components|Timeline|GetPlaybackPosition (Variables|Default|GetMainMovementTimeline)) 0.5 1.0 0.4 0.1) (LocalVariables|GetLDrag)))
      (bind _targetedinteractiblecomponent_2 (Variables|/Game/Blueprints/Player/ThirdPersonCharacter.ThirdPersonCharacter_C|GetTargetedInteractibleComponent (Variables|Refs|GetplayerRef))
        (:then
          (Variables|/Game/Blueprints/AI/Enemy/Trash/BP_Enemy.BP_Enemy_C|SetImpactFxRelativeLocation (.AsBP%20Enemy (Utilities|Casting|CastToBP_Enemy (Default|GetTargetedActor (Variables|Refs|GetplayerRef)))) (AI|Components|Blackboard|GetValueasVector (AI|GetBlackboard 0) (Utilities|Name|MakeLiteralName "naviMovementAnchorLocation")))
          (Default|CallInteractwithOwner _targetedinteractiblecomponent_2)
          (Variables|Default|SethasAppliedDamage true))
        (:else
          _))))
  (if (== (LocalVariables|GetLTime) 1.0) ; LastTick
    _
    (else
      _))
  (return))

(fn UpdateMaxMinHeight
  (bind _returnvalue (Transformation|GetActorLocation))
  (bind _returnvalue_2 (Transformation|GetActorLocation))
  (bind _returnvalue_3 (AI|GetBlackboard 0))
  (bind _returnvalue_4 (Utilities|Name|MakeLiteralName "naviMovementEndLocation"))
  (bind _returnvalue_5 (Transformation|GetActorLocation))
  (bind _returnvalue_6 (AI|GetBlackboard 0))
  (bind _returnvalue_7 (Utilities|Name|MakeLiteralName "naviMovementStartLocation"))
  (bind _returnvalue_8 (AI|GetBlackboard 0))
  (bind _returnvalue_9 (Utilities|Name|MakeLiteralName "naviMovementStartLocation"))
  (bind _returnvalue_10 (AI|GetBlackboard 0))
  (bind _returnvalue_11 (Utilities|Name|MakeLiteralName "naviMovementEndLocation"))
  (bind _returnvalue_12 (AI|Components|Blackboard|GetValueasVector _returnvalue_3 _returnvalue_4))
  (bind _returnvalue_13 (AI|Components|Blackboard|GetValueasVector _returnvalue_6 _returnvalue_7))
  (bind _returnvalue_14 (AI|Components|Blackboard|GetValueasVector _returnvalue_8 _returnvalue_9))
  (bind _returnvalue_15 (AI|Components|Blackboard|GetValueasVector _returnvalue_10 _returnvalue_11))
  (bind _returnvalue_16 (Math|Vector|Lerp(Vector) _returnvalue_13 _returnvalue_12 0.5))
  (bind _returnvalue_17 (+ _returnvalue_2 _returnvalue_15))
  (bind _returnvalue_18 (+ _returnvalue_5 _returnvalue_14))
  (bind _returnvalue_19 (+ _returnvalue _returnvalue_16))
  (bind _ascharacter (Utilities|Casting|CastToCharacter (Variables|/Game/Blueprints/Navi/BP_NaviAttachPoint.BP_NaviAttachPoint_C|GetattachActor (Variables|NaviMovement|GetNaviAttachActor)))
    (:then
      (Variables|NaviMovement|SetmainMovementMaxHeight 99999999.0)
      (Variables|NaviMovement|SetmainMovementMinHeight (- (Class|CharacterMovementComponent|GetWalkableFloorZ (Variables|/Script/Engine.Character|GetCharacterMovement _ascharacter)) 5e+01))
      (return))
    (:CastFailed
      (bind _outhit (Collision|LineTraceForObjects _returnvalue_18 (+ _returnvalue_18 "0,0,-100000.000000") (Utilities|Array|MakeArray "ObjectTypeQuery1") false 0 "Persistent"))
      (if (.bblockinghit _outhit)
        (Variables|NaviMovement|SetmainMovementMinHeight (.Z (Math|Vector|BreakVector (.location _outhit))))
        (else
          (Variables|NaviMovement|SetmainMovementMinHeight (.Z (Math|Vector|BreakVector (.traceend _outhit))))))
      (bind _outhit_2 (Collision|LineTraceForObjects _returnvalue_19 (+ _returnvalue_19 "0,0,-100000.000000") (Utilities|Array|MakeArray "ObjectTypeQuery1") false 0 "Persistent"))
      (if (< (Math|Float|SelectFloat (.Z (Math|Vector|BreakVector (.location _outhit_2))) (.Z (Math|Vector|BreakVector (.traceend _outhit_2))) false) (Variables|NaviMovement|GetmainMovementMinHeight))
        (Variables|NaviMovement|SetmainMovementMinHeight (.Z (Math|Vector|BreakVector (.location _outhit_2)))))
      (bind _outhit_3 (Collision|LineTraceForObjects _returnvalue_17 (+ _returnvalue_17 "0,0,-100000.000000") (Utilities|Array|MakeArray "ObjectTypeQuery1") false 0 "Persistent"))
      (if (< (Math|Float|SelectFloat (.Z (Math|Vector|BreakVector (.location _outhit_3))) (.Z (Math|Vector|BreakVector (.traceend _outhit_3))) false) (Variables|NaviMovement|GetmainMovementMinHeight))
        (Variables|NaviMovement|SetmainMovementMinHeight (.Z (Math|Vector|BreakVector (.location _outhit_3)))))
      (Variables|NaviMovement|SetmainMovementMaxHeight 99999999.0)
      (Variables|NaviMovement|SetmainMovementMinHeight (+ (- (Variables|NaviMovement|GetmainMovementMinHeight) (.z (Transformation|GetActorLocation))) 5e+01))
      (return))))

(fn DeactivateRibbon
  (Components|Activation|Deactivate (Variables|Default|GetAttackTrail)))

(fn GetBlackboardMovementState
  (return (Utilities|Enum|ByteToEnumENaviState (Class|BlackboardComponent|GetValueasEnum (AI|GetBlackboard 0) (Utilities|Name|MakeLiteralName "naviState")))))

(fn IsBlackboardStateEqualto
  (params (States :type Array%20of%20ENaviState%20Enums :default "NewEnumerator0"))
  (for _array_element States
    (if (Utilities|Enum|Equal(Enum) _array_element (CallFunction|GetBlackboardMovementState))
      (return true)))
  (return false))

(fn RepeatMovementTypeinBlackboard
  (params (movementType :type ENaviState%20Enum :default "NewEnumerator0"))
  (AI|Components|Blackboard|SetValueasEnum (AI|GetBlackboard 0) (Utilities|Name|MakeLiteralName "NaviState") (Utilities|Select :Index movementType :NewEnumerator0 1 :NewEnumerator12 0 :NewEnumerator4 0 :NewEnumerator2 0 :NewEnumerator5 0 :NewEnumerator6 0 :NewEnumerator7 0 :NewEnumerator9 0))
  (Default|CallOnMovementTypeUpdateinBlackboard)
  (return))