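; Anchor actor for the Navi companion that follows the player character and tracks which actor Navi relates to.
; It caches the player on BeginPlay, then teleports to the player's location every tick.
; On NaviStateUpdate, it re-expresses Navi's relative location against the current AttachActor, then picks a new one from the blackboard movement state.
; Roaming and hand states select the player, while launch and attack states select the player's targeted actor.
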(event Custom|NaviStateUpdate
  (bind _playerref (Variables|Default|GetplayerRef))
  (bind _actor (Default|GetTargetedActor _playerref))
  (Transformation|SetActorRelativeLocation (Variables|Default|GetnaviRef) (.location (Math|Transform|MakeRelativeTransform (Transformation|GetActorTransform (Variables|Default|GetnaviRef)) (Transformation|GetActorTransform (Variables|Default|GetattachActor)))))
  (Variables|Default|SetattachActor (Utilities|Select :Index (Default|GetBlackboardMovementState (Variables|Default|GetnaviRef)) :NewEnumerator0 _playerref :NewEnumerator12 _playerref :NewEnumerator4 _playerref :NewEnumerator2 _actor :NewEnumerator5 _actor :NewEnumerator6 _actor :NewEnumerator7 _actor :NewEnumerator9 _actor)))

(event EventBeginPlay
  (bind _asthird_person_character (Utilities|Casting|CastToThirdPersonCharacter (Game|GetPlayerCharacter 0)))
  (bind _output_get (Variables|Default|SetplayerRef _asthird_person_character))
  (Variables|Default|SetattachActor _output_get)
  (Actor|Tick|SetActorTickEnabled true))

(event Collision|EventActorBeginOverlap
  (params (OtherActor :type Actor%20Object%20Reference)))

(event EventTick
  (params (DeltaSeconds :type Float%20%28single-precision%29))
  (Transformation|SetActorLocation (Transformation|GetActorLocation (Variables|Default|GetplayerRef)) false true))

(fn ConstructionScript)