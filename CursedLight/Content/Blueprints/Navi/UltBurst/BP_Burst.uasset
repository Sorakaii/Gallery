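; BP_Burst is a randomly colored Niagara projectile, apparently part of Navi's burst ultimate, that flies to a target along a curved path.
; Attack builds a Bezier anchor from a random point on a vertical half-torus around the path midpoint, oriented by the player character.
; The Duration timeline moves the actor along that curve, following the target's current location.
; The actor destroys itself when the timeline finishes or if the target starts invalid.
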(event Custom|Attack
  (params (Navi :type BP%20Navi%20Pawn%20Object%20Reference) (Target :type Actor%20Object%20Reference))
  (Utilities|IsValid Target
    (:Is%20Valid
      (Variables|Default|SetNavi Navi)
      (Variables|Default|SetTarget Target)
      (bind (_navilocref _anchor) (CallFunction|BurstBezier))
      (Variables|Default|SetNavi%20Loc _navilocref)
      (Variables|Default|SetAnchor _anchor)
      (bind _time (Timeline|Duration PlayFromStart)
        (:Update
          (bind _target (Variables|Default|GetTarget)
            (:then
              (Transformation|SetActorLocation (.ReturnValue (CallFunction|GetLocationBezier (Variables|Default|GetNavi%20Loc) (Variables|Default|GetAnchor) (Transformation|GetActorLocation _target) _time 0 0 0 "NewEnumerator3" 0.0 "0, 0, 0")) false false))
            (:else)))
        (:Finished
          (Actor|DestroyActor))))
    (:Is%20Not%20Valid
      (Actor|DestroyActor))))

(event EventBeginPlay
  (bind _asthird_person_character (Utilities|Casting|CastToThirdPersonCharacter (Game|GetPlayerCharacter 0)))
  (Variables|Default|SetPlayerRef _asthird_person_character)
  (Effects|Components|ParticleSystem|SetColorParameter (Variables|Default|GetNiagara) "Color" (Utilities|Struct|MakeLinearColor (Math|Random|RandomFloat) (Math|Random|RandomFloat) (Math|Random|RandomFloat) 1.0)))

(fn ConstructionScript)

(fn BurstBezier
  (bind _radius (LocalVariables|GetRadius))
  (LocalVariables|SetNavi%20Loc%20Ref (Transformation|GetActorLocation))
  (LocalVariables|SetTargetLoc (Transformation|GetActorLocation (Variables|Default|GetTarget)))
  (LocalVariables|SetMiddlePoint (CallFunction|GetRandomPointinTorusVerticalHalfWIP -25.0 25.0 _radius _radius (Math|Vector|Lerp(Vector) (LocalVariables|GetNavi%20Loc%20Ref) (LocalVariables|GetTargetLoc) 0.5) (Variables|Default|GetPlayerRef) -1.8e+02 1.8e+02 "0, 0, 0"))
  (return (LocalVariables|GetNavi%20Loc%20Ref) (CallFunction|GenerateAnchor (LocalVariables|GetNavi%20Loc%20Ref) (LocalVariables|GetMiddlePoint) (LocalVariables|GetTargetLoc))))