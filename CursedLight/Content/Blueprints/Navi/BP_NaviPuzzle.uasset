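; Navi puzzle pawn, a Niagara effect that serves two puzzle modes chosen by IsWallPuzzle.
; Wall mode locks player movement, attaches Navi to the road's wall and steers it along the road's plane by mouse or gamepad; hitting "Error" components resets the road.
; Otherwise it shows a light and root spam-bar widget, whose progress drives ChangeScale.
; Tick eases Niagara scale toward a target; some older scale-pulse logic is disconnected.
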(event OnComponentHit(CollisionComponent)
  (params (HitComponent :type Primitive%20Component%20Object%20Reference) (OtherActor :type Actor%20Object%20Reference) (OtherComp :type Primitive%20Component%20Object%20Reference) (NormalImpulse :type Vector :default "0, 0, 0") (Hit :type Hit%20Result%20Structure%20%28by%20ref%29))
  (Utilities|FlowControl|DoOnce false
    (:Completed
      (if (Components|ComponentHasTag OtherComp "Error")
        (Default|Reset (Variables|Default|GetRoadRef))
        (else
          (CallFunction|ResetDoOnce))))))

(event Custom|StartPuzzle
  (bind _returnvalue (Game|GetPlayerController 0))
  (bind _roadref (Variables|Default|GetRoadRef))
  (bind _spawn (Variables|/Game/Blueprints/Enigmes/BP_NaviRoad.BP_NaviRoad_C|GetSpawn _roadref))
  (bind _returnvalue_2 (Transformation|GetWorldLocation _spawn))
  (bind _screenposition (Class|GameplayStatics|ProjectWorldtoScreen _returnvalue _returnvalue_2 false))
  (bind _asthird_person_character (Utilities|Casting|CastToThirdPersonCharacter (Game|GetPlayerCharacter 0)))
  (Variables|Default|SetPlayerRef _asthird_person_character)
  (if (not (Variables|Default|GetIsWallPuzzle))
    (Rendering|SetVisibility (Variables|Default|GetWidget) true false)
    (Rendering|SetVisibility (Variables|Default|GetLight) true false)
    (Actor|Tick|SetActorTickEnabled true)
    (bind _output_get (Variables|Default|SetNewScaleNavi (/ (Variables|Default|GetNewScaleNavi) 2.0)))
    (Variables|Default|SetScaleIniNaviPuzzle _output_get)
    (Components|Timeline|PlayfromStart (Variables|Default|GetBlinkNavi))
    (else
      (Rendering|SetVisibility (Variables|Default|GetWidget) false false)
      (Default|SetMovementCapabilities (Variables|Default|GetPlayerRef) false false false)
      (Class|PlayerController|SetMouseLocation _returnvalue (Math|Float|Truncate (.x _screenposition)) (Math|Float|Truncate (.y _screenposition)))
      (Transformation|AttachComponentToComponent (Variables|/Game/Blueprints/Enigmes/BP_NaviRoad.BP_NaviRoad_C|GetWall (Variables|Default|GetRoadRef)) "None" "SnapToTarget" "KeepWorld" "KeepWorld" true)
      (Transformation|SetActorRelativeLocation "0.000000,50.000000,-17.000000")
      (Actor|Tick|SetActorTickEnabled true))))

(event Custom|ResetDoOnce
  (Utilities|FlowControl|DoOnce false) ; enters at Reset
)

(event Custom|ChangeScale
  (Variables|Default|SetNewScaleNavi (Math|Vector|Lerp(Vector) (Variables|Default|GetNewScaleNavi) (* (Variables|Default|GetNewScaleNavi) 1.1) (Variables|/Script/UMG.ProgressBar|GetPercent (Variables|/Game/Blueprints/UI/WBP_RootSpamBar.WBP_RootSpamBar_C|GetProgressBar_0 (.AsWBP%20Root%20Spam%20Bar (Utilities|Casting|CastToWBP_RootSpamBar (UserInterface|GetWidget (Variables|Default|GetWidget)))))))))

(event EventBeginPlay
  (bind _asals_player_camera_manager (Utilities|Casting|CastToALS_PlayerCameraManager (Game|GetPlayerCameraManager 0)))
  (Variables|Default|SetCameraManagerRef _asals_player_camera_manager)
  (Variables|Default|SetScale%20Target%20Navi%20Puzzle (Transformation|GetWorldScale (Variables|Default|GetNiagara)))
  (Variables|Default|SetNewScaleNavi (Transformation|GetWorldScale (Variables|Default|GetNiagara))))

(event EventTick
  (params (DeltaSeconds :type Float%20%28single-precision%29))
  (bind _returnvalue (Game|GetPlayerController 0))
  (bind _playerref (Variables|Default|GetPlayerRef))
  (bind _roadref (Variables|Default|GetRoadRef))
  (bind _niagara (Variables|Default|GetNiagara))
  (bind _roadref_2 (Variables|Default|GetRoadRef))
  (bind (_deltax _deltay) (Class|PlayerController|GetInputMouseDelta _returnvalue))
  (bind _movex (Variables|/Game/Blueprints/Player/ThirdPersonCharacter.ThirdPersonCharacter_C|GetmoveX _playerref))
  (bind _movey (Variables|/Game/Blueprints/Player/ThirdPersonCharacter.ThirdPersonCharacter_C|GetmoveY _playerref))
  (Transformation|SetWorldScale3D _niagara (Math|Interpolation|VInterptoConstant (Transformation|GetWorldScale _niagara) (Variables|Default|GetScale%20Target%20Navi%20Puzzle) DeltaSeconds 0.3))
  ;[0.8581 1 0] Movement
  (if (and (Variables|Default|GetIsWallPuzzle) (Variables|Default|GetcanMove))
    (if (Variables|/Game/Blueprints/Player/ThirdPersonCharacter.ThirdPersonCharacter_C|GetGamepad (Variables|Default|GetPlayerRef))
      (Pawn|Input|AddMovementInput (+ (* (Transformation|GetActorForwardVector _roadref_2) (Math|Float|SelectFloat 0.0 _movex (< (Math|Float|Absolute(Float) _movex) 0.25))) (* (Transformation|GetActorUpVector _roadref_2) (Math|Float|SelectFloat 0.0 _movey (< (Math|Float|Absolute(Float) _movey) 0.25)))) 0.2 false)
      (else
        (Pawn|Input|AddMovementInput (+ (* (Transformation|GetActorForwardVector _roadref) _deltax) (* (Transformation|GetActorUpVector _roadref) _deltay)) 0.2 false)))))

(fn ConstructionScript)