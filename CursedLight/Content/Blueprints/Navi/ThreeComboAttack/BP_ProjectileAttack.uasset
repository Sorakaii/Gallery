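; Projectile for Navi's three-combo attack that flies to a target actor along a Bezier arc, damaging it on arrival.
; Attack uses StockVar to vary arc side, curve, duration and scale per combo step.
; BigAttack uses Beziers to space anchors radially by combo index and attack count.
; The ProjMove timeline drives position toward the target's live location and updates Niagara scale and direction, then applies damage and destroys the actor.
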(event Custom|Attack
  (params (Navi :type BP%20Navi%20Pawn%20Object%20Reference) (TargetActor :type Actor%20Object%20Reference))
  (Utilities|IsValid TargetActor
    (:Is%20Valid
      (Variables|Default|SetTargetActorRef TargetActor)
      (Variables|Default|SetNaviRef Navi)
      (Variables|/Game/Blueprints/Navi/BP_NaviPawn.BP_NaviPawn_C|SetattackThreeComboCanAttack (Variables|Default|GetNaviRef) false)
      (CallFunction|StockVar (Variables|Default|GetNaviRef) (Variables|Default|GetTargetActorRef))
      (bind _time (Timeline|ProjMove PlayFromStart)
        (:Update
          (Variables|Default|GetTargetActorRef
            (:then
              (Transformation|SetActorLocation (.ReturnValue (CallFunction|GetLocationBezier (Variables|Default|GetNavi%20Loc%20Ref) (Variables|Default|GetAnchor%20Ref) (Transformation|GetActorLocation (Variables|Default|GetTargetActorRef)) _time 0 0 0 "NewEnumerator0" 0.0 "0, 0, 0")) false false)
              (Niagara|SetNiagaraVariable(Float) (Variables|Default|GetNiagara) "Scale" (* _time (Variables|Default|GetScale)))
              (if (!= (Transformation|GetDistanceTo (Variables|Default|GetTargetActorRef)) 0.0)
                (Niagara|SetNiagaraVariable(Vector3) (Variables|Default|GetNiagara) "ForwardAngle" (Math|Vector|GetForwardVector (Math|Rotator|FindLookatRotation (Transformation|GetActorLocation) (Transformation|GetActorLocation (Variables|Default|GetTargetActorRef)))))))
            (:else)))
        (:Finished
          (Components|Activation|Deactivate (Variables|Default|GetNiagara))
          ;[1 1 1] Damage AI
          (Game|Damage|ApplyDamage (Variables|Default|GetTargetActorRef) (Variables|Default|Getdamage) 0 0)
          (Utilities|FlowControl|Delay 0.5)
          (Actor|DestroyActor))))
    (:Is%20Not%20Valid
      (Actor|DestroyActor))))

(event Custom|BigAttack
  (params (Navi :type BP%20Navi%20Pawn%20Object%20Reference) (TargetActor :type Actor%20Object%20Reference))
  (Utilities|IsValid TargetActor
    (:Is%20Valid
      (Variables|Default|SetTargetActorRef TargetActor)
      (Variables|Default|SetNaviRef Navi)
      (CallFunction|Beziers (Variables|Default|GetNaviRef) (Variables|Default|GetTargetActorRef))
      (bind _time (Timeline|ProjMove PlayFromStart)
        (:Update
          (Variables|Default|GetTargetActorRef
            (:then
              (Transformation|SetActorLocation (.ReturnValue (CallFunction|GetLocationBezier (Variables|Default|GetNavi%20Loc%20Ref) (Variables|Default|GetAnchor%20Ref) (Transformation|GetActorLocation (Variables|Default|GetTargetActorRef)) _time 0 0 0 "NewEnumerator0" 0.0 "0, 0, 0")) false false)
              (Niagara|SetNiagaraVariable(Float) (Variables|Default|GetNiagara) "Scale" (* _time (Variables|Default|GetScale)))
              (if (!= (Transformation|GetDistanceTo (Variables|Default|GetTargetActorRef)) 0.0)
                (Niagara|SetNiagaraVariable(Vector3) (Variables|Default|GetNiagara) "ForwardAngle" (Math|Vector|GetForwardVector (Math|Rotator|FindLookatRotation (Transformation|GetActorLocation) (Transformation|GetActorLocation (Variables|Default|GetTargetActorRef)))))))
            (:else)))
        (:Finished
          (Components|Activation|Deactivate (Variables|Default|GetNiagara))
          ;[1 1 1] Damage AI
          (Game|Damage|ApplyDamage (Variables|Default|GetTargetActorRef) (Variables|Default|Getdamage) 0 0)
          (Utilities|FlowControl|Delay 0.5)
          (Actor|DestroyActor))))
    (:Is%20Not%20Valid
      (Actor|DestroyActor))))

(event EventBeginPlay
  (bind _asthird_person_character (Utilities|Casting|CastToThirdPersonCharacter (Game|GetPlayerCharacter 0)))
  (Variables|Default|SetPlayerRef _asthird_person_character))

(fn ConstructionScript)

(fn StockVar
  (params (Navi :type Actor%20Object%20Reference) (Target :type Actor%20Object%20Reference))
  (bind _playerref (Variables|Default|GetPlayerRef))
  (bind _playerref_2 (Variables|Default|GetPlayerRef))
  (bind _playerref_3 (Variables|Default|GetPlayerRef))
  (bind _projmove (Variables|Default|GetProjMove))
  (bind _projmove_2 (Variables|Default|GetProjMove))
  (bind _projmove_3 (Variables|Default|GetProjMove))
  (bind _returnvalue (Transformation|GetDistanceTo _playerref_2 Target))
  (bind _returnvalue_2 (Transformation|GetDistanceTo _playerref_3 Target))
  (bind _returnvalue_3 (Transformation|GetDistanceTo _playerref Target))
  (bind _returnvalue_4 (* _returnvalue 0.01))
  (bind _returnvalue_5 (* _returnvalue_3 0.01))
  (bind _returnvalue_6 (* _returnvalue_2 0.01))
  (switch int (Variables|Default|GetCombo)
    (:0
      (Variables|Default|SetRadMini (* _returnvalue_4 -35.0))
      (Variables|Default|SetRadMaxi (* _returnvalue_4 -45.0)))
    (:1
      (Variables|Default|SetRadMini (* _returnvalue_5 35.0))
      (Variables|Default|SetRadMaxi (* _returnvalue_5 45.0)))
    (:2
      (LocalVariables|SetRadianMin -3e+01)
      (LocalVariables|SetRadianMax 3e+01)
      (Variables|Default|SetRadMini (* _returnvalue_6 2e+01))
      (Variables|Default|SetRadMaxi (* _returnvalue_6 3e+01))))
  (Variables|Default|SetNavi%20Loc%20Ref (Transformation|GetActorLocation Navi))
  (LocalVariables|SetTargetLoc (Transformation|GetActorLocation Target))
  (LocalVariables|SetLocSegZ (.Z (Math|Vector|BreakVector (CallFunction|GetLocationAlongSegment (Variables|Default|GetNavi%20Loc%20Ref) (LocalVariables|GetTargetLoc) 0.5))))
  (LocalVariables|SetRandPoint (CallFunction|GetRandomPointinTorusVerticalHalfWIP -5e+01 5e+01 (Variables|Default|GetRadMini) (Variables|Default|GetRadMaxi) (CallFunction|GetLocationAlongSegment (Variables|Default|GetNavi%20Loc%20Ref) (LocalVariables|GetTargetLoc) 0.5) (Variables|Default|GetPlayerRef) (LocalVariables|GetRadianMin) (LocalVariables|GetRadianMax) "0, 0, 0"))
  (LocalVariables|SetRightVec (* (Math|Vector|GetRightVector (Math|Rotator|FindLookatRotation (Variables|Default|GetNavi%20Loc%20Ref) (LocalVariables|GetTargetLoc))) 1e+02))
  (switch int (Variables|Default|GetCombo)
    (:0
      (Variables|Default|SetScale 0.1)
      (Class|TimelineComponent|SetTimelineLengthMode _projmove_2 "TL_TimelineLength")
      (Class|TimelineComponent|SetFloatCurve _projmove_2 "/Game/Blueprints/Navi/ThreeComboAttack/C_ComboOne.C_ComboOne" "Time")
      (Components|Timeline|SetTimelineLength _projmove_2 0.5)
      (Variables|Default|SetAnchor%20Ref (CallFunction|GenerateAnchor (Variables|Default|GetNavi%20Loc%20Ref) (Math|Vector|MakeVector (.x (+ (LocalVariables|GetRandPoint) (LocalVariables|GetRightVec))) (.y (+ (LocalVariables|GetRandPoint) (LocalVariables|GetRightVec))) (LocalVariables|GetLocSegZ)) (LocalVariables|GetTargetLoc)))
      (Niagara|SetNiagaraVariable(Float) (Variables|Default|GetNiagara) "SpawnTime" 0.4))
    (:1
      (Variables|Default|SetScale 0.15)
      (Class|TimelineComponent|SetTimelineLengthMode _projmove_3 "TL_TimelineLength")
      (Class|TimelineComponent|SetFloatCurve _projmove_3 "/Game/Blueprints/Navi/ThreeComboAttack/C_ComboTwo.C_ComboTwo" "Time")
      (Components|Timeline|SetTimelineLength _projmove_3 0.6)
      (Variables|Default|SetAnchor%20Ref (CallFunction|GenerateAnchor (Variables|Default|GetNavi%20Loc%20Ref) (Math|Vector|MakeVector (.x (- (LocalVariables|GetRandPoint) (LocalVariables|GetRightVec))) (.y (- (LocalVariables|GetRandPoint) (LocalVariables|GetRightVec))) (LocalVariables|GetLocSegZ)) (LocalVariables|GetTargetLoc)))
      (Niagara|SetNiagaraVariable(Float) (Variables|Default|GetNiagara) "SpawnTime" 0.5))
    (:2
      (Variables|Default|SetScale 0.3)
      (Class|TimelineComponent|SetTimelineLengthMode _projmove "TL_TimelineLength")
      (Class|TimelineComponent|SetFloatCurve _projmove "/Game/Blueprints/Navi/ThreeComboAttack/C_ComboThree.C_ComboThree" "Time")
      (Components|Timeline|SetTimelineLength _projmove 1.0)
      (Variables|Default|SetAnchor%20Ref (CallFunction|GenerateAnchor (Variables|Default|GetNavi%20Loc%20Ref) (LocalVariables|GetRandPoint) (LocalVariables|GetTargetLoc)))
      (Niagara|SetNiagaraVariable(Float) (Variables|Default|GetNiagara) "SpawnTime" 0.75)))
  (return))

(fn Beziers
  (params (Navi :type Actor%20Object%20Reference) (Target :type Actor%20Object%20Reference))
  (bind _radius (LocalVariables|GetRadius))
  (bind _output_get (LocalVariables|SetPoint (Math|Conversions|ToFloat(Integer) (/ 360 (+ (Variables|/Game/Blueprints/Navi/BP_NaviPawn.BP_NaviPawn_C|GetattackThreeComboCountAttack (Variables|Default|GetNaviRef)) 1)))))
  (LocalVariables|SetRadian (+ (LocalVariables|GetRadian) (* _output_get (Variables|Default|GetCombo))))
  (Variables|Default|SetNavi%20Loc%20Ref (Transformation|GetActorLocation Navi))
  (LocalVariables|SetTargetLoc (Transformation|GetActorLocation Target))
  (LocalVariables|SetLocSegZ (.Z (Math|Vector|BreakVector (CallFunction|GetLocationAlongSegment (Variables|Default|GetNavi%20Loc%20Ref) (LocalVariables|GetTargetLoc) 0.5))))
  (LocalVariables|SetMiddlePoint (CallFunction|GetRandomPointinTorusVerticalHalfWIP -5e+01 5e+01 _radius _radius (CallFunction|GetLocationAlongSegment (Variables|Default|GetNavi%20Loc%20Ref) (LocalVariables|GetTargetLoc) 0.5) (Variables|Default|GetPlayerRef) (LocalVariables|GetRadian) (LocalVariables|GetRadian) "0, 0, 0"))
  (Variables|Default|SetAnchor%20Ref (CallFunction|GenerateAnchor (Variables|Default|GetNavi%20Loc%20Ref) (LocalVariables|GetMiddlePoint) (LocalVariables|GetTargetLoc)))
  (Variables|Default|SetScale 0.1)
  (Niagara|SetNiagaraVariable(Float) (Variables|Default|GetNiagara) "SpawnTime" 0.5)
  (return))