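; Checkpoint actor that, when the player first overlaps its box or at BeginPlay if flagged as Spawn, becomes the active respawn point.
; Activation changes the pedestal material, shows an update widget for non-spawn checkpoints and takes over the player's death dispatcher.
; On death, it teleports the player to its Respawn point, restores health and resets linked enemies.
; Surviving enemies regain health; missing ones are respawned at transforms cached during the overlap.
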(event OnComponentBeginOverlap(Box)
  (params (OverlappedComponent :type Primitive%20Component%20Object%20Reference) (OtherActor :type Actor%20Object%20Reference) (OtherComp :type Primitive%20Component%20Object%20Reference) (OtherBodyIndex :type Integer) (bFromSweep :type Boolean) (SweepResult :type Hit%20Result%20Structure%20%28by%20ref%29))
  (if (== OtherActor (Variables|Default|GetPlayerref))
    (Utilities|FlowControl|DoOnce false
      (:Completed
        (CallFunction|CheckpointActivation)
        (if (Utilities|Array|IsNotEmpty (Variables|Default|GetEnemyRef))
          (for _array_element (Variables|Default|GetEnemyRef)
            (Utilities|Array|Add (Variables|Default|GetEnemyTransform) (Variables|/Game/Blueprints/AI/Enemy/Trash/BP_Enemy.BP_Enemy_C|GetTransformRef (.enemy _array_element)))))))))

(event Custom|PlayerRespawnEvent
  (bind _playerref (Variables|Default|GetPlayerref))
  (bind _playerref_2 (Variables|Default|GetPlayerref))
  (Transformation|SetActorLocation _playerref_2 (Transformation|GetWorldLocation (Variables|Default|GetRespawn)) false false)
  (Variables|/Game/Blueprints/Player/ThirdPersonCharacter.ThirdPersonCharacter_C|SetHealth _playerref (Variables|/Game/Blueprints/Player/ThirdPersonCharacter.ThirdPersonCharacter_C|GetmaxHealth _playerref))
  (Variables|/Script/Engine.Actor|SetbCanBeDamaged _playerref_2 true)
  (Pawn|SetControlRotation (Game|GetPlayerController 0) (Transformation|GetActorRotation (Variables|Default|GetPlayerref)))
  (CallFunction|ResetEnemy))

(event Custom|checkpointActivation
  (EventDispatchers|UnbindallEventsfromPlayerDeathDispatcher (Variables|Default|GetPlayerref))
  (Rendering|Material|SetMaterial (Variables|Default|GetCube) 0 "/Game/Maps/Landscape/MAT_checkpoint_piedestal.MAT_checkpoint_piedestal")
  (if (not (Variables|Default|GetSpawn))
    (bind _returnvalue (UserInterface|CreateWidget "/Game/Blueprints/UI/WBP_CheckpointUpdate.WBP_CheckpointUpdate_C"))
    (UserInterface|Viewport|AddtoViewport _returnvalue 0))
  (EventDispatchers|BindEventtoPlayerDeathDispatcher (Variables|Default|GetPlayerref) (delegate Custom|PlayerRespawnEvent)))

(event EventTick
  (params (DeltaSeconds :type Float%20%28single-precision%29)))

(event Collision|EventActorBeginOverlap
  (params (OtherActor :type Actor%20Object%20Reference)))

(event EventBeginPlay
  (bind _asthird_person_character (Utilities|Casting|CastToThirdPersonCharacter (Game|GetPlayerCharacter 0)))
  (Variables|Default|SetPlayerref _asthird_person_character)
  (if (Variables|Default|GetSpawn)
    (CallFunction|CheckpointActivation)))

(fn ConstructionScript)

(fn ResetEnemy
  (for (_array_element _array_index) (Variables|Default|GetEnemyRef)
    (LocalVariables|SetKey (.enemy _array_element))
    (Utilities|IsValid (LocalVariables|GetKey)
      (:Is%20Valid
        (Variables|/Game/Blueprints/AI/Enemy/Trash/BP_Enemy.BP_Enemy_C|SetHealth (LocalVariables|GetKey) (Variables|/Game/Blueprints/AI/Enemy/Trash/DataAssets/PDA_Enemy.PDA_Enemy_C|GetHealth (Variables|/Game/Blueprints/AI/Enemy/Trash/BP_Enemy.BP_Enemy_C|GetEnemy%20Type (LocalVariables|GetKey)))))
      (:Is%20Not%20Valid
        (bind _returnvalue (Game|SpawnActorfromClass "/Game/Blueprints/AI/Enemy/Trash/BP_Enemy.BP_Enemy_C" (Utilities|Array|Get(acopy) (Variables|Default|GetEnemyTransform) _array_index) "Undefined" 0 (.data _array_element) 0))
        (Utilities|Array|SetArrayElem (Variables|Default|GetEnemyRef) _array_index (Utilities|Struct|MakeStruct_CheckpointEnemy _returnvalue (.data _array_element)))))))