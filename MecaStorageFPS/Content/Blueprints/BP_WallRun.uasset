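; Wall-run logic for a character passed into Initialize, with jump-off, landing reset and camera roll.
; A looping timer traces right, then left, accepts near-vertical surfaces while falling, then uses LaunchCharacter to stick and push along the wall while easing gravity.
; Ending a run restores gravity and suppresses re-entry on a timer.
; Tick tilts the control rotation and prints debug values; Climb is an empty stub on its own timer.
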(event Custom|Initialize
  (params (Character :type First%20Person%20Character%20Object%20Reference))
  (bind _output_get (Variables|Default|SetCharacter Character))
  (bind _output_get_2 (Variables|Default|SetCharacter%20Movement (Variables|/Script/Engine.Character|GetCharacterMovement _output_get)))
  (Variables|WallRun|SetGravity (Variables|/Script/Engine.CharacterMovementComponent|GetGravityScale _output_get_2))
  (Utilities|Time|SetTimerbyEvent (delegate Custom|WallRunUpdateEvent) 0.02 true)
  (Utilities|Time|SetTimerbyEvent (delegate Custom|ClimbUpdate) 0.02 true))

(event Custom|Jump
  (CallFunction|WallRunJump))

(event Custom|Land
  (CallFunction|WallRunEnd 0.0)
  (Variables|WallRun|SetWallRunSupressed false))

(event Custom|ClimbUpdate
  (if (Variables|Climb|GetIsClimbing)
    (CallFunction|Climb)))

(event Custom|WallRunUpdateEvent
  (if (not (Variables|WallRun|GetWallRunSupressed))
    (CallFunction|WallRunUpdateFunction)))

(event Custom|ResetWallRunSupression
  (Utilities|Time|ClearTimerbyFunctionName 0 "ResetWallRunSupression")
  (Variables|WallRun|SetWallRunSupressed false))

(event EventBeginPlay)

(event EventTick
  (params (DeltaSeconds :type Float%20%28single-precision%29))
  (Utilities|FlowControl|Sequence
    (:then_0
      (CallFunction|CameraTick))
    (:then_1
      (Development|PrintString (Utilities|String|Append "Gravity : " (Utilities|String|ToString(Float) (Variables|WallRun|GetGravity))) true true "(R=0.000000,G=0.660000,B=1.000000,A=1.000000)" 0.0)
      (Development|PrintString (Utilities|String|Append "WR Normal : " (Utilities|String|ToString(Vector) (Variables|WallRun|GetWallRunNormal))) true true "(R=0.000000,G=0.660000,B=1.000000,A=1.000000)" 0.0)
      (Development|PrintString (Utilities|String|Append "WR Speed : " (Utilities|String|ToString(Float) (Variables|WallRun|GetWallRunSpeed))) true true "(R=0.000000,G=0.660000,B=1.000000,A=1.000000)" 0.0)
      (Development|PrintString (Utilities|String|Append "WR Gravity : " (Utilities|String|ToString(Boolean) (Variables|WallRun|GetWallRunGravity))) true true "(R=0.000000,G=0.660000,B=1.000000,A=1.000000)" 0.0)
      (Development|PrintString (Utilities|String|Append "WR : " (Utilities|String|ToString(Boolean) (Variables|WallRun|GetWallRunning))) true true "(R=0.000000,G=0.660000,B=1.000000,A=1.000000)" 0.0)
      (Development|PrintString (Utilities|String|Append "WR R : " (Utilities|String|ToString(Boolean) (Variables|WallRun|GetWallRunningR))) true true "(R=0.000000,G=0.660000,B=1.000000,A=1.000000)" 0.0)
      (Development|PrintString (Utilities|String|Append "WR L : " (Utilities|String|ToString(Boolean) (Variables|WallRun|GetWallRunningL))) true true "(R=0.000000,G=0.660000,B=1.000000,A=1.000000)" 0.0)
      (Development|PrintString (Utilities|String|Append "WR RTargey: " (Utilities|String|ToString(Float) (Variables|WallRun|GetWallRunTargetGravity))) true true "(R=0.000000,G=0.660000,B=1.000000,A=1.000000)" 0.0)
      (Development|PrintString (Utilities|String|Append "WR Supr : " (Utilities|String|ToString(Boolean) (Variables|WallRun|GetWallRunSupressed))) true true "(R=0.000000,G=0.660000,B=1.000000,A=1.000000)" 0.0)
      (Development|PrintString (Utilities|String|Append "WR JumpH : " (Utilities|String|ToString(Float) (Variables|WallRun|GetWallRunJumpHeight))) true true "(R=0.000000,G=0.660000,B=1.000000,A=1.000000)" 0.0)
      (Development|PrintString (Utilities|String|Append "WR JumpOff : " (Utilities|String|ToString(Float) (Variables|WallRun|GetWallRunJumpOffForce))) true true "(R=0.000000,G=0.660000,B=1.000000,A=1.000000)" 0.0)
      (Development|PrintString (Utilities|String|Append "Control R : " (Utilities|String|ToString(Rotator) (Pawn|GetControlRotation (Pawn|GetController (Variables|Default|GetCharacter)) :!class /Script/Engine.Controller))) true true "(R=0.000000,G=0.660000,B=1.000000,A=1.000000)" 0.0))))

(fn WallRunUpdateFunction
  (bind _character_movement (Variables|Default|GetCharacter%20Movement))
  (bind _onwall (CallFunction|WallRunMovement (Transformation|GetActorLocation (Variables|Default|GetCharacter)) (.Right (Utilities|WallRunEndVectors)) -1.0)) ; Right
  (if _onwall
    (bind _output_get (Variables|WallRun|SetWallRunning true))
    (Variables|WallRun|SetWallRunningR _output_get)
    (Variables|WallRun|SetWallRunningL false)
    (Variables|/Script/Engine.CharacterMovementComponent|SetGravityScale _character_movement (Math|Interpolation|FInterpTo (Variables|/Script/Engine.CharacterMovementComponent|GetGravityScale _character_movement) (Variables|WallRun|GetWallRunTargetGravity) (Utilities|Time|GetWorldDeltaSeconds) 1e+01) :!label _label)
    (elif (Variables|WallRun|GetWallRunningR)
      (CallFunction|WallRunEnd 1.0)
      (else
        (bind _onwall_2 (CallFunction|WallRunMovement (Transformation|GetActorLocation (Variables|Default|GetCharacter)) (.Left (Utilities|WallRunEndVectors)) 1.0)) ; Left
        (if _onwall_2
          (Variables|WallRun|SetWallRunning true)
          (Variables|WallRun|SetWallRunningR false)
          (Variables|WallRun|SetWallRunningL true)
          (goto _label)
          (else
            (CallFunction|WallRunEnd 1.0)))))))

(fn WallRunMovement
  (params (Start :type Vector) (End :type Vector) (WallRunDirection :type Float%20%28single-precision%29))
  (bind _outhit (Collision|LineTraceByChannel Start End "TraceTypeQuery1" false 0 "None"))
  (if (.bBlockingHit (Collision|BreakHitResult _outhit))
    (if (and (AI|Components|NavMovement|IsFalling (Variables|Default|GetCharacter%20Movement)) (.ReturnValue (Utilities|ValidWallRunVectors (.Normal (Collision|BreakHitResult _outhit)))))
      (Variables|WallRun|SetWallRunNormal (.OutVecs (Utilities|ValidWallRunVectors (.Normal (Collision|BreakHitResult _outhit)))))
      (Character|LaunchCharacter (Variables|Default|GetCharacter) (Utilities|PlayertoWallVectors) false false) ; Stick On Wall
      (Character|LaunchCharacter (Variables|Default|GetCharacter) (* (Math|Vector|CrossProduct (Variables|WallRun|GetWallRunNormal) "0, 0,1.000000") (* (Variables|/Script/Engine.CharacterMovementComponent|GetMaxWalkSpeed (Variables|/Script/Engine.Character|GetCharacterMovement (Variables|Default|GetCharacter))) WallRunDirection)) true (not (Variables|WallRun|GetWallRunGravity))) ; Move Forward
      (return true)
      (else
        (return false)))
    (else
      (return false))))

(fn WallRunEnd
  (params (ResetTime :type Float%20%28single-precision%29))
  (if (Variables|WallRun|GetWallRunning)
    (Variables|WallRun|SetWallRunning false)
    (Variables|WallRun|SetWallRunningR false)
    (Variables|WallRun|SetWallRunningL false)
    (Variables|/Script/Engine.CharacterMovementComponent|SetGravityScale (Variables|Default|GetCharacter%20Movement) (Variables|WallRun|GetGravity))
    (CallFunction|SupressWallRun ResetTime)))

(fn SupressWallRun
  (params (Delay :type Float%20%28single-precision%29))
  (Variables|WallRun|SetWallRunSupressed true)
  (Utilities|Time|SetTimerbyFunctionName 0 "ResetWallRunSupression" Delay))

(fn CameraTick
  (if (Variables|WallRun|GetWallRunningL)
    (CallFunction|CameraTilt 15.0)
    (elif (Variables|WallRun|GetWallRunningR)
      (CallFunction|CameraTilt -15.0)
      (else
        (CallFunction|CameraTilt 0.0)))))

(fn CameraTilt
  (params (TargetX :type Float%20%28single-precision%29))
  (bind _character (Variables|Default|GetCharacter))
  (bind _returnvalue (Pawn|GetController _character))
  (bind _returnvalue_2 (Pawn|GetControlRotation _returnvalue :!class /Script/Engine.Controller))
  (bind (_roll _pitch _yaw) (Math|Rotator|BreakRotator _returnvalue_2))
  (Pawn|SetControlRotation _returnvalue (Math|Interpolation|RInterpTo _returnvalue_2 (Math|Rotator|MakeRotator TargetX _pitch _yaw) (Utilities|Time|GetWorldDeltaSeconds) 1e+01)))

(fn WallRunJump
  (bind _wallrunnormal (Variables|WallRun|GetWallRunNormal))
  (bind _wallrunjumpoffforce (Variables|WallRun|GetWallRunJumpOffForce))
  (if (Variables|WallRun|GetWallRunning)
    (CallFunction|WallRunEnd 0.35)
    (Character|LaunchCharacter (Variables|Default|GetCharacter) (Math|Vector|MakeVector (* _wallrunjumpoffforce (.x _wallrunnormal)) (* _wallrunjumpoffforce (.y _wallrunnormal)) (Variables|WallRun|GetWallRunJumpHeight)) false true)))

(fn Climb)